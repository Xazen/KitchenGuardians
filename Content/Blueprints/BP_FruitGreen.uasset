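; BP_FruitGreen is a green fruit enemy that rotates along a spline and damages the Toast, Rice or Ice guardian it hits.
; Tap has the Toast guardian shoot and spawn a knife at it, though the touch-input call is disabled.
; Hits briefly pause movement with particle and material feedback, while death awards score and launches physics giblets.
; Overlapped shadow colliders set the drop shadow's height, and Tick fades it by distance.
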(event `self.ReceiveActorOnInputTouchBegin`
  (params (FingerIndex :type "InputCoreTypes.ETouchIndex Enum" :default "Touch1"))
  (if false
    (`self.Tap`)))

(event `Tap`
  (bind _returnvalue (`Guardian.canShoot` (`self.guardianToast`)))
  (if _returnvalue
    (`Guardian.Shot` (`self.guardianToast`) 1)
    (`self.spawnKnife` "Toaster")))

(event `self.hitRice`
  (`Guardian.GotHit` (`self.guardianRice`))
  (`self.K2_DestroyActor` :!label _label))

(event `self.ReceiveTick`
  (params (DeltaSeconds :type "Float (single-precision)"))
  (bind _dropshadowzvalue (`self.dropShadowZValue`))
  (bind _dropshadow (`self.dropShadow`))
  (bind _returnvalue (- (.z (`SceneComponent.K2_GetComponentLocation` (`self.SkeletalMesh`))) (`self.dropShadowZValue`)))
  (`/Engine/EditorBlueprintResources/StandardMacros.IsValid` self
    (:`Is Valid`
      (if (`self.bAutoDestroyWhenFinished`)
        _
        (elif (`self.canMove`)
          (`self.MoveEnemyAlongSpline`)
          (`self.Rotate` DeltaSeconds)
          (`self.CalculateDistancePercentage` DeltaSeconds)
          (bind _returnvalue_2 (`self.CheckDistancePercentage`))
          ;[1 1 1] shadow
          (if (> _dropshadowzvalue -1.0)
            (`SceneComponent.K2_SetWorldLocation` _dropshadow (`KismetMathLibrary.MakeVector` (.x (`SceneComponent.K2_GetComponentLocation` _dropshadow)) (.y (`SceneComponent.K2_GetComponentLocation` _dropshadow)) _dropshadowzvalue) false)
            (if (> _returnvalue 100.0)
              (set `self.dropShadowAlpha` 0.3)
              (elif (> _returnvalue 80.0)
                (set `self.dropShadowAlpha` 0.4)
                (elif (> _returnvalue 60.0)
                  (set `self.dropShadowAlpha` 0.5)
                  (elif (> _returnvalue 40.0)
                    (set `self.dropShadowAlpha` 0.6)
                    (elif (> _returnvalue 30.0)
                      (set `self.dropShadowAlpha` 0.7)
                      (elif (> _returnvalue 20.0)
                        (set `self.dropShadowAlpha` 0.8)
                        (elif (> _returnvalue 10.0)
                          (set `self.dropShadowAlpha` 0.9)
                          (else
                            (if (> _returnvalue 0.0)
                              _
                              (else
                                _))
                            (set `self.dropShadowAlpha` 1.0)))))))))
            (`PaperSpriteComponent.SetSpriteColor` (`self.dropShadow`) (`KismetMathLibrary.MakeColor` 1.0 1.0 1.0 (`self.dropShadowAlpha`)))
            (if _returnvalue_2
              (set `self.bAutoDestroyWhenFinished` true))))))))

(event `self.hitToast`
  (`/Game/Blueprints/BP_Toast.GotHit` (`self.guardianToast`))
  (goto _label))

(event `self.hitIce`
  (`Guardian.GotHit` (`self.guardianIce`))
  (goto _label))

(event `self.GotHitFeedback`
  (set `self.canMove` false)
  (`GameplayStatics.SpawnEmitterAtLocation` "/Game/VFX/Particles/PS_FruitGreen.PS_FruitGreen" (`self.K2_GetActorLocation`))
  (`AudioComponent.Play` (`self.BP_Cube`) 0.0)
  (`|ExecutionSequence`
    (:`then_0`
      ;[1 1 1] Toaster hit Enemy                                  Smoke PS                                                       Darker Material
      (bind _asbp_toast (cast `/Game/Blueprints/BP_Toast` (`self.guardianToast`)))
      (if (`/Game/Blueprints/BP_Toast.Reload` _asbp_toast)
        (`GameplayStatics.SpawnEmitterAtLocation` "/Game/VFX/Particles/PS_Placeholder.PS_Placeholder" (0.0 0.0 0.0) (struct))
        (`PrimitiveComponent.SetMaterial` (`self.SkeletalMesh`) 0 "/Game/Materials/Burned/BurnedMushroom.BurnedMushroom")
        (`KismetSystemLibrary.Delay` 0.5)
        (`PrimitiveComponent.SetMaterial` (`self.SkeletalMesh`) 0 "/Game/Animations/MushRoom/Mushroom_dDo_d_Mat.Mushroom_dDo_d_Mat")))
    (:`then_1`
      ;[1 1 1] Stop movement for 400 Milliseconds
      (`KismetSystemLibrary.Delay` 0.4)
      (if (not (`self.willDie`))
        (set `self.canMove` true)))))

(event `self.shadowTester.OnComponentBeginOverlap`
  (params (OtherActor :type "Actor Object Reference") (OtherComp :type "PrimitiveComponent Object Reference") (OtherBodyIndex :type Integer) (bFromSweep :type Boolean) (SweepResult :type "EngineTypes.HitResult Structure (by ref)"))
  (bind _dropshadow (`self.dropShadow`))
  ;[1 1 1] Enemy Overlap Shadow Collider
  (bind _asbp_drop_shadow_collider (cast `/Game/Blueprints/BP_DropShadow_Collider` OtherActor))
  (set `self.dropShadowZValue` (`/Game/Blueprints/BP_DropShadow_Collider.objectZ` _asbp_drop_shadow_collider))
  (`SceneComponent.K2_SetWorldLocation` _dropshadow (`KismetMathLibrary.MakeVector` (.x (`SceneComponent.K2_GetComponentLocation` _dropshadow)) (.y (`SceneComponent.K2_GetComponentLocation` _dropshadow)) (`self.dropShadowZValue`)) false)
  (`SceneComponent.SetVisibility` _dropshadow true false))

(event `self.diedFeedback`
  (set `self.willDie` true)
  (set `self.canMove` false)
  (`GameplayStatics.SpawnEmitterAtLocation` "/Game/VFX/Particles/PS_FruitGreen.PS_FruitGreen" (`self.K2_GetActorLocation`))
  (`AudioComponent.Play` (`self.BP_Cube`) 0.0)
  (`/Game/Blueprints/BP_Cube.Scorred` (`self.BP_Cube`) (`self.baseScore`) (`self.enemyType`))
  (`ActorComponent.K2_DestroyComponent` (`self.SkeletalMesh`))
  (`ActorComponent.K2_DestroyComponent` (`self.dropShadow`))
  (`ActorComponent.K2_DestroyComponent` (`self.shadowTester`))
  ;[1 1 1] Giblet Activation and Add Impulse
  (for (_array_element _array_index) (`self.gibletList`)
    (`SceneComponent.SetVisibility` _array_element true false)
    (`PrimitiveComponent.SetSimulatePhysics` _array_element true)
    (switch `int` _array_index
      (:`Default`
        (set `self.impulseVec` (30.0 -10.0 -10.0) :!label _label_2))
      (:`3`
        (set `self.impulseVec` (-30.0 0.0 -10.0)))
      (:`4`
        (goto _label_2))
      (:`5`
        (set `self.impulseVec` (0.0 -40.0 -10.0)))
      (:`6`
        (set `self.impulseVec` (0.0 40.0 -10.0))))
    (`PrimitiveComponent.AddImpulse` _array_element (`self.impulseVec`) "None" false))
  (`KismetSystemLibrary.Delay` 2.5)
  (`self.K2_DestroyActor`))

(event `self.shadowTester.OnComponentEndOverlap`
  (params (OtherActor :type "Actor Object Reference") (OtherComp :type "PrimitiveComponent Object Reference") (OtherBodyIndex :type Integer))
  ;[1 1 1] Enemy Overlap Shadow Collider
  (cast `/Game/Blueprints/BP_DropShadow_Collider` OtherActor)
  (`SceneComponent.SetVisibility` (`self.dropShadow`) false false))

(event `self.spawnKnifeExecute`
  (bind _bp_cube (`self.BP_Cube`))
  (bind _returnvalue (`|SpawnActorFromClass` "/Game/Blueprints/BP_Knife.BP_Knife_C" (`self.knifeSpawn`) true))
  (`/Game/Blueprints/BP_Knife.MoveTowards` _returnvalue self _bp_cube false)
  (`AudioComponent.Play` _bp_cube 0.0))

(fn `UserConstructionScript`
  (bind _gibletlist (`self.gibletList`))
  (`/Engine/EditorBlueprintResources/StandardMacros.DoOnce` false
    (:`Completed`
      (`KismetArrayLibrary.Array_Add` _gibletlist (`self.Giblet01`))
      (`KismetArrayLibrary.Array_Add` _gibletlist (`self.Giblet02`))
      (`KismetArrayLibrary.Array_Add` _gibletlist (`self.Giblet03`))
      (`KismetArrayLibrary.Array_Add` _gibletlist (`self.Giblet04`))
      (`KismetArrayLibrary.Array_Add` _gibletlist (`self.Giblet05`))
      (`KismetArrayLibrary.Array_Add` _gibletlist (`self.Giblet06`))
      (`KismetArrayLibrary.Array_Add` _gibletlist (`self.Giblet07`)))))