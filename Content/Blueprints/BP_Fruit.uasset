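; BP_Fruit is a touchable target that travels along a Waypoints path, costing Ricebot a life and destroying itself at the end.
; Tick moves it toward the current waypoint, scaled by Speed and delta time, and advances the index within a small squared-distance threshold.
; When Loaded, a touch spawns a BP_Knife aimed at the fruit, clearing Loaded only if Hitpoints is below one.
; SpawnKnife zeroes Hitpoints and fires the same way.
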(event `self.ReceiveActorOnInputTouchBegin`
  (params (FingerIndex :type "InputCoreTypes.ETouchIndex Enum" :default "Touch1"))
  (bind _ricebot (`self.Ricebot`))
  (bind _output_get (set `self.Hitpoints` (+ (`self.Hitpoints`) 0)))
  (if (< _output_get 1)
    (if (`self.loaded`)
      (set `self.loaded` false)
      (bind _returnvalue (`|SpawnActorFromClass` "/Game/Blueprints/BP_Knife.BP_Knife_C" (`self.KnifeSpawn`) true))
      (`/Game/Blueprints/BP_Knife.MoveTowards` _returnvalue self _ricebot))
    (elif (`self.loaded`)
      (set `self.loaded` true)
      (bind _returnvalue_2 (`|SpawnActorFromClass` "/Game/Blueprints/BP_Knife.BP_Knife_C" (`self.KnifeSpawn`) true))
      (`/Game/Blueprints/BP_Knife.MoveTowards` _returnvalue_2 self _ricebot))))

(event `self.ReceiveBeginPlay`)

(event `self.ReceiveActorBeginOverlap`
  (params (OtherActor :type "Actor Object Reference")))

(event `self.ReceiveTick`
  (params (DeltaSeconds :type "Float (single-precision)"))
  (bind _location (.location (`self.GetTransform`)))
  (bind _returnvalue (`self.K2_GetActorLocation` (`KismetArrayLibrary.Array_Get` (`self.Waypoints`) (`self.Waypoint_Int`))))
  (if true
    (if (<= (`KismetMathLibrary.VSizeSquared` (- _location _returnvalue)) 100.0)
      (bind _output_get (set `self.Waypoint_Int` (+ (`self.Waypoint_Int`) 1)))
      (if (== _output_get (`KismetArrayLibrary.Array_Length` (`self.Waypoints`)))
        (`/Game/Blueprints/BP_Cube.LostLife` (`self.Ricebot`))
        (`self.K2_DestroyActor`)
        (else
          (`self.K2_SetActorTransform` (`KismetMathLibrary.MakeTransform` (+ _location (* (`KismetMathLibrary.Normal` (`KismetMathLibrary.GetDirectionVector` _location _returnvalue)) (* (`self.Speed`) (* DeltaSeconds 260.0)))) (.rotation (`self.GetTransform`)) (.scale (`self.GetTransform`))) :!label _label)))
      (else
        (goto _label)))))

(fn `GetVector`
  (returns (NewParam :type "Object.Vector Structure"))
  (return (`SceneComponent.K2_GetComponentLocation`)))

(fn `SpawnKnife`
  (set `self.Hitpoints` 0)
  (if (`self.loaded`)
    (set `self.loaded` false)
    (bind _returnvalue (`|SpawnActorFromClass` "/Game/Blueprints/BP_Knife.BP_Knife_C" (`self.KnifeSpawn`) true))
    (`/Game/Blueprints/BP_Knife.MoveTowards` _returnvalue self (`self.Ricebot`))))

(fn `UserConstructionScript`)