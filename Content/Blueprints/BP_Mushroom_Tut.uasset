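; Tutorial mushroom Blueprint that handles hit and death feedback, gated by its OnlySwipe flag.
; A hit plays randomized swipe audio and particles and halts movement briefly unless the mushroom is dying.
; Death removes mesh and shadow, then launches physics giblets via radial impulse, randomly offset or placed at RadialForcePosition, before delayed destruction.
; A SpawnScale helper lerps the scene scale from a minimum to full size.
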(event `self.GotHitRiceFeedback`
  (bind _returnvalue (`self.K2_GetActorLocation`))
  (if (`self.onlySwipe`)
    (`self.playRandomSwipeHitSound` _returnvalue)
    (set `self.canMove` false)
    (`GameplayStatics.SpawnEmitterAtLocation` "/Game/VFX/Particles/PS_FruitGreen.PS_FruitGreen" _returnvalue)
    (`GameplayStatics.PlaySoundAtLocation` "/Game/Audio/SFX/firstIteration/mushroomDied.mushroomDied" _returnvalue)
    (`|ExecutionSequence`
      (:`then_1`
        ;[1 1 1] Stop movement for 400 Milliseconds
        (`KismetSystemLibrary.Delay` 0.4)
        (if (not (`self.willDie`))
          (set `self.canMove` true))))))

(event `self.diedRiceFeedback`
  (if (`self.onlySwipe`)
    (`self.playRandomSwipeHitSound` (`self.K2_GetActorLocation`))
    (set `self.willDie` true)
    (set `self.canMove` false)
    (`|ExecutionSequence`
      (:`then_1`
        (`ActorComponent.K2_DestroyComponent` (`self.SkeletalMesh`))
        (`ActorComponent.K2_DestroyComponent` (`self.dropShadow`))
        (`ActorComponent.K2_DestroyComponent` (`self.shadowTester`))
        ;[1 1 1] Giblet Activation and Add Impulse
        (if (> (`KismetArrayLibrary.Array_Length` (`self.gibletList`)) 0)
          (`|ExecutionSequence`
            (:`then_0`
              (`GameplayStatics.SpawnEmitterAtLocation` "/Game/Effects/P_MushroomDied.P_MushroomDied" (`SceneComponent.K2_GetComponentLocation` (`self.TapReference`)))
              (`GameplayStatics.PlaySoundAtLocation` "/Game/Audio/SFX/firstIteration/mushroomDied.mushroomDied" (`self.K2_GetActorLocation`)))
            (:`then_1`
              (for _array_element (`self.gibletList`)
                (`SceneComponent.SetVisibility` _array_element true false)
                (`PrimitiveComponent.SetSimulatePhysics` _array_element true))
              (`self.GibbletImpulse`)
              (`KismetSystemLibrary.Delay` (`self.GibbletStayTime`))
              (`self.K2_DestroyActor`))))))))

(fn `GibbletImpulse`
  (bind _returnvalue (`KismetMathLibrary.RandomFloatInRange` -20.0 20.0))
  (bind _radialforce (`self.RadialForce`))
  (if (== (`self.RadialForcePosition`) (0.0 0.0 0.0))
    (`SceneComponent.K2_AddLocalOffset` _radialforce (`KismetMathLibrary.MakeVector` _returnvalue _returnvalue _returnvalue) true)
    (set `RadialForceComponent.ImpulseStrength` (`self.GibbletImpulseSwipe`) _radialforce)
    (else
      (`SceneComponent.K2_SetWorldLocation` _radialforce (`self.RadialForcePosition`) true)
      (set `RadialForceComponent.ImpulseStrength` (`self.GibbletImpulseTap`) _radialforce)))
  (`RadialForceComponent.FireImpulse` _radialforce))

(fn `playRandomSwipeHitSound`
  (params (Location :type "Object.Vector Structure" :default (0.0 0.0 0.0)))
  (switch `int` (`KismetMathLibrary.RandomIntegerInRange` 0 2)
    (:`0`
      (`GameplayStatics.PlaySoundAtLocation` "/Game/Audio/SFX/firstIteration/swipeHit1.swipeHit1" Location 1.0 (`KismetMathLibrary.RandomFloatInRange` 0.8 1.2)))
    (:`1`
      (`GameplayStatics.PlaySoundAtLocation` "/Game/Audio/SFX/firstIteration/swipeHit2.swipeHit2" Location 1.0 (`KismetMathLibrary.RandomFloatInRange` 0.8 1.2)))
    (:`2`
      (`GameplayStatics.PlaySoundAtLocation` "/Game/Audio/SFX/firstIteration/swipeHit3.swipeHit3" Location 1.0 (`KismetMathLibrary.RandomFloatInRange` 0.8 1.2)))))

(fn `SpawnScale`
  (params (DeltaTime :type "Float (double-precision)" :default 0.0))
  (bind _returnvalue (`KismetMathLibrary.Lerp` 1.0 (`self.SpawnMinScale`) (/ (`self.CurrentSpawnScaleTime`) (`self.SpawnScaleTime`))))
  (bind _output_get (set `self.CurrentSpawnScaleTime` (- (`self.CurrentSpawnScaleTime`) DeltaTime)))
  (if (<= _output_get 0.0)
    (set `self.isScaling` false)
    (set `self.CurrentSpawnScaleTime` 0.0))
  (`SceneComponent.SetWorldScale3D` (`self.Scene`) (`KismetMathLibrary.MakeVector` _returnvalue _returnvalue _returnvalue)))

(fn `UserConstructionScript`
  (bind _gibletlist (`self.gibletList`))
  (`/Engine/EditorBlueprintResources/StandardMacros.DoOnce` false
    (:`Completed`
      (`KismetArrayLibrary.Array_Add` _gibletlist (`self.GibletBody1`))
      (`KismetArrayLibrary.Array_Add` _gibletlist (`self.GibletBody2`))
      (`KismetArrayLibrary.Array_Add` _gibletlist (`self.GibletHead1`))
      (`KismetArrayLibrary.Array_Add` _gibletlist (`self.GibletHead2`)))))