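; Spawn controller that repeatedly tells randomly chosen Fridges to spawn objects until BPCube reports game over.
; Tick alternates between spawning and a Delay-based reload, whose time decays exponentially toward a floor as the spawn count grows.
; SelectSpawn uses BPCube's HighScore to widen the range of eligible fridges and enable occasional double spawns.
; The double spawn's reroll does not compare against the first fridge used, so both can hit the same one.
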(event EventBeginPlay)

(event EventActorBeginOverlap
  (params (OtherActor :type Actor%20Object%20Reference)))

(event EventTick
  (params (DeltaSeconds :type Float%20%28single-precision%29))
  (if (Variables|/Script/KitchenGuardians.GameLogic|GetisGameover (Variables|Default|GetBP_Cube))
    (Variables|Default|SetisActive false))
  (if (Variables|Default|GetisActive)
    (if (Variables|Default|GetReloaded)
      (Variables|Default|SetReloaded false)
      (if true
        (bind _spawns (CallFunction|SelectSpawn (Variables|/Script/KitchenGuardians.GameLogic|GethighScore (Variables|Default|GetBP_Cube))))
        (Variables|Default|SetReloadTime (+ 1.0 (* 2.5 (Math|Float|Power 2.72 (* -0.02 (Math|Conversions|ToFloat(Integer) _spawns))))))
        (Variables|Default|SetFactor (+ 1.0 (* (Math|Conversions|ToFloat(Integer) (/ (Variables|/Script/KitchenGuardians.GameLogic|GethighScore (Variables|Default|GetBP_Cube)) 1000)) 0.1))))
      (else
        (Utilities|FlowControl|Delay (Variables|Default|GetReloadTime))
        (Variables|Default|SetReloaded true)))))

(fn ConstructionScript)

(fn SelectSpawn
  (params (HighScore :type Integer :default 0))
  (LocalVariables|SetLoc_HighScore HighScore)
  (if (< (LocalVariables|GetLoc_HighScore) 400)
    (LocalVariables|SetLoc_SpawnRage 0)
    (LocalVariables|Setdouble%20spawn false)
    (elif (< (LocalVariables|GetLoc_HighScore) 1800)
      (LocalVariables|SetLoc_SpawnRage 1)
      (LocalVariables|Setdouble%20spawn true)
      (else
        (LocalVariables|SetLoc_SpawnRage 3)
        (LocalVariables|Setdouble%20spawn true))))
  (if (LocalVariables|Getdouble%20spawn)
    (if (<= (Math|Random|RandomIntegerinRange 0 10) 6)
      (Default|SpawnObject (Utilities|Array|Get(acopy) (Variables|Default|GetFridges) (Math|Random|RandomIntegerinRange 0 (LocalVariables|GetLoc_SpawnRage))) :!label _label)
      (else
        (Default|SpawnObject (Utilities|Array|Get(acopy) (Variables|Default|GetFridges) (Math|Random|RandomIntegerinRange 0 (LocalVariables|GetLoc_SpawnRage))))
        (bind _output_get (LocalVariables|SetLocRandom1 (Math|Random|RandomIntegerinRange 0 (LocalVariables|GetLoc_SpawnRage))))
        (LocalVariables|SetLocRandom2 _output_get)
        (while (== (LocalVariables|GetLocRandom2) (LocalVariables|GetLocRandom1))
          (LocalVariables|SetLocRandom2 (Math|Random|RandomIntegerinRange 0 (LocalVariables|GetLoc_SpawnRage))))
        (Default|SpawnObject (Utilities|Array|Get(acopy) (Variables|Default|GetFridges) (LocalVariables|GetLocRandom2)))))
    (else
      (goto _label)))
  (bind _output_get_2 (Variables|Default|SetspawnS (+ (Variables|Default|GetspawnS) 1)))
  (return _output_get_2))