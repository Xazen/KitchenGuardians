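; BP_FruitBlue is a blue fruit target that travels a chain of splines and damages a bot at the end.
; Tick advances it at a rate based on spline direction and progress, then hits the bot chosen by BotHitCase.
; Touching it while Other2 is activated fires a homing-target BP_Knife from that bot, limited by FruitHits and CanShoot.
; GotHit emits particles, reduces Hitpoints and awards score through Ricebot on death.
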(event EventBeginPlay)

(event EventActorBeginOverlap
  (params (OtherActor :type Actor%20Object%20Reference)))

(event EventTick
  (params (DeltaSeconds :type Float%20%28single-precision%29))
  (bind _returnvalue (Transformation|GetActorTransform))
  (bind (_location _rotation _scale) (Math|Transform|BreakTransform _returnvalue))
  (Transformation|SetActorTransform (Math|Transform|MakeTransform (Class|SplineComponent|GetWorldLocationatDistanceAlongSpline (Utilities|Array|Get(acopy) (Variables|Default|GetSplineRoute) (Variables|Default|GetCurrentSpline)) (* (Spline|GetSplineLength (Utilities|Array|Get(acopy) (Variables|Default|GetSplineRoute) (Variables|Default|GetCurrentSpline))) (Variables|Default|GetDistPerc))) _rotation _scale))
  (bind _new_dist_perc (CallFunction|CalcDistPerc DeltaSeconds))
  (bind _output_get (Variables|Default|SetDistPerc _new_dist_perc))
  (if (>= _output_get 1.0)
    (if (< (Variables|Default|GetCurrentSpline) (+ (Utilities|Array|Length (Variables|Default|GetSplineRoute)) -1))
      (Variables|Default|SetDistPerc 0.0)
      (Variables|Default|SetCurrentSpline (+ (Variables|Default|GetCurrentSpline) 1))
      (else
        (switch int (Variables|Default|GetBotHitCase)
          (:1
            (Default|GotHit (Variables|Default|Getother1) 1))
          (:2
            (Default|GotHit (Variables|Default|Getother2) 1))
          (:3
            (Default|GotHit (Variables|Default|Getother3) 1)))
        (Actor|DestroyActor)))))

(event EventActorOnInputTouchBegin
  (params (FingerIndex :type ETouchIndex%20Enum :default "Touch1"))
  (if (Variables|/Game/Blueprints/BP_otherChar2.BP_otherChar2_C|GetActivated (Variables|Default|Getother2))
    (CallFunction|SpawnKnife 2)))

(fn ConstructionScript)

(fn GetVector
  (return (Transformation|GetWorldLocation)))

(fn SpawnKnife
  (params (Spawning%20Bot%20Case :type Integer :default 0))
  (bind _ricebot (Variables|Default|GetRiceBot))
  (if (> (Variables|Default|GetFruitHits) 0)
    (Variables|Default|SetFruitHits (+ (Variables|Default|GetFruitHits) -1))
    (if (== (Variables|Default|GetHitpoints) 0)
      (Variables|Default|Setloaded false))
    (bind (_knifespawn _canshoot) (CallFunction|GetKnifeSpawn Spawning%20Bot%20Case))
    (if _canshoot
      (bind _returnvalue (Game|SpawnActorfromClass "/Game/Blueprints/BP_Knife.BP_Knife_C" _knifespawn true 0))
      (Default|MoveTowards _returnvalue self _ricebot false)
      (Audio|Components|Audio|Play _ricebot 0.0))))

(fn GetKnifeSpawn
  (params (SpawningBot :type Integer :default 0))
  (bind _other2 (Variables|Default|Getother2))
  (bind _other3 (Variables|Default|Getother3))
  (switch int SpawningBot
    (:2
      (LocalVariables|Setloca (Transformation|GetActorTransform _other2))
      (LocalVariables|Setload (Variables|/Game/Blueprints/BP_otherChar2.BP_otherChar2_C|GetcanShoot _other2))
      (Default|Shot _other2))
    (:3
      (LocalVariables|Setloca (Transformation|GetActorTransform _other3))
      (LocalVariables|Setload (Variables|/Game/Blueprints/BP_otherChar3.BP_otherChar3_C|GetcanShoot _other3))
      (Default|Shot _other3)))
  (return (LocalVariables|Getloca) (LocalVariables|Getload)))

(fn GotHit
  (params (Case :type Integer :default 0))
  (bind _ricebot (Variables|Default|GetRicebot))
  (Effects|SpawnEmitteratLocation "/Game/VFX/Particles/PS_FruitBlue.PS_FruitBlue" (Transformation|GetActorLocation))
  (switch int Case
    (:1
      (LocalVariables|SetLoc_DmgPerOther -1))
    (:2
      (LocalVariables|SetLoc_DmgPerOther -1))
    (:3
      (LocalVariables|SetLoc_DmgPerOther -1)))
  (bind _output_get (Variables|Default|SetHitpoints (+ (Variables|Default|GetHitpoints) (LocalVariables|GetLoc_DmgPerOther))))
  (if (<= _output_get 0)
    (Audio|Components|Audio|Play _ricebot 0.0)
    (Default|Scorred (Variables|Default|GetRicebot) (Variables|Default|GetScore))
    (Actor|DestroyActor)
    (else
      (Audio|Components|Audio|Play _ricebot 0.0))))

(fn CalcDistPerc
  (params (Delta :type Float%20%28single-precision%29 :default 0.0))
  (bind _currentspline (Variables|Default|GetCurrentSpline))
  (bind _splineroute (Variables|Default|GetSplineRoute))
  (bind _distperc (Variables|Default|GetDistPerc))
  (bind _item (Utilities|Array|Get(acopy) _splineroute _currentspline))
  (return (+ _distperc (* Delta (+ (* (Math|Float|Absolute(Float) (Math|Trig|Cos(Degrees) (.Z (Math|Vector|BreakVector (Class|SplineComponent|GetWorldDirectionatDistanceAlongSpline _item (* (Spline|GetSplineLength _item) _distperc)))))) 0.5) (+ (* _distperc 0.3) 0.02))))))