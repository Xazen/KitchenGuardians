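; Fake dirt actor that shows splatter on three planes, with Chili and Pumpkin enemy hits on its collision triggering the first two.
; Each plane gets a dynamic material instance, and activation sets full Alpha and a random Degree, waits StayTime, then starts a fade.
; Tick lowers Alpha over FadeTime, with DoOnce gates and active flags limiting retriggers.
; The third plane has fade logic but no hit trigger.
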(event `ActivateDecal3`
  ;[0.25 0.1254 0] p3 - activate
  (bind _output_get (set `self.Alpha3` 1.0))
  (`MaterialInstanceDynamic.SetScalarParameterValue` (`self.DirtInstance3`) "Alpha" _output_get)
  (`MaterialInstanceDynamic.SetScalarParameterValue` (`self.DirtInstance3`) "Degree" (`KismetMathLibrary.RandomFloatInRange` 0.0 1.0))
  (`KismetSystemLibrary.Delay` (`self.StayTime`))
  (set `self.CurrentFadeTime3` (`self.FadeTime`))
  (set `self.isFading3` true))

(event `ActivateDecal2`
  ;[0.98 0.4359 0.1862] p2 - activate
  (set `self.decal2IsActive` true)
  (bind _output_get (set `self.Alpha2` 1.0))
  (`MaterialInstanceDynamic.SetScalarParameterValue` (`self.DirtInstance2`) "Alpha" _output_get)
  (`MaterialInstanceDynamic.SetScalarParameterValue` (`self.DirtInstance2`) "Degree" (`KismetMathLibrary.RandomFloatInRange` 0.0 1.0))
  (`KismetSystemLibrary.Delay` (`self.StayTime`))
  (set `self.CurrentFadeTime2` (`self.FadeTime`))
  (set `self.isFading2` true))

(event `ActivateDecal1`
  ;[1 0.08 0.08] p1 - event
  (set `self.decal1IsActive` true)
  (bind _output_get (set `self.Alpha1` 1.0))
  (`MaterialInstanceDynamic.SetScalarParameterValue` (`self.DirtInstance1`) "Alpha" _output_get)
  (`MaterialInstanceDynamic.SetScalarParameterValue` (`self.DirtInstance1`) "Degree" (`KismetMathLibrary.RandomFloatInRange` 0.0 1.0))
  (`KismetSystemLibrary.Delay` (`self.StayTime`))
  (set `self.CurrentFadeTime1` (`self.FadeTime`))
  (set `self.isFading1` true))

(event `self.ReceiveBeginPlay`
  ;[1 0.08 0.08] p1 get material
  (bind _returnvalue (`PrimitiveComponent.CreateDynamicMaterialInstance` (`self.Plane1`) 0 "/Game/Materials/Dirt_Fluid/DirtRed_Inst.DirtRed_Inst"))
  (bind _output_get (set `self.DirtInstance1` _returnvalue))
  (`MaterialInstanceDynamic.SetScalarParameterValue` _output_get "Alpha" (`self.Alpha1`))
  ;[0.98 0.4359 0.1862] p2 - get Material
  (bind _returnvalue_2 (`PrimitiveComponent.CreateDynamicMaterialInstance` (`self.Plane2`) 0 "/Game/Materials/Dirt_Fluid/DirtExample_Inst.DirtExample_Inst"))
  (bind _output_get_2 (set `self.DirtInstance2` _returnvalue_2))
  (`MaterialInstanceDynamic.SetScalarParameterValue` _output_get_2 "Alpha" (`self.Alpha2`))
  ;[0.25 0.1254 0] p3 - get Material
  (bind _returnvalue_3 (`PrimitiveComponent.CreateDynamicMaterialInstance` (`self.Plane3`) 0 "/Game/Materials/Dirt_Fluid/Dirt3_Inst.Dirt3_Inst"))
  (bind _output_get_3 (set `self.DirtInstance3` _returnvalue_3))
  (`MaterialInstanceDynamic.SetScalarParameterValue` _output_get_3 "Alpha" (`self.Alpha3`)))

(event `self.ReceiveActorBeginOverlap`
  (params (OtherActor :type "Actor Object Reference")))

(event `self.ReceiveTick`
  (params (DeltaSeconds :type "Float (single-precision)"))
  ;[1 0.08 0.08] p1 - fade
  (if (`self.isFading1`)
    (bind _output_get (set `self.CurrentFadeTime1` (- (`self.CurrentFadeTime1`) DeltaSeconds)))
    (if (<= _output_get 0.0)
      (set `self.isFading1` false)
      (bind _output_get_2 (set `self.Alpha1` 0.0))
      (`MaterialInstanceDynamic.SetScalarParameterValue` (`self.DirtInstance1`) "Alpha" _output_get_2)
      (if (`self.decal1IsActive`)
        (set `self.decal1IsActive` false)
        ;[0.98 0.4359 0.1862] p2 - fade
        (`self.Reset1`)
        (if (`self.isFading2`) :!label _label
          (bind _output_get_3 (set `self.CurrentFadeTime2` (- (`self.CurrentFadeTime2`) DeltaSeconds)))
          (if (<= _output_get_3 0.0)
            (set `self.isFading2` false)
            (bind _output_get_4 (set `self.Alpha2` 0.0))
            (`MaterialInstanceDynamic.SetScalarParameterValue` (`self.DirtInstance2`) "Alpha" _output_get_4)
            (if (`self.decal2IsActive`)
              (set `self.decal2IsActive` false)
              (`self.Reset2`))
            (else
              (bind _output_get_5 (set `self.Alpha2` (/ (`self.CurrentFadeTime2`) (`self.FadeTime`))))
              (`MaterialInstanceDynamic.SetScalarParameterValue` (`self.DirtInstance2`) "Alpha" _output_get_5))))
        ;[0.25 0.1254 0] p3 - fade
        (if (`self.isFading3`)
          (bind _output_get_6 (set `self.CurrentFadeTime3` (- (`self.CurrentFadeTime3`) DeltaSeconds)))
          (if (<= _output_get_6 0.0)
            (set `self.isFading3` false)
            (bind _output_get_7 (set `self.Alpha3` 0.0))
            (`MaterialInstanceDynamic.SetScalarParameterValue` (`self.DirtInstance3`) "Alpha" _output_get_7)
            (`self.Reset3`)
            (else
              (bind _output_get_8 (set `self.Alpha3` (/ (`self.CurrentFadeTime3`) (`self.FadeTime`))))
              (`MaterialInstanceDynamic.SetScalarParameterValue` (`self.DirtInstance3`) "Alpha" _output_get_8)))))
      (else
        (bind _output_get_9 (set `self.Alpha1` (/ (`self.CurrentFadeTime1`) (`self.FadeTime`))))
        (`MaterialInstanceDynamic.SetScalarParameterValue` (`self.DirtInstance1`) "Alpha" _output_get_9)
        (goto _label)))
    (else
      (goto _label))))

(event `Reset2`
  ;[0.98 0.4359 0.1862] p2 - activate
  (if (not (> (`self.Alpha2`) 0.0))
    (goto _label_3 :!via `Reset`)))

(event `self.Collision.OnComponentHit`
  (params (OtherActor :type "Actor Object Reference") (OtherComp :type "PrimitiveComponent Object Reference") (NormalImpulse :type "Object.Vector Structure") (Hit :type "EngineTypes.HitResult Structure (by ref)"))
  ;[1 1 1] gibblets must
  ; be physical actor
  ;  and simulate hit
  (bind _asenemies (cast `Enemies` OtherActor))
  (switch `Enemies.EnemyTypeEnum` (`Enemies.enemyType` _asenemies)
    (:`Chili`
      ;[1 0.08 0.08] p1 - trigger
      (`/Engine/EditorBlueprintResources/StandardMacros.DoOnce` false :!label _label_2
        (:`Completed`
          (if (not (`self.decal1IsActive`))
            (`self.ActivateDecal1`)))))
    (:`Pumpkin`
      ;[0.98 0.4359 0.1862] p2 - activate
      (`/Engine/EditorBlueprintResources/StandardMacros.DoOnce` false :!label _label_3
        (:`Completed`
          (if (not (`self.decal2IsActive`))
            (`self.ActivateDecal2`)))))))

(event `Reset3`
  ;[0.25 0.1254 0] p3 - activate
  (`/Engine/EditorBlueprintResources/StandardMacros.DoOnce` false :!via `Reset`
    (:`Completed`
      (`self.ActivateDecal3`))))

(event `Reset1`
  (if (> (`self.Alpha1`) 0.0)
    (goto _label_2 :!via `Reset`)))

(fn `UserConstructionScript`)