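; Pumpkin enemy that moves along a spline, scaling up on spawn unless static, with a height-faded drop shadow placed via collider overlaps.
; Rice and toast hit events briefly pause it with particles, sound and a Toaster-only material flash.
; Death events report score to BPCube, including close-kill and golden-pumpkin bonuses, then swap the mesh for physics giblets blasted by a radial impulse.
; The Rice hit case gets an optional-enemy material.
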(event `self.ReceiveBeginPlay`
  (`|ExecutionSequence`
    (:`then_0`
      (if (<= (`KismetMathLibrary.RandomIntegerInRange` 0 100) (`self.SpawnVocalLikelihood`))
        (`GameplayStatics.PlaySoundAtLocation` "/Game/Audio/SFX/Placeholder/pumpkinPlaceholder.pumpkinPlaceholder" (`SceneComponent.K2_GetComponentLocation`)))
      (if (not (`self.staticEnemy`))
        (set `self.isScaling` true)
        (set `self.CurrentSpawnScaleTime` (`self.SpawnScaleTime`))))
    (:`then_1`
      ;[1 1 1] takes a little time till hitcase gets updated
      (`KismetSystemLibrary.Delay` 0.05)
      (if (`|EnumEquality` (`self.guardianHitCaseEnum`) "Rice")
        (`PrimitiveComponent.SetMaterial` 0 "/Game/Materials/Placeholder/Ma_optionalEnemy_Inst.Ma_optionalEnemy_Inst")
        (`PrimitiveComponent.SetMaterial` 0 "/Game/Materials/Placeholder/Ma_optionalEnemy_Inst.Ma_optionalEnemy_Inst")
        (`PrimitiveComponent.SetMaterial` 0 "/Game/Materials/Placeholder/Ma_optionalEnemy_Inst.Ma_optionalEnemy_Inst")
        (`PrimitiveComponent.SetMaterial` 0 "/Game/Materials/Placeholder/Ma_optionalEnemy_Inst.Ma_optionalEnemy_Inst")
        (`PrimitiveComponent.SetMaterial` 0 "/Game/Materials/Placeholder/Ma_optionalEnemy_Inst.Ma_optionalEnemy_Inst")
        (`PrimitiveComponent.SetMaterial` 0 "/Game/Materials/Placeholder/Ma_optionalEnemy_Inst.Ma_optionalEnemy_Inst")
        (`PrimitiveComponent.SetMaterial` 0 "/Game/Materials/Placeholder/Ma_optionalEnemy_Inst.Ma_optionalEnemy_Inst")))))

(event `self.ReceiveTick`
  (params (DeltaSeconds :type "Float (single-precision)"))
  (bind _dropshadowzvalue (`self.dropShadowZValue`))
  (bind _dropshadow (`self.dropShadow`))
  (`/Engine/EditorBlueprintResources/StandardMacros.IsValid` self
    (:`Is Valid`
      (if (`self.bAutoDestroyWhenFinished`)
        _
        (elif (`self.staticEnemy`)
          _
          (elif (`self.canMove`)
            (`|ExecutionSequence`
              (:`then_0`
                (if (`self.isScaling`)
                  (`self.SpawnScale` DeltaSeconds)))
              (:`then_1`
                (`self.MoveEnemyAlongSpline`)
                (`self.Rotate` DeltaSeconds)
                (`self.CalculateDistancePercentage` DeltaSeconds)
                (bind _returnvalue (`self.CheckDistancePercentage`))
                (if (`self.canMove`)
                  ;[1 1 1] shadow
                  (if (> _dropshadowzvalue -1.0)
                    (`SceneComponent.K2_SetWorldLocation` _dropshadow (`KismetMathLibrary.MakeVector` (.x (`SceneComponent.K2_GetComponentLocation` _dropshadow)) (.y (`SceneComponent.K2_GetComponentLocation` _dropshadow)) _dropshadowzvalue) false)
                    (bind _returnvalue_2 (`self.calcDropShadowAlpha` (- (.z (`SceneComponent.K2_GetComponentLocation` (`self.SkeletalMesh`))) (`self.dropShadowZValue`))))
                    (set `self.dropShadowAlpha` _returnvalue_2)
                    (`PaperSpriteComponent.SetSpriteColor` (`self.dropShadow`) (`KismetMathLibrary.MakeColor` 1.0 1.0 1.0 (`self.dropShadowAlpha`)))
                    (if _returnvalue
                      (set `self.bAutoDestroyWhenFinished` true))))))))))))

(event `self.GotHitRiceFeedback`
  (bind _returnvalue (`self.K2_GetActorLocation`))
  (bind _skeletalmesh (`self.SkeletalMesh`))
  (`self.playRandomSwipeHitSound` _returnvalue)
  (set `self.canMove` false :!label _label)
  (`GameplayStatics.SpawnEmitterAtLocation` "/Game/Effects/P_pumpkinGotHit.P_pumpkinGotHit" (`SceneComponent.K2_GetComponentLocation` (`self.TapReference`)))
  (`GameplayStatics.PlaySoundAtLocation` "/Game/Audio/SFX/firstIteration/pumpkinGotHit.pumpkinGotHit" _returnvalue 1.0 (`KismetMathLibrary.RandomFloatInRange` 0.7 1.4))
  (`|ExecutionSequence`
    (:`then_1`
      (if (`|EnumEquality` (`self.guardianHitCaseEnum`) "Toaster")
        (`PrimitiveComponent.SetMaterial` _skeletalmesh 0 "/Game/Materials/Characters/flashTest.flashTest")
        (`KismetSystemLibrary.Delay` 0.05)
        (`PrimitiveComponent.SetMaterial` _skeletalmesh 0 "/Game/Materials/pumpkin/Pumpkin.Pumpkin")))
    (:`then_2`
      ;[1 1 1] Stop movement for 400 Milliseconds
      (`KismetSystemLibrary.Delay` 0.1)
      (if (not (`self.willDie`))
        (set `self.canMove` true)))))

(event `self.GotHitToastFeedback`
  (goto _label))

(event `self.hitToastFeedback`
  (set `self.willDie` true)
  (set `self.canMove` false)
  (`ActorComponent.K2_DestroyComponent` (`self.SkeletalMesh`) :!label _label_2)
  ;[1 1 1] because no skeletal mesh by now
  (`ActorComponent.K2_DestroyComponent` (`self.SkeletalMesh`))
  (`ActorComponent.K2_DestroyComponent` (`self.dropShadow`))
  (`ActorComponent.K2_DestroyComponent` (`self.shadowTester`))
  (`|ExecutionSequence`
    (:`then_0`
      (`GameplayStatics.SpawnEmitterAtLocation` "/Game/Effects/P_pumpkinDie.P_pumpkinDie" (`SceneComponent.K2_GetComponentLocation` (`self.TapReference`)))
      (`GameplayStatics.PlaySoundAtLocation` "/Game/Audio/SFX/firstIteration/pumpkinDied.pumpkinDied" (`self.K2_GetActorLocation`) 1.0 (`KismetMathLibrary.RandomFloatInRange` 0.7 1.4)))
    (:`then_1`
      ;[1 1 1] Giblet Activation and Add Impulse
      (for _array_element (`self.gibletList`)
        (`SceneComponent.SetVisibility` _array_element true false)
        (`PrimitiveComponent.SetSimulatePhysics` _array_element true))
      (`self.GibbletImpulse`)
      (`KismetSystemLibrary.Delay` (`self.GibbletStayTime`))
      (`self.K2_DestroyActor`))))

(event `self.diedRiceFeedback`
  (`self.playRandomSwipeHitSound` (`self.K2_GetActorLocation`))
  (set `self.willDie` true :!label _label_3)
  (set `self.canMove` false)
  (`|ExecutionSequence`
    (:`then_0`
      (if (<= (`KismetMathLibrary.VSize` (- (`self.K2_GetActorLocation`) (`self.K2_GetActorLocation` (`self.BP_Cube`)))) (`self.CloseKillDistance`))
        (`/Game/Blueprints/BP_Cube.specialScore` (`self.BP_Cube`) (`self.K2_GetActorLocation`) "CloseKill")))
    (:`then_1`
      (if (`|EnumEquality` (`self.guardianHitCaseEnum`) "Toaster")
        (`/Game/Blueprints/BP_Cube.Scorred` (`self.BP_Cube`) (`self.baseScore`) (`self.enemyType`))
        (goto _label_2)
        (else
          (`/Game/Blueprints/BP_Cube.specialScore` (`self.BP_Cube`) (`self.K2_GetActorLocation`) "GoldenPumpkin")
          (`/Game/Blueprints/BP_Cube.Scorred` (`self.BP_Cube`) 0 (`self.enemyType`))
          (goto _label_2))))))

(event `self.shadowTester.OnComponentBeginOverlap`
  (params (OtherActor :type "Actor Object Reference") (OtherComp :type "PrimitiveComponent Object Reference") (OtherBodyIndex :type Integer) (bFromSweep :type Boolean) (SweepResult :type "EngineTypes.HitResult Structure (by ref)"))
  (bind _dropshadow (`self.dropShadow`))
  ;[1 1 1] Enemy Overlap Shadow Collider
  (bind _asbp_drop_shadow_collider (cast `/Game/Blueprints/BP_DropShadow_Collider` OtherActor))
  (set `self.dropShadowZValue` (`/Game/Blueprints/BP_DropShadow_Collider.objectZ` _asbp_drop_shadow_collider))
  (`SceneComponent.K2_SetWorldLocation` _dropshadow (`KismetMathLibrary.MakeVector` (.x (`SceneComponent.K2_GetComponentLocation` _dropshadow)) (.y (`SceneComponent.K2_GetComponentLocation` _dropshadow)) (`self.dropShadowZValue`)) false)
  (`SceneComponent.SetVisibility` _dropshadow true false))

(event `self.diedToastFeedback`
  (goto _label_3))

(event `self.shadowTester.OnComponentEndOverlap`
  (params (OtherActor :type "Actor Object Reference") (OtherComp :type "PrimitiveComponent Object Reference") (OtherBodyIndex :type Integer))
  ;[1 1 1] Enemy Overlap Shadow Collider
  (cast `/Game/Blueprints/BP_DropShadow_Collider` OtherActor)
  (`SceneComponent.SetVisibility` (`self.dropShadow`) false false))

(event `self.ReachedEndAsBonusEnemy`
  (`self.K2_DestroyActor`))

(fn `GibbletImpulse`
  (bind _returnvalue (`KismetMathLibrary.RandomFloatInRange` -25.0 25.0))
  (bind _radialforce (`self.RadialForce`))
  (if (== (`self.RadialForcePosition`) (0.0 0.0 0.0))
    (`SceneComponent.K2_AddLocalOffset` _radialforce (`KismetMathLibrary.MakeVector` _returnvalue _returnvalue _returnvalue) true)
    (set `RadialForceComponent.ImpulseStrength` (`self.GibbletImpulseSwipe`) _radialforce)
    (else
      (`SceneComponent.K2_SetWorldLocation` _radialforce (`self.RadialForcePosition`) true)
      (set `RadialForceComponent.ImpulseStrength` (`self.GibbletImpulseTap`) _radialforce)))
  (`RadialForceComponent.FireImpulse` _radialforce))

(fn `playRandomSwipeHitSound`
  (params (Location :type "Object.Vector Structure" :default (0.0 0.0 0.0)))
  (switch `int` (`KismetMathLibrary.RandomIntegerInRange` 0 2)
    (:`0`
      (`GameplayStatics.PlaySoundAtLocation` "/Game/Audio/SFX/firstIteration/swipeHit1.swipeHit1" Location 1.0 (`KismetMathLibrary.RandomFloatInRange` 0.8 1.2)))
    (:`1`
      (`GameplayStatics.PlaySoundAtLocation` "/Game/Audio/SFX/firstIteration/swipeHit2.swipeHit2" Location 1.0 (`KismetMathLibrary.RandomFloatInRange` 0.8 1.2)))
    (:`2`
      (`GameplayStatics.PlaySoundAtLocation` "/Game/Audio/SFX/firstIteration/swipeHit3.swipeHit3" Location 1.0 (`KismetMathLibrary.RandomFloatInRange` 0.8 1.2)))))

(fn `SpawnScale`
  (params (DeltaTime :type "Float (double-precision)" :default 0.0))
  (bind _returnvalue (`KismetMathLibrary.Lerp` 1.0 (`self.SpawnMinScale`) (/ (`self.CurrentSpawnScaleTime`) (`self.SpawnScaleTime`))))
  (bind _output_get (set `self.CurrentSpawnScaleTime` (- (`self.CurrentSpawnScaleTime`) DeltaTime)))
  (if (<= _output_get 0.0)
    (set `self.isScaling` false)
    (set `self.CurrentSpawnScaleTime` 0.0))
  (`SceneComponent.SetWorldScale3D` (`self.Scene`) (`KismetMathLibrary.MakeVector` _returnvalue _returnvalue _returnvalue)))

(fn `UserConstructionScript`
  (bind _gibletlist (`self.gibletList`))
  (`/Engine/EditorBlueprintResources/StandardMacros.DoOnce` false
    (:`Completed`
      (`KismetArrayLibrary.Array_Add` _gibletlist (`self.Pumpkin_Gibblets_1__Gibblet_Part_01`))
      (`KismetArrayLibrary.Array_Add` _gibletlist (`self.Pumpkin_Gibblets_1__Gibblet_Part_02`))
      (`KismetArrayLibrary.Array_Add` _gibletlist (`self.Pumpkin_Gibblets_1__Gibblet_Part_03`))
      (`KismetArrayLibrary.Array_Add` _gibletlist (`self.Pumpkin_Gibblets_1__LP_Auge`))
      (`KismetArrayLibrary.Array_Add` _gibletlist (`self.Pumpkin_Gibblets_1__Gibblet_Part_04`)))))