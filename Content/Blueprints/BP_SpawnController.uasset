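; Spawn controller actor that runs looping enemy waves from kitchen spawn points until the game is over.
; PrepareSpawn fills a queue of weighted-random patterns up to the wave's projected score, then picks spawn point, path and delay.
; SpawnEnemy spawns along that path and advances the wave when the queue empties, while reload time shrinks exponentially with spawn count.
; AddWave appends authored waves; J test-spawns wave zero.
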(event Custom|AddWave
  (bind _newwave (Variables|Blutilities|GetnewWave))
  (if (!= (Utilities|Array|Length (.curveList (Utilities|Struct|BreakEnemyPathStruct (Utilities|Array|Get(acopy) (.pathList (Utilities|Struct|BreakEnemyPatternStruct (Utilities|Array|Get(acopy) (.enemyPatternList (Utilities|Struct|BreakEnemyWaveStruct _newwave))))))))) 0)
    (Utilities|Array|Add (Variables|Blutilities|GetwaveList) _newwave)))

(event EventTick
  (params (DeltaSeconds :type Float%20%28single-precision%29))
  (Utilities|FlowControl|Sequence
    (:then_0
      (if (Variables|/Script/KitchenGuardians.GameLogic|GetisGameover (Variables|Default|GetBP_Cube))
        (Variables|Default|SetisActive false))
      (if (Variables|Default|GetisActive)
        (if (!= (Utilities|Array|Length (Variables|Blutilities|GetwaveList)) 0)
          (if (Variables|Default|GetReloaded)
            (Variables|Default|SetReloaded false)
            (if (Variables|Default|GetwaveCompleted)
              (Variables|Default|SetwaveNr (+ (Variables|Default|GetwaveNr) 1))
              (if (> (Variables|Default|GetwaveNr) (- (Utilities|Array|Length (Variables|Blutilities|GetwaveList)) 1))
                (Variables|Default|SetwaveNr 0))
              (Variables|Default|SetwaveCompleted false))
            (bind (_spawndelay _enemypath) (CallFunction|PrepareSpawn (Variables|Default|GetwaveNr)))
            (Utilities|FlowControl|Delay _spawndelay)
            (CallFunction|SpawnEnemy _enemypath)
            (Variables|Default|SetReloadTime (+ 1.0 (* 2.5 (Math|Float|Power 2.72 (* -0.02 (Math|Conversions|ToFloat(Integer) (Variables|Default|GetSpawnCounter)))))))
            (else
              (Utilities|FlowControl|Delay (Variables|Default|GetReloadTime))
              (Variables|Default|SetReloaded true))))))
    (:then_1
      (Utilities|FlowControl|DoOnce false :!label _label
        (:Completed
          (Development|PrintString (Utilities|String|Append "Wave: " (Utilities|String|ToString(Integer) (Variables|Default|GetwaveNr))))
          (Utilities|FlowControl|Delay 2.0)
          (goto _label Reset))))))

(event EventBeginPlay)

(event EventActorBeginOverlap
  (params (OtherActor :type Actor%20Object%20Reference)))

(event Input|KeyboardEvents|J
  (:Pressed
    (bind (_spawndelay _enemypath) (CallFunction|PrepareSpawn))
    (Utilities|FlowControl|Delay _spawndelay)
    (CallFunction|SpawnEnemy _enemypath)))

(fn ConstructionScript
  (bind _newwave (Variables|Blutilities|GetnewWave))
  (bind (_timetokillmultiplier _totalprojectedscore _enemyspawnpoint _enemypatternlist _probabilityofpatternlist) (Utilities|Struct|BreakEnemyWaveStruct _newwave))
  ;[1 1 1] Add a default value for POPL to prevent missing values
  (Utilities|Array|Resize _probabilityofpatternlist (Utilities|Array|Length _enemypatternlist)))

(fn PrepareSpawn
  (params (waveIndex :type Integer :default 0))
  (bind _randomprobabilitylist (Variables|Default|GetrandomProbabilityList))
  (bind _item (Utilities|Array|Get(acopy) _randomprobabilitylist))
  ;[1 1 1] Get Wave from waveList[waveIndex]
  (LocalVariables|SetLocWaveStruct (Utilities|Array|Get(acopy) (Variables|Blutilities|GetwaveList) waveIndex))
  ;[1 1 1] On Wave Start
  (Variables|Default|SettotalPropability 0)
  (for _array_element (.probabilityOfPatternList (Utilities|Struct|BreakEnemyWaveStruct (LocalVariables|GetLocWaveStruct)))
    (Variables|Default|SettotalPropability (+ _array_element (Variables|Default|GettotalPropability))))
  (if (<= (Variables|Default|GetcurrentProjectedScore) (.totalProjectedScore (Utilities|Struct|BreakEnemyWaveStruct (LocalVariables|GetLocWaveStruct)))) :!label _label
    (bind (_array_element_2 _array_index) (Utilities|Array|ForEachLoopwithBreak (.probabilityOfPatternList (Utilities|Struct|BreakEnemyWaveStruct (LocalVariables|GetLocWaveStruct))) :!label _label_2)
      (:LoopBody
        (bind _output_get (LocalVariables|SetlastValueMax (+ (LocalVariables|GetlastValueMax) _array_element_2)))
        (if (>= _output_get (Math|Random|RandomIntegerinRange 1 (Variables|Default|GettotalPropability)))
          (Utilities|Array|Add (Variables|Default|GetrandomProbabilityList) _array_index)
          (Variables|Default|SetcurrentProjectedScore (+ (Variables|Default|GetcurrentProjectedScore) (.projectedScore (Utilities|Struct|BreakEnemyPatternStruct (Utilities|Array|Get(acopy) (.enemyPatternList (Utilities|Struct|BreakEnemyWaveStruct (LocalVariables|GetLocWaveStruct))) _array_index)))))
          (goto _label_2 Break)))
      (:Completed
        (LocalVariables|SetlastValueMax 0)
        (goto _label)))
    (else
      ;[1 1 1] Ready to Spawn
      (Development|PrintString (Utilities|String|Append "Pattern: " (Utilities|String|ToString(Integer) _item)))
      ;[1 1 1] Switch on Spawn Point
      (switch Utilities|FlowControl|Switch|SwitchonEnemySpawnPointsEnum (.enemySpawnPoint (Utilities|Struct|BreakEnemyWaveStruct (LocalVariables|GetLocWaveStruct)))
        (:Fridge
          (Variables|Default|SetspawnLocation (Variables|Default|GetSpawn_Fridge)))
        (:Microwave
          (Variables|Default|SetspawnLocation (Variables|Default|GetSpawn_Microwave)))
        (:Stove
          (Variables|Default|SetspawnLocation (Variables|Default|GetSpawn_Stove)))
        (:UpperWall
          (Variables|Default|SetspawnLocation (Variables|Default|GetSpawn_UpperWall))))
      ;[1 1 1] Get Path and check if lastPathNumber is higher than Size(-1) of pathList -> false: Set lastPathNr to Zero || -> true: Return spawnDelay
      (if (> (Variables|Default|GetlastPathNr) (- (Utilities|Array|Length (.pathList (Utilities|Struct|BreakEnemyPatternStruct (Utilities|Array|Get(acopy) (.enemyPatternList (Utilities|Struct|BreakEnemyWaveStruct (LocalVariables|GetLocWaveStruct))) _item)))) 1))
        (Variables|Default|SetlastPathNr 0))
      (return (Utilities|Array|Get(acopy) (.pathDelayList (Utilities|Struct|BreakEnemyPatternStruct (Utilities|Array|Get(acopy) (.enemyPatternList (Utilities|Struct|BreakEnemyWaveStruct (LocalVariables|GetLocWaveStruct))) _item))) (Variables|Default|GetlastPathNr)) (Utilities|Array|Get(acopy) (.pathList (Utilities|Struct|BreakEnemyPatternStruct (Utilities|Array|Get(acopy) (.enemyPatternList (Utilities|Struct|BreakEnemyWaveStruct (LocalVariables|GetLocWaveStruct))) _item))) (Variables|Default|GetlastPathNr))))))

(fn SpawnEnemy
  (params (pathStruct :type Enemy%20Path%20Struct%20Structure))
  (bind _randomprobabilitylist (Variables|Default|GetrandomProbabilityList))
  ;[1 1 1] Call SpawnObject-Function
  (Default|SpawnObject (Variables|Default|GetspawnLocation) pathStruct)
  ;[1 1 1] Increase lastPathNr and SpawnCounter (++)
  (Variables|Default|SetlastPathNr (+ (Variables|Default|GetlastPathNr) 1))
  (Variables|Default|SetSpawnCounter (+ (Variables|Default|GetSpawnCounter) 1))
  ;[1 1 1] Remove Item and check if List is empty
  (Utilities|Array|RemoveIndex _randomprobabilitylist)
  (Utilities|FlowControl|Sequence
    (:then_0
      (if (== (Utilities|Array|Length _randomprobabilitylist) 0)
        ;[1 1 1] Reset currentProjectedScore and start next wave
        (Variables|Default|SetcurrentProjectedScore 0)
        (Variables|Default|SetwaveCompleted true)))))