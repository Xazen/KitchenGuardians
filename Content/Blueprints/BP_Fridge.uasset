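; BP_Fridge is an enemy spawner that creates food enemies at its own transform when its SpawnObject function is called.
; SpawnObject maps the path struct's enemy type to one of four classes (red, green and blue fruit, or pumpkin).
; It passes BPCube, both guardians and the struct's curves, target, movement and timing settings to the spawned enemy.
; If either GuardianRice or GuardianToast is dead, it triggers BPCube's game over once instead of spawning.
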(event EventBeginPlay)

(event EventActorBeginOverlap
  (params (OtherActor :type Actor%20Object%20Reference)))

(event EventTick
  (params (DeltaSeconds :type Float%20%28single-precision%29)))

(fn ConstructionScript)

(fn SpawnObject
  (params (EnemyPathStruct :type Enemy%20Path%20Struct%20Structure))
  (bind _returnvalue (Transformation|GetActorTransform))
  (bind (_location _rotation) (Math|Transform|BreakTransform _returnvalue))
  (bind _returnvalue_2 (Math|Transform|MakeTransform _location _rotation))
  (LocalVariables|SetLocPathStruct EnemyPathStruct)
  (if (not (or (Variables|/Script/KitchenGuardians.Guardian|GetisDead (Variables|Default|GetGuardian%20Rice)) (Variables|/Script/KitchenGuardians.Guardian|GetisDead (Variables|Default|GetGuardian%20Toast))))
    (switch Utilities|FlowControl|Switch|SwitchonEnemyTypeEnum (.enemyType (Utilities|Struct|BreakEnemyPathStruct (LocalVariables|GetLocPathStruct)))
      (:Aubergine
        (bind _returnvalue_3 (Game|SpawnActorfromClass "/Game/Blueprints/BP_FruitRed.BP_FruitRed_C" _returnvalue_2 true 0))
        (Variables|/Game/Blueprints/BP_FruitRed.BP_FruitRed_C|SetBP_Cube _returnvalue_3 (Variables|Default|GetBP_Cube))
        (bind _asenemies (Utilities|Casting|CastToEnemies _returnvalue_3))
        (LocalVariables|SetLocEnemies _asenemies))
      (:Mushroom
        (bind _returnvalue_4 (Game|SpawnActorfromClass "/Game/Blueprints/BP_FruitGreen.BP_FruitGreen_C" _returnvalue_2 true 0))
        (Variables|/Game/Blueprints/BP_FruitGreen.BP_FruitGreen_C|SetBP_Cube _returnvalue_4 (Variables|Default|GetBP_Cube))
        (bind _asenemies_2 (Utilities|Casting|CastToEnemies _returnvalue_4))
        (LocalVariables|SetLocEnemies _asenemies_2))
      (:Chili
        (bind _returnvalue_5 (Game|SpawnActorfromClass "/Game/Blueprints/BP_FruitBlue.BP_FruitBlue_C" _returnvalue_2 true 0))
        (Variables|/Game/Blueprints/BP_FruitBlue.BP_FruitBlue_C|SetBP_Cube _returnvalue_5 (Variables|Default|GetBP_Cube))
        (bind _asenemies_3 (Utilities|Casting|CastToEnemies _returnvalue_5))
        (LocalVariables|SetLocEnemies _asenemies_3))
      (:Pumpkin
        (bind _returnvalue_6 (Game|SpawnActorfromClass "/Game/Blueprints/BP_Pumpkin.BP_Pumpkin_C" _returnvalue_2 true 0))
        (Variables|/Game/Blueprints/BP_Pumpkin.BP_Pumpkin_C|SetBP_Cube _returnvalue_6 (Variables|Default|GetBP_Cube))
        (bind _asenemies_4 (Utilities|Casting|CastToEnemies _returnvalue_6))
        (LocalVariables|SetLocEnemies _asenemies_4)))
    (Variables|/Script/KitchenGuardians.Enemies|SetcurveList (LocalVariables|GetLocEnemies) (.curveList (Utilities|Struct|BreakEnemyPathStruct (LocalVariables|GetLocPathStruct))))
    (Utilities|FlowControl|Sequence
      (:then_0
        (Variables|/Script/KitchenGuardians.Enemies|SetguardianRice (LocalVariables|GetLocEnemies) (Variables|Default|GetGuardian%20Rice))
        (Variables|/Script/KitchenGuardians.Enemies|SetguardianToast (LocalVariables|GetLocEnemies) (Variables|Default|GetGuardian%20Toast)))
      (:then_1
        ;[1 1 1] Set Parameters for Enemies from Enemy Path Struct
        (Variables|/Script/KitchenGuardians.Enemies|SetenemyType (LocalVariables|GetLocEnemies) (.enemyType (Utilities|Struct|BreakEnemyPathStruct (LocalVariables|GetLocPathStruct))))
        (Variables|/Script/KitchenGuardians.Enemies|SetguardianHitCaseEnum (LocalVariables|GetLocEnemies) (.targetGuardian (Utilities|Struct|BreakEnemyPathStruct (LocalVariables|GetLocPathStruct))))
        (Variables|/Script/KitchenGuardians.Enemies|SetidleTime (LocalVariables|GetLocEnemies) (.idleTime (Utilities|Struct|BreakEnemyPathStruct (LocalVariables|GetLocPathStruct))))
        (Variables|/Script/KitchenGuardians.Enemies|SetspeedFactor (LocalVariables|GetLocEnemies) (.enemySpeed (Utilities|Struct|BreakEnemyPathStruct (LocalVariables|GetLocPathStruct))))
        (Variables|/Script/KitchenGuardians.Enemies|SetenemyMoveType (LocalVariables|GetLocEnemies) (.movementType (Utilities|Struct|BreakEnemyPathStruct (LocalVariables|GetLocPathStruct))))
        (Variables|/Script/KitchenGuardians.Enemies|SetwalkingList (LocalVariables|GetLocEnemies) (.shouldWalkList (Utilities|Struct|BreakEnemyPathStruct (LocalVariables|GetLocPathStruct))))))
    (elif (not (Variables|/Script/KitchenGuardians.GameLogic|GetisGameover (Variables|Default|GetBP_Cube)))
      (Class|GameLogic|GameOver (Variables|Default|GetBP_Cube)))))