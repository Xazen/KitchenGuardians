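; Game-state actor for Kitchen Guardians that tracks score and lives and relays shots to linked bots.
; Scorred adds points to Highscore and writes the total to the scoreboard widget's field for that enemy type.
; LostLife sets a flag that Tick turns into a brief hit flash; at zero lives it saves the score, shows GameOver and hides guardian tap bars.
; EmptyShot fires Other2 or Other3 and returns its load state.
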(event EventBeginPlay
  (bind _returnvalue (UserInterface|CreateWidget "/Game/Blueprints/HUD/gotHit.gotHit_C" (Game|GetPlayerController 0)))
  (Variables|Default|SetgotHitFlash _returnvalue)
  (Widget|SetVisibility _returnvalue "Hidden")
  (UserInterface|Viewport|AddtoViewport _returnvalue 0))

(event EventActorBeginOverlap
  (params (OtherActor :type Actor%20Object%20Reference)))

(event EventTick
  (params (DeltaSeconds :type Float%20%28single-precision%29))
  (bind _gothitflash (Variables|Default|GetgotHitFlash))
  (if (Variables|Default|GetdoFlash)
    (Variables|Default|SetdoFlash false)
    (Widget|SetVisibility _gothitflash "Visible")
    (Utilities|FlowControl|Delay 0.1)
    (Widget|SetVisibility _gothitflash "Hidden")))

(fn ConstructionScript)

(fn Scorred
  (params (Points :type Integer :default 0) (enemyType :type EnemyTypeEnum%20Enum :default "NewEnumerator0"))
  (bind _output_get (Variables|Default|SetHighscore (+ (Variables|Default|GetHighscore) Points)))
  (bind _asscore (Utilities|Casting|CastToScore (UserInterface|GetUserWidgetObject (Variables|Default|GetscoreBoard))))
  (switch Utilities|FlowControl|Switch|SwitchonEnemyTypeEnum enemyType
    (:NewEnumerator0
      (Variables|/Game/Blueprints/HUD/Score.Score_C|SetscoreEnemy1 _asscore _output_get))
    (:NewEnumerator1
      (Variables|/Game/Blueprints/HUD/Score.Score_C|SetscoreEnemy2 _asscore _output_get))
    (:NewEnumerator2
      (Variables|/Game/Blueprints/HUD/Score.Score_C|SetscoreEnemy3 _asscore _output_get))))

(fn LostLife
  (bind _highscore (Variables|Default|GetHighscore))
  (Variables|Default|SetLifes (+ (Variables|Default|GetLifes) -1))
  (Variables|Default|SetdoFlash true)
  (if (== (Variables|Default|GetLifes) 0)
    (bind _returnvalue (SaveGame|DoesSaveGameExist "KitchenGuardians"))
    (if _returnvalue
      (bind _returnvalue_2 (SaveGame|LoadGamefromSlot "KitchenGuardians"))
      (bind _asbp_save_game (Utilities|Casting|CastToBP_SaveGame _returnvalue_2))
      (Class|SaveGameKitchenGuardians|SaveNewScore _asbp_save_game _highscore)
      (SaveGame|SaveGametoSlot _asbp_save_game "KitchenGuardians")
      (else
        (bind _returnvalue_3 (SaveGame|CreateSaveGameObject "/Game/Blueprints/BP_SaveGame.BP_SaveGame_C"))
        (bind _asbp_save_game_2 (Utilities|Casting|CastToBP_SaveGame _returnvalue_3))
        (Class|SaveGameKitchenGuardians|AddFirstScore _asbp_save_game_2 _highscore "Player X")
        (SaveGame|SaveGametoSlot _returnvalue_3 "KitchenGuardians")))
    (bind _returnvalue_4 (UserInterface|CreateWidget "/Game/Blueprints/HUD/GameOver.GameOver_C" (Game|GetPlayerController 0)))
    (Widget|SetVisibility _returnvalue_4 "Visible")
    (UserInterface|Viewport|AddtoViewport _returnvalue_4 0)
    (bind _asbp_main_hud (Utilities|Casting|CastToBP_MainHUD (HUD|GetHUD (Game|GetPlayerController 0))))
    (Utilities|FlowControl|Sequence
      (:then_0
        (Default|SetTapBarVisibilityforGuardian _asbp_main_hud 1 "Hidden"))
      (:then_1
        (Default|SetTapBarVisibilityforGuardian _asbp_main_hud 2 "Hidden"))
      (:then_2
        (Default|SetTapBarVisibilityforGuardian _asbp_main_hud 3 "Hidden")))))

(fn EmptyShot
  (params (Shooting%20Bot%20Case :type Integer :default 0))
  (bind _other2 (Variables|Default|Getother2))
  (bind _other3 (Variables|Default|Getother3))
  (switch int Shooting%20Bot%20Case
    (:2
      (if (Variables|/Game/Blueprints/BP_otherChar2.BP_otherChar2_C|GetActivated _other2)
        (bind _output_get (LocalVariables|Setload (Variables|/Game/Blueprints/BP_otherChar2.BP_otherChar2_C|GetcanShoot _other2)))
        (if _output_get
          (Default|Shot _other2))))
    (:3
      (if (Variables|/Game/Blueprints/BP_otherChar3.BP_otherChar3_C|GetActivated _other3)
        (LocalVariables|Setload (Variables|/Game/Blueprints/BP_otherChar3.BP_otherChar3_C|GetcanShoot _other3))
        (Default|Shot _other3))))
  (return (LocalVariables|Getload)))