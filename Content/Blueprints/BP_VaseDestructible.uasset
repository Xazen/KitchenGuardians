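; BP_VaseDestructible is a two-piece vase that topples when a BP_Knife overlaps its top or bottom mesh.
; Each mesh's overlap sets a hit flag through a DoOnce, which resets if the other part is mid-fall so only one animates at a time.
; Tick fakes the fall without physics, stepping pitch down to -90 degrees with small location offsets, then marks that part as down.
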(event `self.ReceiveBeginPlay`)

(event `self.ReceiveActorBeginOverlap`
  (params (OtherActor :type "Actor Object Reference")))

(event `self.ReceiveTick`
  (params (DeltaSeconds :type "Float (single-precision)"))
  (bind _pitch (.pitch (`SceneComponent.K2_GetComponentRotation`)))
  (bind _pitch_2 (.pitch (`SceneComponent.K2_GetComponentRotation`)))
  (if (`self.wasHittedTop`)
    (if (`self.topIsDown`)
      _
      (elif (> _pitch_2 -90.0)
        (`SceneComponent.K2_SetWorldRotation` (`KismetMathLibrary.MakeRot` (- _pitch_2 3.0) (.yaw (`SceneComponent.K2_GetComponentRotation`)) (.roll (`SceneComponent.K2_GetComponentRotation`))))
        (`SceneComponent.K2_SetWorldLocation` (`KismetMathLibrary.MakeVector` (.x (`SceneComponent.K2_GetComponentLocation`)) (.y (`SceneComponent.K2_GetComponentLocation`)) (+ (.z (`SceneComponent.K2_GetComponentLocation`)) 0.3)))
        (else
          (set `self.wasHittedTop` false)
          (set `self.topIsDown` true))))
    (elif (`self.wasHittedBottom`)
      (if (`self.bottomIsDown`)
        _
        (elif (> _pitch -90.0)
          (`SceneComponent.K2_SetWorldRotation` (`KismetMathLibrary.MakeRot` (- _pitch 3.0) (.yaw (`SceneComponent.K2_GetComponentRotation`)) (.roll (`SceneComponent.K2_GetComponentRotation`))))
          (`SceneComponent.K2_SetWorldLocation` (`KismetMathLibrary.MakeVector` (.x (`SceneComponent.K2_GetComponentLocation`)) (+ (.y (`SceneComponent.K2_GetComponentLocation`)) 0.33) (+ (.z (`SceneComponent.K2_GetComponentLocation`)) 0.2)))
          (else
            (set `self.wasHittedBottom` false)
            (set `self.bottomIsDown` true)))))))

(event `self.vaseTopMesh.OnComponentBeginOverlap`
  (params (OtherActor :type "Actor Object Reference") (OtherComp :type "PrimitiveComponent Object Reference") (OtherBodyIndex :type Integer) (bFromSweep :type Boolean) (SweepResult :type "EngineTypes.HitResult Structure (by ref)"))
  (if (== (`GameplayStatics.GetObjectClass` OtherActor) "/Game/Blueprints/BP_Knife.BP_Knife_C")
    (`/Engine/EditorBlueprintResources/StandardMacros.DoOnce` false :!label _label
      (:`Completed`
        (if (`self.wasHittedBottom`)
          (goto _label :!via `Reset`)
          (else
            (set `self.wasHittedTop` true)))))))

(event `self.vaseBottomMesh.OnComponentBeginOverlap`
  (params (OtherActor :type "Actor Object Reference") (OtherComp :type "PrimitiveComponent Object Reference") (OtherBodyIndex :type Integer) (bFromSweep :type Boolean) (SweepResult :type "EngineTypes.HitResult Structure (by ref)"))
  (if (== (`GameplayStatics.GetObjectClass` OtherActor) "/Game/Blueprints/BP_Knife.BP_Knife_C")
    (`/Engine/EditorBlueprintResources/StandardMacros.DoOnce` false :!label _label_2
      (:`Completed`
        (if (`self.wasHittedTop`)
          (goto _label_2 :!via `Reset`)
          (else
            (set `self.wasHittedBottom` true)))))))

(fn `UserConstructionScript`)