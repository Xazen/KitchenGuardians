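; BP_Ice is guardian 3, a touch-controlled character with a tap-to-revive mechanic and regenerating projectile count.
; Touching it activates it and deactivates GuardianRice and GuardianToast, with Cube2 showing the active state unless AlwaysActivated.
; During revive, taps fill a HUD bar that Tick recalculates, reviving at maximum or marking it dead at zero.
; Tick also reloads projectiles outside revive, and hits briefly flash a screen widget.
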(event `self.ReceiveTick`
  (params (DeltaSeconds :type "Float (single-precision)"))
  (if (`self.reviveIsActive`)
    (`self.calculateReviveTapCurrent` DeltaSeconds)
    (if (<= (`self.reviveTapsCurrent`) 0.0)
      (set `self.reviveTapsCurrent` 0.0)
      (set `self.isDead` true))
    (`/Game/Blueprints/Misc/BP_MainHUD.RefreshGuardianTap` (`self.mainHudRef`) 3 (`self.reviveTapsCurrent`) (`KismetMathLibrary.Conv_IntToDouble` (`self.reviveTapsMaximum`))))
  (if (not (or (`self.Always Activated`) (`self.activated`)))
    (`SceneComponent.SetVisibility` (`self.Cube2`) false false))
  (if (< (`self.projectilesCurrent`) (`self.projectilesMaximum`))
    (if (`self.Reload`)
      (if (not (`self.reviveIsActive`))
        (set `self.projectilesCurrent` (+ (`self.projectilesCurrent`) 1.0)))
      (set `self.Reload` false)
      (else
        (`KismetSystemLibrary.Delay` (`self.ReloadTime`))
        (set `self.Reload` true)))))

(event `self.ReceiveActorOnInputTouchBegin`
  (params (FingerIndex :type "InputCoreTypes.ETouchIndex Enum" :default "Touch1"))
  (if (not (`self.Always Activated`))
    (set `self.activated` true)
    (`SceneComponent.SetVisibility` (`self.Cube2`) true false)
    (set `Guardian.activated` false (`self.Guardian Rice`))
    (set `Guardian.activated` false (`self.Guardian Toast`)))
  (if (`self.reviveIsActive`)
    (bind _output_get (set `self.reviveTapsCurrent` (+ (`self.reviveTapsCurrent`) 1.0)))
    (`/Game/Blueprints/Misc/BP_MainHUD.RefreshGuardianTap` (`self.mainHudRef`) 3 _output_get (`KismetMathLibrary.Conv_IntToDouble` (`self.reviveTapsMaximum`)))
    (if (>= _output_get (`KismetMathLibrary.Conv_IntToDouble` (`self.reviveTapsMaximum`)))
      (`/Game/Blueprints/Misc/BP_MainHUD.SetTapBarVisibilityForGuardian` (`self.mainHudRef`) 3 "Hidden")
      (`self.Revive`))))

(event `self.ReceiveBeginPlay`
  (if (`self.Always Activated`)
    (`SceneComponent.SetVisibility` (`self.Cube2`) true false))
  (bind _returnvalue (`|CreateWidget` "/Game/Blueprints/HUD/gotHit.gotHit_C" (`GameplayStatics.GetPlayerController` 0)))
  (set `self.gotHitFlash` _returnvalue)
  (`Widget.SetVisibility` _returnvalue "Hidden")
  (`UserWidget.AddToViewport` _returnvalue 0)
  (bind _asbp_main_hud (cast `/Game/Blueprints/Misc/BP_MainHUD` (`PlayerController.GetHUD` (`GameplayStatics.GetPlayerController` 0))))
  (bind _output_get (set `self.mainHudRef` _asbp_main_hud))
  (`/Game/Blueprints/Misc/BP_MainHUD.SetTapBarVisibilityForGuardian` _output_get 3 "Hidden"))

(event `self.InitRevive`
  (bind _mainhudref (`self.mainHudRef`))
  (`/Game/Blueprints/Misc/BP_MainHUD.SetTapBarVisibilityForGuardian` _mainhudref 3 "Visible")
  (bind _output_get (set `self.reviveTapsCurrent` (`KismetMathLibrary.Conv_IntToDouble` (`self.reviveTapsStart`))))
  (`/Game/Blueprints/Misc/BP_MainHUD.RefreshGuardianTap` _mainhudref 3 _output_get (`KismetMathLibrary.Conv_IntToDouble` (`self.reviveTapsMaximum`))))

(event `self.GotHitFeedback`
  (bind _gothitflash (`self.gotHitFlash`))
  (`Widget.SetVisibility` _gothitflash "Visible")
  (`KismetSystemLibrary.Delay` 0.1)
  (`Widget.SetVisibility` _gothitflash "Hidden"))

(fn `UserConstructionScript`)