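; BP_Vegetable is a touch-targeted enemy that travels a waypoint path, costing the Ricebot a life and destroying itself at the end.
; Tick moves it in a straight line at a frame-rate-scaled speed, advancing waypoints by a squared-distance check.
; Touching it calls SpawnKnife, which, while Veghits remain, decrements them and launches a BP_Knife from KnifeSpawn toward this vegetable.
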(event `self.ReceiveActorOnInputTouchBegin`
  (params (FingerIndex :type "InputCoreTypes.ETouchIndex Enum" :default "Touch1"))
  (`self.SpawnKnife`))

(event `self.ReceiveActorBeginOverlap`
  (params (OtherActor :type "Actor Object Reference")))

(event `self.ReceiveTick`
  (params (DeltaSeconds :type "Float (single-precision)"))
  (bind _location (.location (`self.GetTransform`)))
  (bind _returnvalue (`self.K2_GetActorLocation` (`KismetArrayLibrary.Array_Get` (`self.Waypoints`) (`self.Waypoint_Int`))))
  (if true
    (if (<= (`KismetMathLibrary.VSizeSquared` (- _location _returnvalue)) 100.0)
      (bind _output_get (set `self.Waypoint_Int` (+ (`self.Waypoint_Int`) 1)))
      (if (== _output_get (`KismetArrayLibrary.Array_Length` (`self.Waypoints`)))
        (`/Game/Blueprints/BP_Cube.LostLife` (`self.Ricebot`))
        (`self.K2_DestroyActor`)
        (else
          (`self.K2_SetActorTransform` (`KismetMathLibrary.MakeTransform` (+ _location (* (`KismetMathLibrary.Normal` (`KismetMathLibrary.GetDirectionVector` _location _returnvalue)) (* (`self.Speed`) (* DeltaSeconds 260.0)))) (.rotation (`self.GetTransform`)) (.scale (`self.GetTransform`))) :!label _label)))
      (else
        (goto _label)))))

(fn `GetVector`
  (returns (NewParam :type "Object.Vector Structure"))
  (return (`SceneComponent.K2_GetComponentLocation`)))

(fn `SpawnKnife`
  (if (> (`self.veghits`) 0)
    (set `self.veghits` (+ (`self.veghits`) -1))
    (if (== (`self.Hitpoints`) 0)
      (set `self.loaded` false))
    (bind _returnvalue (`|SpawnActorFromClass` "/Game/Blueprints/BP_Knife.BP_Knife_C" (`self.KnifeSpawn`) true))
    (`/Game/Blueprints/BP_Knife.MoveTowards` _returnvalue self (`self.RiceBot`))))

(fn `UserConstructionScript`)