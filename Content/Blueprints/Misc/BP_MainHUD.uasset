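; Main HUD Blueprint for Kitchen Guardian that manages the flow from bootup screen to in-game UI.
; BeginPlay reads the save game: a restart plays a timed black fade, clears the flag and sets StartGame; otherwise it shows the Bootup widget.
; Once StartGame is true, Tick creates GameUI once (fading first if not already done), flags ReadyToStart and restores the UI's visibility from hidden or non-hit-testable states.
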(event `self.ReceiveBeginPlay`
  (set `self.readyToStart` false)
  (`|ExecutionSequence`
    (:`then_0`
      (bind _returnvalue (`GameplayStatics.DoesSaveGameExist` "KitchenGuardian"))
      (if _returnvalue
        (bind _returnvalue_2 (`GameplayStatics.LoadGameFromSlot` "KitchenGuardian"))
        (bind _assave_game_kitchen_guardian (cast `SaveGameKitchenGuardian` _returnvalue_2))
        (if (`SaveGameKitchenGuardian.wasRestart` _assave_game_kitchen_guardian)
          (set `self.blackBufferWasActive` true)
          (bind _returnvalue_3 (`|CreateWidget` "/Game/Blueprints/HUD/FadeBlack.FadeBlack_C" (`self.GetOwningPlayerController`)))
          (`UserWidget.AddToViewport` _returnvalue_3 2)
          (`KismetSystemLibrary.Delay` 2.0)
          (`/Game/Blueprints/HUD/FadeBlack.Fade Out` _returnvalue_3)
          (`KismetSystemLibrary.Delay` 1.0)
          (`Widget.RemoveFromParent` _returnvalue_3)
          (set `SaveGameKitchenGuardian.wasRestart` false _assave_game_kitchen_guardian)
          (`GameplayStatics.SaveGameToSlot` _assave_game_kitchen_guardian "KitchenGuardian")
          (set `self.startGame` true)
          (else
            (bind _returnvalue_4 (`|CreateWidget` "/Game/Blueprints/HUD/Bootup.Bootup_C" (`GameplayStatics.GetPlayerController` 0) :!label _label))
            (`UserWidget.AddToViewport` _returnvalue_4 1)))
        (else
          (goto _label))))
    (:`then_1`
      (bind _outactors (`GameplayStatics.GetAllActorsOfClass` "/Game/Blueprints/BP_Cube.BP_Cube_C"))
      (set `self.soundCubeRef` (`KismetArrayLibrary.Array_Get` _outactors)))))

(event `self.ReceiveTick`
  (params (DeltaSeconds :type "Float (single-precision)"))
  (bind _gameuiref (`self.gameUIRef`))
  (if (`self.startGame`)
    (`|ExecutionSequence`
      (:`then_0`
        (`/Engine/EditorBlueprintResources/StandardMacros.DoOnce` false
          (:`Completed`
            (if (not (`self.blackBufferWasActive`))
              (bind _returnvalue (`|CreateWidget` "/Game/Blueprints/HUD/FadeBlack.FadeBlack_C" (`self.GetOwningPlayerController`)))
              (`UserWidget.AddToViewport` _returnvalue 2)
              (`KismetSystemLibrary.Delay` 2.0)
              (`/Game/Blueprints/HUD/FadeBlack.Fade Out` _returnvalue)
              (`KismetSystemLibrary.Delay` 1.0)
              (`Widget.RemoveFromParent` _returnvalue))
            (bind _returnvalue_2 (`|CreateWidget` "/Game/Blueprints/HUD/GameUI.GameUI_C" (`GameplayStatics.GetPlayerController` 0)))
            (set `self.gameUIRef` _returnvalue_2)
            (`UserWidget.AddToViewport` _returnvalue_2 1)
            (set `self.readyToStart` true))))
      (:`then_1`
        (`/Engine/EditorBlueprintResources/StandardMacros.IsValid` _gameuiref
          (:`Is Valid`
            (switch `ESlateVisibility` (`Widget.GetVisibility` _gameuiref)
              (:`Hidden`
                _)
              (:`HitTestInvisible`
                _)
              (:`SelfHitTestInvisible`
                _))
            (`Widget.SetVisibility` _gameuiref "Visible")))))))

(event `self.ReceiveActorBeginOverlap`
  (params (OtherActor :type "Actor Object Reference")))

(fn `UserConstructionScript`)