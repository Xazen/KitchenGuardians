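; Tutorial mushroom that plays feedback when hit or killed by rice, active only when its OnlySwipe flag is set.
; A hit spawns green fruit particles and sound and pauses movement briefly.
; Death destroys the skeletal mesh, then reveals head and body giblets gathered in the construction script, launches them with physics impulses and destroys the actor after a delay.
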(event `self.GotHitRiceFeedback`
  (bind _returnvalue (`self.K2_GetActorLocation`))
  (if (`self.onlySwipe`)
    (set `self.canMove` false)
    (`GameplayStatics.SpawnEmitterAtLocation` "/Game/VFX/Particles/PS_FruitGreen.PS_FruitGreen" _returnvalue)
    (`GameplayStatics.PlaySoundAtLocation` "/Game/Audio/SFX/Placeholder/fruitHit.fruitHit" _returnvalue)
    (`|ExecutionSequence`
      (:`then_1`
        ;[1 1 1] Stop movement for 400 Milliseconds
        (`KismetSystemLibrary.Delay` 0.4)
        (if (not (`self.willDie`))
          (set `self.canMove` true))))))

(event `self.diedRiceFeedback`
  (bind _returnvalue (`self.K2_GetActorLocation`))
  (if (`self.onlySwipe`)
    (set `self.willDie` true)
    (set `self.canMove` false)
    (`GameplayStatics.SpawnEmitterAtLocation` "/Game/VFX/Particles/PS_FruitGreen.PS_FruitGreen" _returnvalue)
    (`GameplayStatics.PlaySoundAtLocation` "/Game/Audio/SFX/Placeholder/fruitDestroy.fruitDestroy" _returnvalue)
    (`ActorComponent.K2_DestroyComponent` (`self.SkeletalMesh`))
    (if (> (`KismetArrayLibrary.Array_Length` (`self.gibletList`)) 0)
      ;[1 1 1] Giblet Activation and Add Impulse
      (for _array_element (`self.gibletList`)
        (`SceneComponent.SetVisibility` _array_element true false)
        (`PrimitiveComponent.SetSimulatePhysics` _array_element true)
        (`self.AddGibbletImpulse2` _array_element))
      (`KismetSystemLibrary.Delay` 2.5)
      (`self.K2_DestroyActor`))))

(fn `UserConstructionScript`
  (bind _gibletlist (`self.gibletList`))
  (`/Engine/EditorBlueprintResources/StandardMacros.DoOnce` false
    (:`Completed`
      (`KismetArrayLibrary.Array_Add` _gibletlist (`self.GibletHead`))
      (`KismetArrayLibrary.Array_Add` _gibletlist (`self.GibletBody`)))))