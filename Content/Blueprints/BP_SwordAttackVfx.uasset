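; BP_SwordAttackVfx is a sword attack projectile that homes in on a target and plays a camera shake and particle burst on impact.
; Tick moves it toward the target's first static mesh while that enemy is alive, otherwise toward an empty location.
; On losing the target, a line trace along its travel direction sets that location.
; Enemy overlap, reaching the empty point or a long BeginPlay timeout destroys it.
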(event `self.Cube.OnComponentBeginOverlap`
  (params (OtherActor :type "Actor Object Reference") (OtherComp :type "PrimitiveComponent Object Reference") (OtherBodyIndex :type Integer) (bFromSweep :type Boolean) (SweepResult :type "EngineTypes.HitResult Structure (by ref)"))
  (cast `Enemies` OtherActor
    (:`then`
      (`self.Impact Feedback`)
      (`self.K2_DestroyActor`))
    (:`CastFailed`
      (cast `AlterableObject` OtherActor)
      (`KismetSystemLibrary.PrintString` (`KismetSystemLibrary.GetDisplayName` OtherActor)))))

(event `Impact Feedback`
  (`PlayerController.ClientStartCameraShake` :`self` (`GameplayStatics.GetPlayerController` 0) :`Shake` "/Game/Blueprints/BP_ScreenShake.BP_ScreenShake_C" :`Scale` 0.5)
  (`GameplayStatics.SpawnEmitterAtLocation` "/Game/VFX/Particles/PS_Placeholder.PS_Placeholder" (.location (`self.GetTransform`)) (.rotation (`self.GetTransform`))))

(event `self.ReceiveBeginPlay`
  (set `self.StartPosition` (`self.K2_GetActorLocation`))
  (`KismetSystemLibrary.Delay` 200.0)
  (`KismetSystemLibrary.PrintString` "time destroy -inform oelke")
  (`self.Impact Feedback`)
  (`self.K2_DestroyActor`))

(event `self.ReceiveTick`
  (params (DeltaSeconds :type "Float (single-precision)"))
  (bind _targ (`self.targ`))
  (bind _emptylocation (`self.EmptyLocation`))
  (bind _location (.location (`self.GetTransform`)))
  (bind _location_2 (.location (`self.GetTransform`)))
  (bind _returnvalue (* DeltaSeconds (`self.KnifeTapSpeed`)))
  (if (`self.empty`)
    (`self.K2_SetActorTransform` (`KismetMathLibrary.MakeTransform` (+ _location (* (`KismetMathLibrary.Normal` (`KismetMathLibrary.GetDirectionVector` _location _emptylocation)) _returnvalue)) (.rotation (`self.GetTransform`)) (.scale (`self.GetTransform`))) :!label _label)
    (if (<= (`KismetMathLibrary.VSizeSquared` (- _emptylocation _location)) 200.0)
      (`self.Impact Feedback`)
      (`self.K2_DestroyActor`))
    (else
      (bind _asenemies (cast `Enemies` _targ)
        (:`then`
          _)
        (:`CastFailed`
          _))
      (if (and (`KismetSystemLibrary.IsValid` _targ) (> (`Enemies.hitPoints` _asenemies) 0))
        (`self.K2_SetActorTransform` (`KismetMathLibrary.MakeTransform` (+ _location_2 (* (`KismetMathLibrary.Normal` (`KismetMathLibrary.GetDirectionVector` _location_2 (`SceneComponent.K2_GetComponentLocation` (`KismetArrayLibrary.Array_Get` (`self.K2_GetComponentsByClass` (`self.targ`) "/Script/Engine.StaticMeshComponent"))))) _returnvalue)) (.rotation (`self.GetTransform`)) (.scale (`self.GetTransform`))))
        (else
          (`self.switchToEmpty`)
          (goto _label))))))

(fn `MoveTowards`
  (params (Target :type "Actor Object Reference") (RiceBot :type "/Game/Blueprints/BP_Cube Object Reference") (IsEmpty :type Boolean :default false))
  (set `self.BP_Cube` RiceBot)
  (set `self.targ` Target)
  (if IsEmpty
    (set `self.empty` true)))

(fn `switchToEmpty`
  (bind _returnvalue (`self.K2_GetActorLocation`))
  (bind _outhit (`KismetSystemLibrary.LineTraceSingle` _returnvalue (+ _returnvalue (* (`KismetMathLibrary.GetDirectionVector` (`self.StartPosition`) _returnvalue) 50000.0)) "TraceTypeQuery1" true))
  (set `self.EmptyLocation` (`.ImpactPoint` (`GameplayStatics.BreakHitResult` _outhit)))
  (set `self.empty` true))

(fn `UserConstructionScript`)