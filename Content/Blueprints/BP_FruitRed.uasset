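; BP_FruitRed is a red fruit enemy that moves and rotates along a spline and awards score when killed.
; Tick drives movement and a drop shadow, whose height comes from overlapped collider actors and whose alpha follows mesh height.
; Rice and toast hits share feedback: effects, a brief stop and a burned-material flash if the toaster's Reload is set.
; Death swaps the mesh for physics giblets, then destroys the actor after a delay.
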(event `self.ReceiveTick`
  (params (DeltaSeconds :type "Float (single-precision)"))
  (bind _dropshadowzvalue (`self.dropShadowZValue`))
  (bind _dropshadow (`self.dropShadow`))
  (`/Engine/EditorBlueprintResources/StandardMacros.IsValid` self
    (:`Is Valid`
      (if (`self.bAutoDestroyWhenFinished`)
        _
        (elif (`self.staticEnemy`)
          _
          (elif (`self.canMove`)
            (`self.MoveEnemyAlongSpline`)
            (`self.Rotate` DeltaSeconds)
            (`self.CalculateDistancePercentage` DeltaSeconds)
            (bind _returnvalue (`self.CheckDistancePercentage`))
            ;[1 1 1] shadow
            (if (> _dropshadowzvalue -1.0)
              (`SceneComponent.K2_SetWorldLocation` _dropshadow (`KismetMathLibrary.MakeVector` (.x (`SceneComponent.K2_GetComponentLocation` _dropshadow)) (.y (`SceneComponent.K2_GetComponentLocation` _dropshadow)) _dropshadowzvalue) false)
              (bind _returnvalue_2 (`self.calcDropShadowAlpha` (- (.z (`SceneComponent.K2_GetComponentLocation` (`self.SkeletalMesh`))) (`self.dropShadowZValue`))))
              (set `self.dropShadowAlpha` _returnvalue_2)
              (`PaperSpriteComponent.SetSpriteColor` (`self.dropShadow`) (`KismetMathLibrary.MakeColor` 1.0 1.0 1.0 (`self.dropShadowAlpha`)))
              (if _returnvalue
                (set `self.bAutoDestroyWhenFinished` true)))))))))

(event `self.hitToastFeedback`
  (`self.K2_DestroyActor`))

(event `self.GotHitRiceFeedback`
  (bind _returnvalue (`self.K2_GetActorLocation`))
  (bind _skeletalmesh (`self.SkeletalMesh`))
  (bind _skeletalmesh_2 (`self.SkeletalMesh`))
  (set `self.canMove` false :!label _label)
  (`GameplayStatics.SpawnEmitterAtLocation` "/Game/VFX/Particles/PS_FruitRed.PS_FruitRed" _returnvalue)
  (`GameplayStatics.PlaySoundAtLocation` "/Game/Audio/SFX/fruitHit.fruitHit" _returnvalue)
  (`|ExecutionSequence`
    (:`then_0`
      ;[1 1 1] Toaster hit Enemy
      (bind _asbp_toast (cast `/Game/Blueprints/BP_Toast` (`self.guardianToast`)))
      (if (`/Game/Blueprints/BP_Toast.Reload` _asbp_toast)
        (`GameplayStatics.SpawnEmitterAtLocation` "/Game/VFX/Particles/PS_Placeholder.PS_Placeholder")
        (`PrimitiveComponent.SetMaterial` _skeletalmesh_2 0 "/Game/Materials/Burned/BurnedAubergine.BurnedAubergine")
        (`PrimitiveComponent.SetMaterial` _skeletalmesh_2 1 "/Game/Materials/Burned/BurnedAubergine.BurnedAubergine")
        (`PrimitiveComponent.SetMaterial` _skeletalmesh_2 2 "/Game/Materials/Burned/BurnedAubergine.BurnedAubergine")
        (`KismetSystemLibrary.Delay` 0.5)
        (`PrimitiveComponent.SetMaterial` _skeletalmesh 0 "/Game/Animations/Placeholder/chili_hat.chili_hat")
        (`PrimitiveComponent.SetMaterial` _skeletalmesh 1 "/Game/Animations/Placeholder/chili_repaint.chili_repaint")
        (`PrimitiveComponent.SetMaterial` _skeletalmesh 2 "/Game/Animations/Placeholder/chili_moustache.chili_moustache")))
    (:`then_1`
      ;[1 1 1] Stop movement for 400 Milliseconds
      (`KismetSystemLibrary.Delay` 0.4)
      (if (not (`self.willDie`))
        (set `self.canMove` true)))))

(event `self.GotHitToastFeedback`
  (goto _label))

(event `self.diedRiceFeedback`
  (bind _returnvalue (`self.K2_GetActorLocation`))
  (set `self.willDie` true :!label _label_2)
  (set `self.canMove` false)
  (`GameplayStatics.SpawnEmitterAtLocation` "/Game/VFX/Particles/PS_FruitRed.PS_FruitRed" _returnvalue)
  (`GameplayStatics.PlaySoundAtLocation` "/Game/Audio/SFX/fruitDestroy.fruitDestroy" _returnvalue)
  (`/Game/Blueprints/BP_Cube.Scorred` (`self.BP_Cube`) (`self.baseScore`) (`self.enemyType`))
  (`ActorComponent.K2_DestroyComponent` (`self.SkeletalMesh`))
  (`ActorComponent.K2_DestroyComponent` (`self.dropShadow`))
  (`ActorComponent.K2_DestroyComponent` (`self.shadowTester`))
  ;[1 1 1] Giblet Activation and Add Impulse
  (for _array_element (`self.gibletList`)
    (`SceneComponent.SetVisibility` _array_element true false)
    (`PrimitiveComponent.SetSimulatePhysics` _array_element true)
    (`self.AddGibbletImpulse2` _array_element))
  (`KismetSystemLibrary.Delay` 2.5)
  (`self.K2_DestroyActor`))

(event `self.shadowTester.OnComponentBeginOverlap`
  (params (OtherActor :type "Actor Object Reference") (OtherComp :type "PrimitiveComponent Object Reference") (OtherBodyIndex :type Integer) (bFromSweep :type Boolean) (SweepResult :type "EngineTypes.HitResult Structure (by ref)"))
  (bind _dropshadow (`self.dropShadow`))
  ;[1 1 1] shadow
  (bind _asbp_drop_shadow_collider (cast `/Game/Blueprints/BP_DropShadow_Collider` OtherActor))
  (set `self.dropShadowZValue` (`/Game/Blueprints/BP_DropShadow_Collider.objectZ` _asbp_drop_shadow_collider))
  (`SceneComponent.K2_SetWorldLocation` _dropshadow (`KismetMathLibrary.MakeVector` (.x (`SceneComponent.K2_GetComponentLocation` _dropshadow)) (.y (`SceneComponent.K2_GetComponentLocation` _dropshadow)) (`self.dropShadowZValue`)) false)
  (`SceneComponent.SetVisibility` _dropshadow true false))

(event `self.diedToastFeedback`
  (goto _label_2))

(event `self.shadowTester.OnComponentEndOverlap`
  (params (OtherActor :type "Actor Object Reference") (OtherComp :type "PrimitiveComponent Object Reference") (OtherBodyIndex :type Integer))
  ;[1 1 1] shadow
  (cast `/Game/Blueprints/BP_DropShadow_Collider` OtherActor)
  (`SceneComponent.SetVisibility` (`self.dropShadow`) false false))

(fn `UserConstructionScript`
  (bind _gibletlist (`self.gibletList`))
  (`/Engine/EditorBlueprintResources/StandardMacros.DoOnce` false
    (:`Completed`
      (`KismetArrayLibrary.Array_Add` _gibletlist (`self.Giblet01`))
      (`KismetArrayLibrary.Array_Add` _gibletlist (`self.Giblet02`))
      (`KismetArrayLibrary.Array_Add` _gibletlist (`self.Giblet03`))
      (`KismetArrayLibrary.Array_Add` _gibletlist (`self.Giblet04`)))))