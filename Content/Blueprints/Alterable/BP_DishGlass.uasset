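; BP_DishGlass is a breakable glass dish actor that shatters when an enemy or knife overlaps its box.
; Enemies always trigger the break, while a BP_Knife triggers it only if the overlapping component's name lacks "AoESphere", filtering out the knife's area-of-effect.
; Breaking plays a smash sound at a random pitch, spawns a glass particle effect and destroys the actor.
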(event `self.ReceiveBeginPlay`)

(event `self.ReceiveActorBeginOverlap`
  (params (OtherActor :type "Actor Object Reference")))

(event `self.ReceiveTick`
  (params (DeltaSeconds :type "Float (single-precision)")))

(event `self.Box.OnComponentBeginOverlap`
  (params (OtherActor :type "Actor Object Reference") (OtherComp :type "PrimitiveComponent Object Reference") (OtherBodyIndex :type Integer) (bFromSweep :type Boolean) (SweepResult :type "HitResult Structure (by ref)"))
  (bind _returnvalue (`self.K2_GetActorLocation`))
  (cast `Enemies` OtherActor
    (:`then`
      (`GameplayStatics.PlaySoundAtLocation` "/Game/Audio/SFX/firstIteration/Environment/glass_plate_smash.glass_plate_smash" _returnvalue (struct) 1.0 (`KismetMathLibrary.RandomFloatInRange` 1.0 1.4) :!label _label)
      (`GameplayStatics.SpawnEmitterAtLocation` "/Game/VFX/Particles/test/P_GlassDishes.P_GlassDishes" _returnvalue)
      (`self.K2_DestroyActor`))
    (:`CastFailed`
      (if (and (== (`GameplayStatics.GetObjectClass` OtherActor) "/Game/Blueprints/BP_Knife.BP_Knife_C") (== (`KismetStringLibrary.FindSubstring` (`KismetSystemLibrary.GetDisplayName` OtherComp) "AoESphere") -1))
        (goto _label)))))

(fn `UserConstructionScript`)