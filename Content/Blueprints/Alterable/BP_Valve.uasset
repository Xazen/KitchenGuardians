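; BP_Valve is a valve actor that releases steam when hit by a BP_Knife.
; Its Box overlap filters out the knife's AoE sphere by component display name, then activates the Steam component and plays a release sound at the actor's location.
; A DoOnce gate blocks retriggering until the steam deactivates after a timed delay and a short cooldown passes.
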(event `self.ReceiveActorBeginOverlap`
  (params (OtherActor :type "Actor Object Reference")))

(event `self.ReceiveTick`
  (params (DeltaSeconds :type "Float (single-precision)")))

(event `self.Box.OnComponentBeginOverlap`
  (params (OtherActor :type "Actor Object Reference") (OtherComp :type "PrimitiveComponent Object Reference") (OtherBodyIndex :type Integer) (bFromSweep :type Boolean) (SweepResult :type "EngineTypes.HitResult Structure (by ref)"))
  (if (and (== (`GameplayStatics.GetObjectClass` OtherActor) "/Game/Blueprints/BP_Knife.BP_Knife_C") (== (`KismetStringLibrary.FindSubstring` (`KismetSystemLibrary.GetDisplayName` OtherComp) "AoESphere") -1))
    (`/Engine/EditorBlueprintResources/StandardMacros.DoOnce` false :!label _label
      (:`Completed`
        (`ActorComponent.Activate` (`self.Steam`) false)
        (`GameplayStatics.PlaySoundAtLocation` "/Game/Audio/SFX/firstIteration/Environment/valveReleaseSFX5_5sec.valveReleaseSFX5_5sec" (`self.K2_GetActorLocation`))
        (`KismetSystemLibrary.Delay` 5.1)
        (`ActorComponent.Deactivate` (`self.Steam`))
        (`KismetSystemLibrary.Delay` 1.0)
        (goto _label :!via `Reset`)))))

(fn `UserConstructionScript`)