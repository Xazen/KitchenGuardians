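; Breakable window glass actor that cracks under knife hits and shatters when a living enemy touches it.
; A dynamic material instance shows three crack stages, advanced by chained DoOnce gates with short reset delays between knife hits.
; An enemy overlap swaps the whole mesh for the broken one and sets IsBroken, ending knife reactions.
; Impacts play smash sounds, randomized for knife hits, and spawn placeholder particles.
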(event `self.ReceiveBeginPlay`
  (bind _returnvalue (`PrimitiveComponent.CreateDynamicMaterialInstance` (`self.WindowGlasWhole`) 0 "/Game/Meshes/Window/Window_Glass_Inst.Window_Glass_Inst"))
  (set `self.GlassMaterial` _returnvalue))

(event `windowHitSound`
  (`GameplayStatics.PlaySoundAtLocation` "/Game/Audio/SFX/firstIteration/Environment/windowSmash.windowSmash" (`self.K2_GetActorLocation`) (`KismetMathLibrary.RandomFloatInRange` 0.9 1.1) (`KismetMathLibrary.RandomFloatInRange` 0.7 1.3)))

(event `self.ReceiveActorBeginOverlap`
  (params (OtherActor :type "Actor Object Reference")))

(event `self.ReceiveTick`
  (params (DeltaSeconds :type "Float (single-precision)")))

(event `self.BoxCollision.OnComponentBeginOverlap`
  (params (OtherActor :type "Actor Object Reference") (OtherComp :type "PrimitiveComponent Object Reference") (OtherBodyIndex :type Integer) (bFromSweep :type Boolean) (SweepResult :type "EngineTypes.HitResult Structure (by ref)"))
  (bind _asbp_knife (cast `/Game/Blueprints/BP_Knife` OtherActor)
    (:`then`
      (if (not (`self.isBroken`))
        (`|ExecutionSequence`
          (:`then_0`
            (`/Engine/EditorBlueprintResources/StandardMacros.DoOnce` true :!label _label
              (:`Completed`
                (`self.windowHitSound`)
                (`GameplayStatics.SpawnEmitterAtLocation` "/Game/VFX/Particles/PS_Placeholder.PS_Placeholder" (`self.K2_GetActorLocation`))
                (`MaterialInstanceDynamic.SetScalarParameterValue` (`self.GlassMaterial`) "Broken_03" 1.0))))
          (:`then_1`
            (`/Engine/EditorBlueprintResources/StandardMacros.DoOnce` true :!label _label_2
              (:`Completed`
                (`self.windowHitSound`)
                (`GameplayStatics.SpawnEmitterAtLocation` "/Game/VFX/Particles/PS_Placeholder.PS_Placeholder" (`self.K2_GetActorLocation` _asbp_knife))
                (`MaterialInstanceDynamic.SetScalarParameterValue` (`self.GlassMaterial`) "Broken_02" 1.0)
                (`KismetSystemLibrary.Delay` 0.6)
                (goto _label :!via `Reset`))))
          (:`then_2`
            (`/Engine/EditorBlueprintResources/StandardMacros.DoOnce` false
              (:`Completed`
                (`self.windowHitSound`)
                (`GameplayStatics.SpawnEmitterAtLocation` "/Game/VFX/Particles/PS_Placeholder.PS_Placeholder" (`self.K2_GetActorLocation` _asbp_knife))
                (`MaterialInstanceDynamic.SetScalarParameterValue` (`self.GlassMaterial`) "Broken_01" 1.0)
                (`KismetSystemLibrary.Delay` 0.6)
                (goto _label_2 :!via `Reset`)))))))
    (:`CastFailed`
      (bind _asenemies (cast `Enemies` OtherActor))
      (if (> (`Enemies.hitPoints` _asenemies) 0)
        (`/Engine/EditorBlueprintResources/StandardMacros.DoOnce` false
          (:`Completed`
            (`SceneComponent.SetVisibility` (`self.WondGlassBroken`) true false)
            (set `self.isBroken` true)
            (`SceneComponent.SetVisibility` (`self.WindowGlasWhole`) false false)
            (bind _returnvalue (`self.K2_GetActorLocation` _asenemies))
            (`GameplayStatics.PlaySoundAtLocation` "/Game/Audio/SFX/firstIteration/Environment/windowSmash.windowSmash" _returnvalue)
            (`GameplayStatics.SpawnEmitterAtLocation` "/Game/VFX/Particles/PS_Placeholder.PS_Placeholder" _returnvalue)))))))

(fn `UserConstructionScript`)