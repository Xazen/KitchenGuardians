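; BP_ScreenFlash is a Blueprint that flashes the screen through a ScreenSplash widget, created and added to the viewport on BeginPlay.
; Overlapping its Collision component with an Enemies actor at zero HitPoints fires the flash through a DoOnce gate.
; The gate resets after a delay, throttling repeat flashes.
; Pressing F triggers the same flash-and-reset chain directly, bypassing the gate.
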(event `self.ReceiveBeginPlay`
  (bind _returnvalue (`|CreateWidget` "/Game/Blueprints/HUD/ScreenSplash.ScreenSplash_C" (`GameplayStatics.GetPlayerController` 0)))
  (bind _output_get (set `self.ScreenSplash` _returnvalue))
  (`UserWidget.AddToViewport` _output_get 0))

(event `self.ReceiveActorBeginOverlap`
  (params (OtherActor :type "Actor Object Reference")))

(event `self.ReceiveTick`
  (params (DeltaSeconds :type "Float (single-precision)")))

(event `Key|F`
  (:`Pressed`
    (`/Game/Blueprints/HUD/ScreenSplash.ScreenFlash` (`self.ScreenSplash`) :!label _label)
    (`KismetSystemLibrary.Delay` 6.0)
    (goto _label_2 :!via `Reset`)))

(event `self.Collision.OnComponentBeginOverlap`
  (params (OtherActor :type "Actor Object Reference") (OtherComp :type "PrimitiveComponent Object Reference") (OtherBodyIndex :type Integer) (bFromSweep :type Boolean) (SweepResult :type "EngineTypes.HitResult Structure (by ref)"))
  (bind _asenemies (cast `Enemies` OtherActor))
  (if (== (`Enemies.hitPoints` _asenemies) 0)
    (`/Engine/EditorBlueprintResources/StandardMacros.DoOnce` false :!label _label_2
      (:`Completed`
        (goto _label)))))

(fn `UserConstructionScript`)