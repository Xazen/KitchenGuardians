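; Fridge prop that bursts open with cold effects when a living enemy touches its trigger volume.
; The first touch makes the door simulate physics, plays a clatter sound and activates the spawn fog and a physics thruster.
; Touches also activate a blizzard effect, throttled by a one-second DoOnce.
; OnReset deactivates the effects and thruster but leaves the door and one-shot gate as they are; the saved start transform is unused here.
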(event `self.ReceiveBeginPlay`
  (if (not (`self.firstStart`))
    (set `self.startPosition` (`self.K2_GetActorLocation`))
    (set `self.startRotation` (`self.K2_GetActorRotation`))
    (set `self.firstStart` true)))

(event `self.EnemyTouchTest.OnComponentBeginOverlap`
  (params (OtherActor :type "Actor Object Reference") (OtherComp :type "PrimitiveComponent Object Reference") (OtherBodyIndex :type Integer) (bFromSweep :type Boolean) (SweepResult :type "HitResult Structure (by ref)"))
  (bind _asenemies (cast `Enemies` OtherActor))
  (if (> (`Enemies.hitPoints` _asenemies) 0)
    (`|ExecutionSequence`
      (:`then_0`
        (`/Engine/EditorBlueprintResources/StandardMacros.DoOnce` false
          (:`Completed`
            (`PrimitiveComponent.SetSimulatePhysics` (`self.FridgeDoor`) true)
            ;[1 1 1] Play Clatter Sound
            (`GameplayStatics.PlaySoundAtLocation` "/Game/Audio/SFX/firstIteration/Environment/cuppboardHit2.cuppboardHit2" (`SceneComponent.K2_GetComponentLocation`))
            (`ActorComponent.Activate` (`self.P_SpawnFog`) false)
            (`ActorComponent.Activate` (`self.PhysicsThruster`) false))))
      (:`then_1`
        (`/Engine/EditorBlueprintResources/StandardMacros.DoOnce` false :!label _label
          (:`Completed`
            (`ActorComponent.Activate` (`self.P_Blizzard`) false)
            (`KismetSystemLibrary.Delay` 1.0)
            (goto _label :!via `Reset`)))))))

(event `self.K2_OnReset`
  ;[1 1 1] Reset functionality
  (`ActorComponent.Deactivate` (`self.P_Blizzard`))
  (`ActorComponent.Deactivate` (`self.P_SpawnFog`))
  (`ActorComponent.Deactivate` (`self.PhysicsThruster`)))

(fn `UserConstructionScript`)