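; Lower-wall cupboard whose door breaks loose when struck by a BP_Knife.
; On door mesh overlap, it filters out the knife's AoESphere component by display-name substring, so area effects do not trigger it.
; A valid hit turns on physics simulation for the door and uses a DoOnce node around playing a clatter sound at the door's location.
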(event `self.DoorMesh.OnComponentBeginOverlap`
  (params (OtherActor :type "Actor Object Reference") (OtherComp :type "PrimitiveComponent Object Reference") (OtherBodyIndex :type Integer) (bFromSweep :type Boolean) (SweepResult :type "EngineTypes.HitResult Structure (by ref)"))
  (bind _doormesh (`self.DoorMesh`))
  (if (and (== (`GameplayStatics.GetObjectClass` OtherActor) "/Game/Blueprints/BP_Knife.BP_Knife_C") (== (`KismetStringLibrary.FindSubstring` (`KismetSystemLibrary.GetDisplayName` OtherComp) "AoESphere") -1))
    (`|ExecutionSequence`
      (:`then_0`
        (`PrimitiveComponent.SetSimulatePhysics` _doormesh true)
        (goto _label :!via `Reset`))
      (:`then_1`
        (`/Engine/EditorBlueprintResources/StandardMacros.DoOnce` true :!label _label
          (:`Completed`
            ;[1 1 1] Play Clatter Sound
            (`GameplayStatics.PlaySoundAtLocation` "/Game/Audio/SFX/Placeholder/clatter_sound.clatter_sound" (`SceneComponent.K2_GetComponentLocation` _doormesh))
            (goto _label :!via `Reset`)))))))

(event `self.ReceiveBeginPlay`)

(event `self.ReceiveActorBeginOverlap`
  (params (OtherActor :type "Actor Object Reference")))

(event `self.ReceiveTick`
  (params (DeltaSeconds :type "Float (single-precision)")))

(fn `UserConstructionScript`)