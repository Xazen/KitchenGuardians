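; Fake dirt decal actor that shows enemy-specific splatter (chili, pumpkin, mushroom) on three stacked planes with dynamic materials.
; Collision hits from Enemies trigger the matching decal through a DoOnce gate, though only Chili and Pumpkin are handled.
; Activation randomizes the inactive decal's Degree parameter and raises its plane via small Z offsets.
; After StayTime the gate resets and Tick fades Alpha out over FadeTime.
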(event OnComponentHit(Collision)
  (params (OtherActor :type Actor%20Object%20Reference) (OtherComp :type Primitive%20Component%20Object%20Reference) (NormalImpulse :type Vector :default "0, 0, 0") (Hit :type Hit%20Result%20Structure%20%28by%20ref%29))
  ;[1 1 1] gibblets must
  ; be physical actor
  ;  and simulate hit
  (bind _asenemies (Utilities|Casting|CastToEnemies OtherActor))
  (switch Utilities|FlowControl|Switch|SwitchonEnemyTypeEnum (Variables|/Script/KitchenGuardians.Enemies|GetenemyType _asenemies)
    (:Chili
      ;[1 0.08 0.08] p1 - trigger
      (Utilities|FlowControl|DoOnce false
        (:Completed
          (CallFunction|ActivateDecal1))))
    (:Pumpkin
      ;[0.98 0.4359 0.1862] p2 - activate
      (Utilities|FlowControl|DoOnce false
        (:Completed
          (CallFunction|ActivateDecal2))))))

(event Custom|ActivateDecal1
  ;[1 0.08 0.08] p1 - event
  (CallFunction|SorttoTop)
  (bind _output_get (Variables|Plane1|SetAlpha1 1.0))
  (Rendering|Material|SetScalarParameterValue (Variables|Plane1|GetDirtInstance1) "Alpha" _output_get :!class /Script/Engine.MaterialInstanceDynamic)
  (if (Variables|Plane1|Getdecal1IsActive)
    _
    (else
      (Rendering|Material|SetScalarParameterValue (Variables|Plane1|GetDirtInstance1) "Degree" (Math|Random|RandomFloatinRange 0.0 1.0) :!class /Script/Engine.MaterialInstanceDynamic)
      (Variables|Plane1|Setdecal1IsActive true)))
  (Variables|Plane1|SetisFading1 false)
  (Utilities|FlowControl|Delay (Variables|Default|GetStayTime))
  (Variables|Plane1|SetCurrentFadeTime1 (Variables|Default|GetFadeTime))
  (Variables|Plane1|SetisFading1 true)
  (CallFunction|Reset1))

(event Custom|Reset1
  ;[1 0.08 0.08] p1 - trigger
  (Utilities|FlowControl|DoOnce false) ; enters at Reset
)

(event Custom|ActivateDecal2
  ;[0.98 0.4359 0.1862] p2 - activate
  (CallFunction|SorttoTop 1)
  (bind _output_get (Variables|Plane2|SetAlpha2 1.0))
  (Rendering|Material|SetScalarParameterValue (Variables|Plane2|GetDirtInstance2) "Alpha" _output_get :!class /Script/Engine.MaterialInstanceDynamic)
  (if (Variables|Plane2|Getdecal2IsActive)
    _
    (else
      (Rendering|Material|SetScalarParameterValue (Variables|Plane2|GetDirtInstance2) "Degree" (Math|Random|RandomFloatinRange 0.0 1.0) :!class /Script/Engine.MaterialInstanceDynamic)
      (Variables|Plane2|Setdecal2IsActive true)))
  (Variables|Plane2|SetisFading2 false)
  (Utilities|FlowControl|Delay (Variables|Default|GetStayTime))
  (Variables|Plane2|SetCurrentFadeTime2 (Variables|Default|GetFadeTime))
  (Variables|Plane2|SetisFading2 true)
  (CallFunction|Reset2))

(event Custom|Reset2
  ;[0.98 0.4359 0.1862] p2 - activate
  (Utilities|FlowControl|DoOnce false) ; enters at Reset
)

(event Custom|ActivateDecal3
  ;[0.25 0.1254 0] p3 - activate
  (CallFunction|SorttoTop 2)
  (bind _output_get (Variables|Plane3|SetAlpha3 1.0))
  (Rendering|Material|SetScalarParameterValue (Variables|Plane3|GetDirtInstance3) "Alpha" _output_get :!class /Script/Engine.MaterialInstanceDynamic)
  (if (Variables|Plane3|Getdecal3IsActive)
    _
    (else
      (Rendering|Material|SetScalarParameterValue (Variables|Plane3|GetDirtInstance3) "Degree" (Math|Random|RandomFloatinRange 0.0 1.0) :!class /Script/Engine.MaterialInstanceDynamic)
      (Variables|Plane3|Setdecal3IsActive true)))
  (Variables|Plane3|SetisFading3 false)
  (Utilities|FlowControl|Delay (Variables|Default|GetStayTime))
  (Variables|Plane3|SetCurrentFadeTime3 (Variables|Default|GetFadeTime))
  (Variables|Plane3|SetisFading3 true)
  (CallFunction|Reset3))

(event Custom|Reset3
  ;[0.25 0.1254 0] p3 - activate
  (Utilities|FlowControl|DoOnce false ; enters at Reset
    (:Completed
      (CallFunction|ActivateDecal3))))

(event EventBeginPlay
  ;[1 0.08 0.08] p1 get material
  (bind _returnvalue (Rendering|Material|CreateDynamicMaterialInstance (Variables|Default|GetPlane1) 0 "/Game/Materials/Dirt_Fluid/DirtChili_Inst.DirtChili_Inst" :!class /Script/Engine.PrimitiveComponent))
  (bind _output_get (Variables|Plane1|SetDirtInstance1 _returnvalue))
  (Rendering|Material|SetScalarParameterValue _output_get "Alpha" (Variables|Plane1|GetAlpha1) :!class /Script/Engine.MaterialInstanceDynamic)
  ;[0.98 0.4359 0.1862] p2 - get Material
  (bind _returnvalue_2 (Rendering|Material|CreateDynamicMaterialInstance (Variables|Default|GetPlane2) 0 "/Game/Materials/Dirt_Fluid/DirtPumpkin_Inst.DirtPumpkin_Inst" :!class /Script/Engine.PrimitiveComponent))
  (bind _output_get_2 (Variables|Plane2|SetDirtInstance2 _returnvalue_2))
  (Rendering|Material|SetScalarParameterValue _output_get_2 "Alpha" (Variables|Plane2|GetAlpha2) :!class /Script/Engine.MaterialInstanceDynamic)
  ;[0.25 0.1254 0] p3 - get Material
  (bind _returnvalue_3 (Rendering|Material|CreateDynamicMaterialInstance (Variables|Default|GetPlane3) 0 "/Game/Materials/Dirt_Fluid/DirtMushroom_Inst.DirtMushroom_Inst" :!class /Script/Engine.PrimitiveComponent))
  (bind _output_get_3 (Variables|Plane3|SetDirtInstance3 _returnvalue_3))
  (Rendering|Material|SetScalarParameterValue _output_get_3 "Alpha" (Variables|Plane3|GetAlpha3) :!class /Script/Engine.MaterialInstanceDynamic))

(event EventActorBeginOverlap
  (params (OtherActor :type Actor%20Object%20Reference)))

(event EventTick
  (params (DeltaSeconds :type Float%20%28single-precision%29))
  ;[1 0.08 0.08] p1 - fade
  (if (Variables|Plane1|GetisFading1)
    (bind _output_get (Variables|Plane1|SetCurrentFadeTime1 (- (Variables|Plane1|GetCurrentFadeTime1) DeltaSeconds)))
    (if (<= _output_get 0.0)
      (Variables|Plane1|SetisFading1 false)
      (bind _output_get_2 (Variables|Plane1|SetAlpha1 0.0))
      (Rendering|Material|SetScalarParameterValue (Variables|Plane1|GetDirtInstance1) "Alpha" _output_get_2 :!class /Script/Engine.MaterialInstanceDynamic)
      (Variables|Plane1|Setdecal1IsActive false)
      (else
        (bind _output_get_3 (Variables|Plane1|SetAlpha1 (/ (Variables|Plane1|GetCurrentFadeTime1) (Variables|Default|GetFadeTime))))
        (Rendering|Material|SetScalarParameterValue (Variables|Plane1|GetDirtInstance1) "Alpha" _output_get_3 :!class /Script/Engine.MaterialInstanceDynamic))))
  ;[0.98 0.4359 0.1862] p2 - fade
  (if (Variables|Plane2|GetisFading2)
    (bind _output_get_4 (Variables|Plane2|SetCurrentFadeTime2 (- (Variables|Plane2|GetCurrentFadeTime2) DeltaSeconds)))
    (if (<= _output_get_4 0.0)
      (Variables|Plane2|SetisFading2 false)
      (bind _output_get_5 (Variables|Plane2|SetAlpha2 0.0))
      (Rendering|Material|SetScalarParameterValue (Variables|Plane2|GetDirtInstance2) "Alpha" _output_get_5 :!class /Script/Engine.MaterialInstanceDynamic)
      (Variables|Plane2|Setdecal2IsActive false)
      (else
        (bind _output_get_6 (Variables|Plane2|SetAlpha2 (/ (Variables|Plane2|GetCurrentFadeTime2) (Variables|Default|GetFadeTime))))
        (Rendering|Material|SetScalarParameterValue (Variables|Plane2|GetDirtInstance2) "Alpha" _output_get_6 :!class /Script/Engine.MaterialInstanceDynamic))))
  ;[0.25 0.1254 0] p3 - fade
  (if (Variables|Plane3|GetisFading3)
    (bind _output_get_7 (Variables|Plane3|SetCurrentFadeTime3 (- (Variables|Plane3|GetCurrentFadeTime3) DeltaSeconds)))
    (if (<= _output_get_7 0.0)
      (Variables|Plane3|SetisFading3 false)
      (bind _output_get_8 (Variables|Plane3|SetAlpha3 0.0))
      (Rendering|Material|SetScalarParameterValue (Variables|Plane3|GetDirtInstance3) "Alpha" _output_get_8 :!class /Script/Engine.MaterialInstanceDynamic)
      (Variables|Plane3|Setdecal3IsActive false)
      (else
        (bind _output_get_9 (Variables|Plane3|SetAlpha3 (/ (Variables|Plane3|GetCurrentFadeTime3) (Variables|Default|GetFadeTime))))
        (Rendering|Material|SetScalarParameterValue (Variables|Plane3|GetDirtInstance3) "Alpha" _output_get_9 :!class /Script/Engine.MaterialInstanceDynamic)))))

(fn ConstructionScript
  (Utilities|Array|Add (Variables|Default|GetPlanes) (Variables|Default|GetPlane1))
  (Utilities|Array|Add (Variables|Default|GetPlanes) (Variables|Default|GetPlane2))
  (Utilities|Array|Add (Variables|Default|GetPlanes) (Variables|Default|GetPlane3)))

(fn SorttoTop
  (params (TopIndex :type Integer :default 0))
  (if (not (== TopIndex (Variables|Default|GetCurrentTop)))
    (Utilities|FlowControl|Sequence
      (:then_0
        (LocalVariables|Setloc_IndexTop TopIndex)
        (LocalVariables|Setloc_IndexMid (Variables|Default|GetCurrentTop))
        (Variables|Default|SetCurrentTop (LocalVariables|Getloc_IndexTop))
        (LocalVariables|Setloc_IndexBottom (- 3 (+ (LocalVariables|Getloc_IndexTop) (LocalVariables|Getloc_IndexMid)))))
      (:then_1
        (Utilities|FlowControl|Sequence
          (:then_0
            (Transformation|SetRelativeLocation (Utilities|Array|Get(acopy) (Variables|Default|GetPlanes) (Variables|Default|GetCurrentTop)) "0, 0,0.150000" false))
          (:then_1
            (Transformation|SetRelativeLocation (Utilities|Array|Get(acopy) (Variables|Default|GetPlanes) (LocalVariables|Getloc_IndexMid)) "0, 0,0.100000" false))
          (:then_2
            (Transformation|SetRelativeLocation (Utilities|Array|Get(acopy) (Variables|Default|GetPlanes) (LocalVariables|Getloc_IndexBottom)) "0, 0,0.050000" false)))))))