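; BP_Pliers_4 is a physics-simulated pliers prop that can be reset to where it began.
; On first BeginPlay it stores its starting location and rotation.
; An OnReset event briefly disables physics, teleports the mesh back to that stored transform, then re-enables simulation.
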(event `self.ReceiveBeginPlay`
  (if (not (`self.firstStart`))
    (set `self.startPosition` (`self.K2_GetActorLocation`))
    (set `self.startRotation` (`self.K2_GetActorRotation`))
    (set `self.firstStart` true)))

(event `self.K2_OnReset`
  (bind _pliersmesh (`self.PliersMesh`))
  ;[1 1 1] Reset functionality
  (`PrimitiveComponent.SetSimulatePhysics` _pliersmesh false)
  (`SceneComponent.K2_SetWorldLocationAndRotation` _pliersmesh (`self.startPosition`) (`self.startRotation`) false true)
  (`PrimitiveComponent.SetSimulatePhysics` _pliersmesh true))

(fn `UserConstructionScript`)