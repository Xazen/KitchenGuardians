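; BP_Sink is an interactive sink that runs water when a BP_Knife overlaps its Box.
; The overlap ignores components named like AoESphere, so the knife's area-of-effect volume does not trigger it.
; A hit activates the particle system and plays a pitch-randomized water sound, then stops the particles after a delay.
; A DoOnce gate blocks retriggering until a further cooldown resets it.
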(event `self.ReceiveBeginPlay`)

(event `self.ReceiveActorBeginOverlap`
  (params (OtherActor :type "Actor Object Reference")))

(event `self.ReceiveTick`
  (params (DeltaSeconds :type "Float (single-precision)")))

(event `self.Box.OnComponentBeginOverlap`
  (params (OtherActor :type "Actor Object Reference") (OtherComp :type "PrimitiveComponent Object Reference") (OtherBodyIndex :type Integer) (bFromSweep :type Boolean) (SweepResult :type "HitResult Structure (by ref)"))
  (if (and (== (`GameplayStatics.GetObjectClass` OtherActor) "/Game/Blueprints/BP_Knife.BP_Knife_C") (== (`KismetStringLibrary.FindSubstring` (`KismetSystemLibrary.GetDisplayName` OtherComp) "AoESphere") -1))
    (`/Engine/EditorBlueprintResources/StandardMacros.DoOnce` false :!label _label
      (:`Completed`
        (`ActorComponent.Activate` (`self.ParticleSystem`) false)
        (`GameplayStatics.PlaySoundAtLocation` "/Game/Audio/SFX/firstIteration/Environment/waterRunning.waterRunning" (`self.K2_GetActorLocation`) (struct) 1.0 (`KismetMathLibrary.RandomFloatInRange` 0.8 1.3))
        (`KismetSystemLibrary.Delay` 6.0)
        (`ActorComponent.Deactivate` (`self.ParticleSystem`))
        (`KismetSystemLibrary.Delay` 3.0)
        (goto _label :!via `Reset`)))))

(fn `UserConstructionScript`)