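; A destructible four-blade ventilator whose blades break off when hit by BP_Knife.
; Each blade gets random hit points at BeginPlay, and CheckKnife filters overlaps to knife hits, ignoring its AoE sphere.
; Hits on blades 1–3 play a randomized sound and decrement health, breaking the physics constraint at zero; broken blades are destroyed after a delay.
; Blade 4's damage logic is disconnected, so knife hits never damage it.
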(event `self.ReceiveBeginPlay`
  (set `self.HitPointsBlade1` (`KismetMathLibrary.RandomIntegerInRange` 2 3))
  (set `self.HitPointsBlade2` (`KismetMathLibrary.RandomIntegerInRange` 2 3))
  (set `self.HitPointsBlade3` (`KismetMathLibrary.RandomIntegerInRange` 2 3))
  (set `self.HitPointsBlade4` (`KismetMathLibrary.RandomIntegerInRange` 2 3)))

(event `self.ReceiveActorBeginOverlap`
  (params (OtherActor :type "Actor Object Reference")))

(event `self.ReceiveTick`
  (params (DeltaSeconds :type "Float (single-precision)")))

(event `self.PhysicsConstraint_Blade1.OnConstraintBroken`
  (params (ConstraintIndex :type Integer))
  (`KismetSystemLibrary.Delay` 2.0)
  (`ActorComponent.K2_DestroyComponent` (`self.Ventilator_LP_Blade1`)))

(event `HitSound`
  (bind _returnvalue (`KismetMathLibrary.RandomFloatInRange` 0.7 1.3))
  (`GameplayStatics.PlaySoundAtLocation` "/Game/Audio/SFX/firstIteration/Environment/fanHit.fanHit" (`self.K2_GetActorLocation`) (struct) _returnvalue _returnvalue))

(event `self.PhysicsConstraint_Blade2.OnConstraintBroken`
  (params (ConstraintIndex :type Integer))
  (`KismetSystemLibrary.Delay` 2.0)
  (`ActorComponent.K2_DestroyComponent` (`self.Ventilator_LP_Blade2`)))

(event `self.PhysicsConstraint_Blade3.OnConstraintBroken`
  (params (ConstraintIndex :type Integer))
  (`KismetSystemLibrary.Delay` 2.0)
  (`ActorComponent.K2_DestroyComponent` (`self.Ventilator_LP_Blade3`)))

(event `self.PhysicsConstraint_Blade4.OnConstraintBroken`
  (params (ConstraintIndex :type Integer))
  (`KismetSystemLibrary.Delay` 2.0)
  (`ActorComponent.K2_DestroyComponent` (`self.Ventilator_LP_Blade4`)))

(event `self.Ventilator_LP_Blade1.OnComponentBeginOverlap`
  (params (OtherActor :type "Actor Object Reference") (OtherComp :type "PrimitiveComponent Object Reference") (OtherBodyIndex :type Integer) (bFromSweep :type Boolean) (SweepResult :type "HitResult Structure (by ref)"))
  (bind _isknife (`self.CheckKnife` OtherActor OtherComp))
  (if (and _isknife (> (`self.HitPointsBlade1`) 0))
    (`self.HitSound`)
    (bind _output_get (set `self.HitPointsBlade1` (+ (`self.HitPointsBlade1`) -1)))
    (if (== _output_get 0)
      (`PhysicsConstraintComponent.BreakConstraint` (`self.PhysicsConstraint_Blade1`)))))

(event `self.Ventilator_LP_Blade2.OnComponentBeginOverlap`
  (params (OtherActor :type "Actor Object Reference") (OtherComp :type "PrimitiveComponent Object Reference") (OtherBodyIndex :type Integer) (bFromSweep :type Boolean) (SweepResult :type "HitResult Structure (by ref)"))
  (bind _isknife (`self.CheckKnife` OtherActor OtherComp))
  (if (and _isknife (> (`self.HitPointsBlade2`) 0))
    (`self.HitSound`)
    (bind _output_get (set `self.HitPointsBlade2` (+ (`self.HitPointsBlade2`) -1)))
    (if (== _output_get 0)
      (`PhysicsConstraintComponent.BreakConstraint` (`self.PhysicsConstraint_Blade2`)))))

(event `self.Ventilator_LP_Blade3.OnComponentBeginOverlap`
  (params (OtherActor :type "Actor Object Reference") (OtherComp :type "PrimitiveComponent Object Reference") (OtherBodyIndex :type Integer) (bFromSweep :type Boolean) (SweepResult :type "HitResult Structure (by ref)"))
  (bind _isknife (`self.CheckKnife` OtherActor OtherComp))
  (if (and _isknife (> (`self.HitPointsBlade3`) 0))
    (`self.HitSound`)
    (bind _output_get (set `self.HitPointsBlade3` (+ (`self.HitPointsBlade3`) -1)))
    (if (== _output_get 0)
      (`PhysicsConstraintComponent.BreakConstraint` (`self.PhysicsConstraint_Blade3`)))))

(event `self.Ventilator_LP_Blade4.OnComponentBeginOverlap`
  (params (OtherActor :type "Actor Object Reference") (OtherComp :type "PrimitiveComponent Object Reference") (OtherBodyIndex :type Integer) (bFromSweep :type Boolean) (SweepResult :type "HitResult Structure (by ref)"))
  (bind _isknife (`self.CheckKnife` OtherActor OtherComp)))

(fn `CheckKnife`
  (params (OtherActor :type "Actor Object Reference") (OtherComponent :type "ActorComponent Object Reference"))
  (returns (isKnife :type Boolean))
  (return (and (== (`GameplayStatics.GetObjectClass` OtherActor) "/Game/Blueprints/BP_Knife.BP_Knife_C") (== (`KismetStringLibrary.FindSubstring` (`KismetSystemLibrary.GetDisplayName` OtherComponent) "AoESphere") -1))))

(fn `UserConstructionScript`)