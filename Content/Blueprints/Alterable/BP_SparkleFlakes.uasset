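; BP_SparkleFlakes is a breakable flakes prop that takes two hits to destroy.
; Mesh overlaps from Enemies or BP_Knife count as hits, excluding the knife's AoE sphere by component name.
; Two DoOnce gates stage the break: the first hit arms the initially closed destroy gate after a short delay, and a later hit destroys the actor.
; Each hit spawns flake particles and plays a sound with randomized volume and pitch.
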(event `self.ReceiveBeginPlay`)

(event `self.ReceiveActorBeginOverlap`
  (params (OtherActor :type "Actor Object Reference")))

(event `self.ReceiveTick`
  (params (DeltaSeconds :type "Float (single-precision)"))
  ;[1 1 1] Disabled
)

(event `self.schellocksMesh.OnComponentBeginOverlap`
  (params (OtherActor :type "Actor Object Reference") (OtherComp :type "PrimitiveComponent Object Reference") (OtherBodyIndex :type Integer) (bFromSweep :type Boolean) (SweepResult :type "HitResult Structure (by ref)"))
  (bind _returnvalue (`GameplayStatics.GetObjectClass` OtherActor))
  (bind _returnvalue_2 (`KismetMathLibrary.RandomFloatInRange` 0.7 1.3))
  (bind _returnvalue_3 (`KismetMathLibrary.RandomFloatInRange` 0.7 1.3))
  (bind _returnvalue_4 (`SceneComponent.K2_GetComponentLocation` (`self.P_Reference`)))
  (bind _returnvalue_5 (`SceneComponent.K2_GetComponentLocation` (`self.P_Reference`)))
  (if (or (== _returnvalue "/Script/KitchenGuardians.Enemies") (and (== _returnvalue "/Game/Blueprints/BP_Knife.BP_Knife_C") (== (`KismetStringLibrary.FindSubstring` (`KismetSystemLibrary.GetDisplayName` OtherComp) "AoESphere") -1)))
    (`|ExecutionSequence`
      (:`then_0`
        (`/Engine/EditorBlueprintResources/StandardMacros.DoOnce` true :!label _label
          (:`Completed`
            (`GameplayStatics.SpawnEmitterAtLocation` "/Game/VFX/Particles/P_flakes.P_flakes" _returnvalue_4)
            (`GameplayStatics.PlaySoundAtLocation` "/Game/Audio/SFX/firstIteration/Environment/schellogsHit.schellogsHit" _returnvalue_4 (struct) _returnvalue_3 _returnvalue_3)
            (`KismetSystemLibrary.Delay` 1.0)
            (`self.K2_DestroyActor`))))
      (:`then_1`
        (`/Engine/EditorBlueprintResources/StandardMacros.DoOnce` false
          (:`Completed`
            (`GameplayStatics.SpawnEmitterAtLocation` "/Game/VFX/Particles/P_flakes.P_flakes" _returnvalue_5)
            (`GameplayStatics.PlaySoundAtLocation` "/Game/Audio/SFX/firstIteration/Environment/schellogsHit.schellogsHit" _returnvalue_5 (struct) _returnvalue_2 _returnvalue_2)
            (`KismetSystemLibrary.Delay` 0.3)
            (goto _label :!via `Reset`)))))))

(event `ReceiveActorBeginOverlap_Copy`
  (params (OtherActor :type "Actor Object Reference"))
  ;[1 1 1] to avoid AoE Effect
)

(fn `UserConstructionScript`)