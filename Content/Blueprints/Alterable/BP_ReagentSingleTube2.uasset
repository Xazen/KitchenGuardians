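; Breakable reagent tube prop with a physics-simulated stand that can be reset to its starting state.
; Any Box overlap except with BP_ReagentSingleTube1 plays a pitch-randomized smash sound, spawns shards and hides the bottle and Box, without disabling collision.
; OnReset teleports the stand to the actor transform saved on BeginPlay, restores visibility and re-enables physics.
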(event `self.ReceiveBeginPlay`
  (if (not (`self.firstStart`))
    (set `self.startPosition` (`self.K2_GetActorLocation`))
    (set `self.startRotation` (`self.K2_GetActorRotation`))
    (set `self.firstStart` true)))

(event `self.Box.OnComponentBeginOverlap`
  (params (OtherActor :type "Actor Object Reference") (OtherComp :type "PrimitiveComponent Object Reference") (OtherBodyIndex :type Integer) (bFromSweep :type Boolean) (SweepResult :type "HitResult Structure (by ref)"))
  (bind _returnvalue (`self.K2_GetActorLocation`))
  (cast `/Game/Blueprints/Alterable/BP_ReagentSingleTube1` OtherActor
    (:`CastFailed`
      (`GameplayStatics.PlaySoundAtLocation` "/Game/Audio/SFX/firstIteration/Environment/glass_plate_smash.glass_plate_smash" _returnvalue (struct) 1.0 (`KismetMathLibrary.RandomFloatInRange` 0.8 1.2))
      (`GameplayStatics.SpawnEmitterAtLocation` "/Game/VFX/Particles/test/P_Shards2.P_Shards2" _returnvalue)
      (`SceneComponent.SetVisibility` (`self.Reagent_Bottle_01`) false false)
      (`SceneComponent.SetVisibility` (`self.Box`) false false))))

(event `self.K2_OnReset`
  ;[1 1 1] Reset functionality
  (`PrimitiveComponent.SetSimulatePhysics` (`self.Reagent_Stand_03`) false)
  (`SceneComponent.K2_SetWorldLocationAndRotation` (`self.Reagent_Stand_03`) (`self.startPosition`) (`self.startRotation`) false true)
  (`SceneComponent.SetVisibility` (`self.Reagent_Bottle_01`) true false)
  (`SceneComponent.SetVisibility` (`self.Box`) true false)
  (`PrimitiveComponent.SetSimulatePhysics` (`self.Reagent_Stand_03`) true))

(fn `UserConstructionScript`)