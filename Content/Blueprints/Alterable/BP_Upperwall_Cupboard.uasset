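; BP_Upperwall_Cupboard is a breakable wall cupboard whose door reacts to knife overlaps.
; BeginPlay randomizes the door joint's swing limits and height, plus hit counts for opening and falling.
; Knife hits first deplete the opening count to enable door physics, then the fall count to break the constraint and, after a delay, destroy the door and its child components.
; Each hit also calls HitDoorEffect, which is empty here.
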(event `self.ReceiveBeginPlay`
  (bind _cupboardjoint (`self.CupboardJoint`))
  (`PhysicsConstraintComponent.SetAngularSwing1Limit` (`self.CupboardJoint`) "ACM_Limited" (`KismetMathLibrary.RandomFloatInRange` 20.0 40.0))
  (`PhysicsConstraintComponent.SetAngularSwing2Limit` (`self.CupboardJoint`) "ACM_Free" (`KismetMathLibrary.RandomFloatInRange` 0.0 20.0))
  (`SceneComponent.K2_SetRelativeLocation` _cupboardjoint (`KismetMathLibrary.MakeVector` (.x (`SceneComponent.RelativeLocation` _cupboardjoint)) (.y (`SceneComponent.RelativeLocation` _cupboardjoint)) (`KismetMathLibrary.RandomFloatInRange` 8.0 55.0)) false)
  (set `self.openingHitpoints` (`KismetMathLibrary.RandomIntegerInRange` 2 6))
  (set `self.fallDownHitpoints` (`KismetMathLibrary.RandomIntegerInRange` 2 6)))

(event `HitDoorEffect`)

(event `self.DoorMesh.OnComponentBeginOverlap`
  (params (OtherActor :type "Actor Object Reference") (OtherComp :type "PrimitiveComponent Object Reference") (OtherBodyIndex :type Integer) (bFromSweep :type Boolean) (SweepResult :type "EngineTypes.HitResult Structure (by ref)"))
  (bind _doormesh (`self.DoorMesh`))
  (if (== (`GameplayStatics.GetObjectClass` OtherActor) "/Game/Blueprints/BP_Knife.BP_Knife_C")
    (`|ExecutionSequence`
      (:`then_0`
        (if (> (`self.openingHitpoints`) 0)
          (bind _output_get (set `self.openingHitpoints` (+ (`self.openingHitpoints`) -1)))
          (if (== _output_get 0)
            (`PrimitiveComponent.SetSimulatePhysics` (`self.DoorMesh`) true))
          (elif (> (`self.fallDownHitpoints`) 0)
            (bind _output_get_2 (set `self.fallDownHitpoints` (+ (`self.fallDownHitpoints`) -1)))
            (if (== _output_get_2 0)
              (`PhysicsConstraintComponent.BreakConstraint` (`self.CupboardJoint`))
              (`KismetSystemLibrary.Delay` 10.0)
              (for _array_element (`SceneComponent.GetChildrenComponents` _doormesh false)
                (`ActorComponent.K2_DestroyComponent` _array_element))
              (`ActorComponent.K2_DestroyComponent` _doormesh)))))
      (:`then_1`
        (`self.HitDoorEffect`)))))

(event `self.ReceiveActorBeginOverlap`
  (params (OtherActor :type "Actor Object Reference")))

(event `self.ReceiveTick`
  (params (DeltaSeconds :type "Float (single-precision)")))

(fn `UserConstructionScript`)