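; Tutorial pumpkin actor that reacts to toast hits and can be killed by tapping, both gated by OnlyTap.
; A hit plays fluid and sound effects and briefly clears CanMove, restoring it unless the pumpkin is dying.
; Releasing a touch on TapBox, when the camera reference allows it, swaps the body for physics-driven giblets with impulses, then destroys the actor after a delay.
; The construction script fills the giblet list.
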(event `self.GotHitToastFeedback`
  (bind _returnvalue (`self.K2_GetActorLocation`))
  (if (`self.onlyTap`)
    (set `self.canMove` false)
    (`GameplayStatics.SpawnEmitterAtLocation` "/Game/VFX/Particles/darius/PumpkinFluid.PumpkinFluid" _returnvalue)
    (`GameplayStatics.PlaySoundAtLocation` "/Game/Audio/SFX/swipeHit2.swipeHit2" _returnvalue)
    (`|ExecutionSequence`
      (:`then_1`
        ;[1 1 1] Stop movement for 400 Milliseconds
        (`KismetSystemLibrary.Delay` 0.4)
        (if (not (`self.willDie`))
          (set `self.canMove` true))))))

(event `self.tapBox.OnInputTouchEnd`
  (params (FingerIndex :type "InputCoreTypes.ETouchIndex Enum" :default "Touch1") (TouchedComponent :type "PrimitiveComponent Object Reference"))
  (if (`/Game/Blueprints/BP_Cam.canShootonRelease` (`self.camRefForTap`))
    (if (`self.onlyTap`)
      (set `self.willDie` true)
      (set `self.canMove` false)
      (`GameplayStatics.PlaySoundAtLocation` "/Game/Audio/SFX/fruitDied2.fruitDied2" (`self.K2_GetActorLocation`))
      (`ActorComponent.K2_DestroyComponent` (`self.SkeletalMesh`))
      ;[1 1 1] because no skeletal mesh by now
      (`ActorComponent.K2_DestroyComponent` (`self.pumpkinTmp`))
      (`ActorComponent.K2_DestroyComponent` (`self.tapBox`))
      ;[1 1 1] Giblet Activation and Add Impulse
      (for _array_element (`self.gibletList`)
        (`SceneComponent.SetVisibility` _array_element true false)
        (`PrimitiveComponent.SetSimulatePhysics` _array_element true)
        (`self.AddGibbletImpulse2` _array_element))
      (`KismetSystemLibrary.Delay` 2.5)
      (`self.K2_DestroyActor`))))

(fn `UserConstructionScript`
  (bind _gibletlist (`self.gibletList`))
  (`/Engine/EditorBlueprintResources/StandardMacros.DoOnce` false
    (:`Completed`
      (`KismetArrayLibrary.Array_Add` _gibletlist (`self.Pumpkin_Gibblets_1__Gibblet_Part_01`))
      (`KismetArrayLibrary.Array_Add` _gibletlist (`self.Pumpkin_Gibblets_1__Gibblet_Part_02`))
      (`KismetArrayLibrary.Array_Add` _gibletlist (`self.Pumpkin_Gibblets_1__Gibblet_Part_03`))
      (`KismetArrayLibrary.Array_Add` _gibletlist (`self.Pumpkin_Gibblets_1__LP_Auge`))
      (`KismetArrayLibrary.Array_Add` _gibletlist (`self.Pumpkin_Gibblets_1__Gibblet_Part_04`)))))