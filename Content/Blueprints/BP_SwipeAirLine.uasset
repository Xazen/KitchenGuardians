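; Visual projectile actor for a swipe effect that flies to a target point with speedlines and bursts on arrival.
; MoveTowards records start and target and turns the actor to face the target; Tick then moves it at KnifeTapSpeed without sweeping.
; Within 50 units it spawns one of three random hit emitters just short of the target and destroys itself.
; A 15-second timeout also destroys it, printing a debug message.
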(event `TriggerDetonate`
  (bind _returnvalue (`KismetMathLibrary.VLerp` (`self.StartPosition`) (`self.TargetPosition`) 0.95))
  (switch `int` (`KismetMathLibrary.RandomIntegerInRange` 0 2)
    (:`0`
      (`GameplayStatics.SpawnEmitterAtLocation` "/Game/VFX/Particles/test/SwipeHit1.SwipeHit1" _returnvalue))
    (:`1`
      (`GameplayStatics.SpawnEmitterAtLocation` "/Game/VFX/Particles/test/SwipeHit2.SwipeHit2" _returnvalue))
    (:`2`
      (`GameplayStatics.SpawnEmitterAtLocation` "/Game/VFX/Particles/test/SwipeHit3.SwipeHit3" _returnvalue)))
  (`self.K2_DestroyActor`))

(event `self.ReceiveBeginPlay`
  (`ActorComponent.Activate` (`self.Speedlines`) false)
  (`KismetSystemLibrary.Delay` 15.0)
  (`KismetSystemLibrary.PrintString` "time destroy -inform oelke")
  (`self.K2_DestroyActor`))

(event `self.ReceiveTick`
  (params (DeltaSeconds :type "Float (single-precision)"))
  (bind _location (.location (`self.GetTransform`)))
  (`self.K2_SetActorTransform` (`KismetMathLibrary.MakeTransform` (+ _location (* (`KismetMathLibrary.GetDirectionVector` _location (`self.TargetPosition`)) (* DeltaSeconds (`self.KnifeTapSpeed`)))) (.rotation (`self.GetTransform`)) (.scale (`self.GetTransform`))))
  (if (<= (`KismetMathLibrary.VSize` (- (`SceneComponent.K2_GetComponentLocation`) (`self.TargetPosition`))) 50.0)
    (`/Engine/EditorBlueprintResources/StandardMacros.DoOnce` false
      (:`Completed`
        (`self.TriggerDetonate`)))))

(fn `MoveTowards`
  (params (targetPosition :type "Object.Vector Structure" :default (0.0 0.0 0.0)))
  (bind _output_get (set `self.TargetPosition` targetPosition))
  (bind _output_get_2 (set `self.StartPosition` (`self.K2_GetActorLocation`)))
  (set `self.OriginalDistance` (`KismetMathLibrary.VSize` (- _output_get_2 _output_get)))
  (set `self.movDirection` (`KismetMathLibrary.Normal` (`KismetMathLibrary.GetDirectionVector` _output_get_2 (`self.TargetPosition`))))
  ;[1 1 1] rotate to direction
  (`self.K2_SetActorTransform` (`KismetMathLibrary.MakeTransform` (.location (`self.GetTransform`)) (`KismetMathLibrary.FindLookAtRotation` (`self.StartPosition`) (`self.TargetPosition`)) (.scale (`self.GetTransform`)))))

(fn `UserConstructionScript`)