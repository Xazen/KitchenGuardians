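; BP_Knife is an exploding projectile that flies along a direction set by MoveTowards and self-destroys after five seconds.
; Box overlaps filter targets: most trigger one detonation, regular cupboards only play hit sounds, and some actors are ignored or just remove it.
; Detonation hits living enemies inside AoESphere (Chilli only when vulnerable), awards multi-kill scores through BP_Cube, then plays explosion feedback and destroys itself.
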(event `HitCuppboardEffect`
  (bind _returnvalue (`KismetMathLibrary.RandomFloatInRange` 0.6 1.4))
  (bind _returnvalue_2 (`self.K2_GetActorLocation`))
  (`/Engine/EditorBlueprintResources/StandardMacros.DoOnce` false :!label _label
    (:`Completed`
      (if (`KismetMathLibrary.RandomBool`)
        (`GameplayStatics.PlaySoundAtLocation` "/Game/Audio/SFX/firstIteration/Environment/cuppboardHit1.cuppboardHit1" _returnvalue_2 _returnvalue _returnvalue)
        (else
          (`GameplayStatics.PlaySoundAtLocation` "/Game/Audio/SFX/firstIteration/Environment/cuppboardHit2.cuppboardHit2" _returnvalue_2 _returnvalue _returnvalue)))
      (`KismetSystemLibrary.Delay` 0.3)
      (goto _label :!via `Reset`))))

(event `self.Box.OnComponentBeginOverlap`
  (params (OtherActor :type "Actor Object Reference") (OtherComp :type "PrimitiveComponent Object Reference") (OtherBodyIndex :type Integer) (bFromSweep :type Boolean) (SweepResult :type "EngineTypes.HitResult Structure (by ref)"))
  (bind _aoesphere (`self.AoESphere`))
  (bind _aoesphere_2 (`self.AoESphere`))
  (bind _asenemies (cast `Enemies` OtherActor)
    (:`then`
      (if (> (`Enemies.hitPoints` _asenemies) 0)
        (`/Engine/EditorBlueprintResources/StandardMacros.DoOnce` false :!label _label_2
          (:`Completed`
            (set `self.isDetonated` true)
            (`SceneComponent.SetVisibility` _aoesphere true false)
            (`SceneComponent.SetHiddenInGame` _aoesphere false false)
            (set `self.MultiKillCount` 0)
            (`|ExecutionSequence`
              (:`then_0`
                (if (or (> (`KismetArrayLibrary.Array_Length` (`PrimitiveComponent.GetOverlappingActors` _aoesphere_2 "/Game/Blueprints/Alterable/BP_Lowerwall_Cupboard.BP_Lowerwall_Cupboard_C")) 0) (> (`KismetArrayLibrary.Array_Length` (`PrimitiveComponent.GetOverlappingActors` _aoesphere_2 "/Game/Blueprints/Alterable/BP_Upperwall_Cupboard.BP_Upperwall_Cupboard_C")) 0) (> (`KismetArrayLibrary.Array_Length` (`PrimitiveComponent.GetOverlappingActors` _aoesphere_2 "/Game/Blueprints/Alterable/BP_Upperwall_Cupboard.BP_Upperwall_Cupboard_C")) 0))
                  (`self.HitCuppboardEffect`)))
              (:`then_1`
                (for _array_element (`PrimitiveComponent.GetOverlappingActors` (`self.AoESphere`) "/Script/KitchenGuardians.Enemies")
                  (bind _asenemies_2 (cast `Enemies` _array_element))
                  (bind _asbp_chilli (cast `/Game/Blueprints/BP_Chilli` _asenemies_2)
                    (:`then`
                      (bind _returnvalue (> (`Enemies.hitPoints` _asenemies_2) 0))
                      (if (and (`Enemies.isEnemyVulnerable` _asbp_chilli) _returnvalue)
                        (set `self.MultiKillCount` (+ (`self.MultiKillCount`) 1) :!label _label_3)
                        ;[1 1 1] do once location?
                        (`Enemies.GotHit` _asenemies_2 "Tap" (`self.K2_GetActorLocation`))))
                    (:`CastFailed`
                      (if _returnvalue
                        (goto _label_3)))))
                (`|ExecutionSequence`
                  (:`then_0`
                    (if (>= (`self.MultiKillCount`) 3)
                      (bind _outactors (`GameplayStatics.GetAllActorsOfClass` "/Game/Blueprints/BP_Cube.BP_Cube_C"))
                      (`/Game/Blueprints/BP_Cube.specialScore` (`KismetArrayLibrary.Array_Get` _outactors) (`self.K2_GetActorLocation`) "Massacre")
                      (elif (>= (`self.MultiKillCount`) 2)
                        (bind _outactors_2 (`GameplayStatics.GetAllActorsOfClass` "/Game/Blueprints/BP_Cube.BP_Cube_C"))
                        (`/Game/Blueprints/BP_Cube.specialScore` (`KismetArrayLibrary.Array_Get` _outactors_2) (`self.K2_GetActorLocation`) "MultiKill"))))
                  (:`then_1`
                    (`self.Impact Feedback`)
                    (`|ExecutionSequence`
                      (:`then_0`
                        (`ActorComponent.K2_DestroyComponent`))
                      (:`then_1`
                        (`ActorComponent.K2_DestroyComponent`))
                      (:`then_2`
                        (`ActorComponent.K2_DestroyComponent`))
                      (:`then_3`
                        (`ActorComponent.K2_DestroyComponent`))
                      (:`then_4`
                        (`KismetSystemLibrary.Delay` 0.2)
                        (`self.K2_DestroyActor`)))))))))))
    (:`CastFailed`
      (cast `Guardian` OtherActor
        (:`CastFailed`
          (bind _asalterable_object (cast `AlterableObject` OtherActor)
            (:`then`
              (cast `/Game/Blueprints/Alterable/BP_FridgeSpawn2` _asalterable_object
                (:`then`
                  (goto _label_2))
                (:`CastFailed`
                  (cast `/Game/Blueprints/Alterable/BP_Upperwall_CupboardSpawn` _asalterable_object
                    (:`then`
                      (goto _label_2))
                    (:`CastFailed`
                      (cast `/Game/Blueprints/Alterable/BP_Lowerwall_Cupboard` _asalterable_object
                        (:`then`
                          _)
                        (:`CastFailed`
                          (cast `/Game/Blueprints/Alterable/BP_Upperwall_Cupboard` _asalterable_object)))
                      (`self.HitCuppboardEffect`))))))
            (:`CastFailed`
              (cast `/Game/Blueprints/Alterable/BP_ToastCatch` OtherActor
                (:`then`
                  (`self.K2_DestroyActor`))
                (:`CastFailed`
                  (cast `/Game/Blueprints/BP_Knife` OtherActor
                    (:`CastFailed`
                      (goto _label_2))))))))))))

(event `Impact Feedback`
  (bind _returnvalue (`SceneComponent.K2_GetComponentLocation` (`self.ToastMesh`)))
  (switch `int` (`KismetMathLibrary.RandomIntegerInRange` 0 2)
    (:`0`
      (`GameplayStatics.PlaySoundAtLocation` "/Game/Audio/SFX/firstIteration/TapAttack/toast_explosion1.toast_explosion1" _returnvalue))
    (:`1`
      (`GameplayStatics.PlaySoundAtLocation` "/Game/Audio/SFX/firstIteration/TapAttack/toast_explosion2.toast_explosion2" _returnvalue))
    (:`2`
      (`GameplayStatics.PlaySoundAtLocation` "/Game/Audio/SFX/firstIteration/TapAttack/toast_explosion3.toast_explosion3" _returnvalue)))
  (`PlayerController.ClientStartCameraShake` :`self` (`GameplayStatics.GetPlayerController` 0) :`Shake` "/Game/Blueprints/ScreenShake/BP_ScreenShake.BP_ScreenShake_C" :`Scale` 3.0)
  (`GameplayStatics.SpawnEmitterAtLocation` "/Game/VFX/Particles/darius/P_Explosion_smallN.P_Explosion_smallN" (.location (`self.GetTransform`)) (.rotation (`self.GetTransform`))))

(event `self.ReceiveBeginPlay`
  (`KismetSystemLibrary.Delay` 5.0)
  (`KismetSystemLibrary.PrintString` "time destroy -inform oelke")
  (`self.K2_DestroyActor`))

(event `self.ReceiveTick`
  (params (DeltaSeconds :type "Float (single-precision)"))
  (if (not (`self.isDetonated`))
    (`self.K2_SetActorTransform` (`KismetMathLibrary.MakeTransform` (+ (.location (`self.GetTransform`)) (* (`self.movDirection`) (* DeltaSeconds (`self.KnifeTapSpeed`)))) (.rotation (`self.GetTransform`)) (.scale (`self.GetTransform`))))))

(fn `MoveTowards`
  (params (targetPosition :type "Object.Vector Structure" :default (0.0 0.0 0.0)))
  (set `self.TargetPosition` targetPosition)
  (bind _output_get (set `self.StartPosition` (`self.K2_GetActorLocation`)))
  (set `self.movDirection` (`KismetMathLibrary.Normal` (`KismetMathLibrary.GetDirectionVector` _output_get (`self.TargetPosition`))))
  ;[1 1 1] rotate to direction
  (`self.K2_SetActorTransform` (`KismetMathLibrary.MakeTransform` (.location (`self.GetTransform`)) (`KismetMathLibrary.FindLookAtRotation` (`self.StartPosition`) (`self.TargetPosition`)) (.scale (`self.GetTransform`)))))

(fn `UserConstructionScript`)