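; Main HUD Blueprint that shows the player's enemy score and life bar on screen.
; On BeginPlay it creates the Score and Lifebar widgets for player controller 0 and adds both to the viewport.
; SetScore switches on enemy type (Blue, Green, Red) and overwrites the matching score variable on the Score widget.
; ReduceLife subtracts damage directly from the Lifebar's current percent, with no clamping in this Blueprint.
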(event `self.ReceiveBeginPlay`
  (bind _returnvalue (`GameplayStatics.GetPlayerController` 0))
  (`|ExecutionSequence`
    (:`then_0`
      (bind _returnvalue_2 (`|CreateWidget` "/Game/Blueprints/HUD/Score.Score_C" _returnvalue))
      (bind _output_get (set `self.scoreWidget` _returnvalue_2))
      (`UserWidget.AddToViewport` _output_get 0))
    (:`then_1`
      (bind _returnvalue_3 (`|CreateWidget` "/Game/Blueprints/HUD/Lifebar.Lifebar_C" _returnvalue))
      (bind _output_get_2 (set `self.healthWidget` _returnvalue_3))
      (`UserWidget.AddToViewport` _output_get_2 0))))

(event `self.ReceiveActorBeginOverlap`
  (params (OtherActor :type "Actor Object Reference")))

(event `self.ReceiveTick`
  (params (DeltaSeconds :type "Float (single-precision)")))

(fn `ReduceLife`
  (params (damageTaken :type "Float (double-precision)"))
  (bind _healthwidget (`self.healthWidget`))
  (`/Game/Blueprints/HUD/Lifebar.SetPercentLifebar` _healthwidget (- (`/Game/Blueprints/HUD/Lifebar.GetPercentLifebar` _healthwidget) damageTaken)))

(fn `SetScore`
  (params (pointsOfEnemy :type Integer) (enemyType :type "/Game/Blueprints/Enums/EnemyTypeEnum Enum" :default "NewEnumerator0"))
  (bind _scorewidget (`self.scoreWidget`))
  (switch `/Game/Blueprints/Enums/EnemyTypeEnum` enemyType
    (:`NewEnumerator0`
      (set `/Game/Blueprints/HUD/Score.scoreEnemy1` pointsOfEnemy _scorewidget))
    (:`NewEnumerator1`
      (set `/Game/Blueprints/HUD/Score.scoreEnemy2` pointsOfEnemy _scorewidget))
    (:`NewEnumerator2`
      (set `/Game/Blueprints/HUD/Score.scoreEnemy3` pointsOfEnemy _scorewidget))))

(fn `UserConstructionScript`)