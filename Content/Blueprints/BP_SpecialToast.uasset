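; Special toast projectile that flies to a target point and detonates in an area attack under slow motion.
; MoveTowards sets target and facing; Tick moves it, deepening global slow motion on a quartic distance curve.
; On arrival it fades the AoE sphere, hits overlapping living Enemies, fires impulse, effects and shake, then a timeline restores time before destruction.
; A delayed destroy acts as fallback; giblet physics code is unconnected.
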(event `fadeAoE`
  (bind _returnvalue (`PrimitiveComponent.CreateDynamicMaterialInstance` 0 "/Game/Materials/Placeholder/AoeFade_Inst.AoeFade_Inst"))
  (bind (_direction _alpha) (`Timeline|Fade`)
    (:`Update`
      (`MaterialInstanceDynamic.SetScalarParameterValue` _returnvalue "Alpha" _alpha))))

(event `scaleToast`
  (bind (_direction _scale) (`Timeline|scale`)
    (:`Update`
      (`SceneComponent.SetRelativeScale3D` (`KismetMathLibrary.MakeVector` _scale _scale _scale)))))

(event `Impact Feedback`
  (bind _returnvalue (`SceneComponent.K2_GetComponentLocation` (`self.Cube`)))
  (`ActorComponent.K2_DestroyComponent` (`self.Cube`))
  (`|ExecutionSequence`
    (:`then_4`
      (`RadialForceComponent.FireImpulse` (`self.RadialForce`))
      (switch `int` (`KismetMathLibrary.RandomIntegerInRange` 0 2)
        (:`0`
          (`GameplayStatics.PlaySoundAtLocation` "/Game/Audio/SFX/firstIteration/TapAttack/toast_explosion1.toast_explosion1" _returnvalue 3.0 0.7))
        (:`1`
          (`GameplayStatics.PlaySoundAtLocation` "/Game/Audio/SFX/firstIteration/TapAttack/toast_explosion2.toast_explosion2" _returnvalue 3.0 0.7))
        (:`2`
          (`GameplayStatics.PlaySoundAtLocation` "/Game/Audio/SFX/firstIteration/TapAttack/toast_explosion3.toast_explosion3" _returnvalue 3.0 0.7)))
      (`PlayerController.ClientStartCameraShake` :`self` (`GameplayStatics.GetPlayerController` 0) :`Shake` "/Game/Blueprints/ScreenShake/BP_ScreenShakeSpecialShot.BP_ScreenShakeSpecialShot_C" :`Scale` 6.0)
      (`GameplayStatics.SpawnEmitterAtLocation` "/Game/VFX/Particles/darius/P_Explosion_SpecialToast.P_Explosion_SpecialToast" (.location (`self.GetTransform`)) (.rotation (`self.GetTransform`))))))

(event `TriggerDetonate`
  (bind _aoesphere (`self.AoESphere`))
  (`SceneComponent.SetVisibility` _aoesphere true false)
  (`PrimitiveComponent.SetCollisionEnabled` _aoesphere "QueryAndPhysics")
  (`SceneComponent.SetHiddenInGame` _aoesphere false false)
  (`self.fadeAoE`)
  (for _array_element (`PrimitiveComponent.GetOverlappingActors` (`self.AoESphere`) "/Script/KitchenGuardians.Enemies")
    (bind _asenemies (cast `Enemies` _array_element))
    (if (> (`Enemies.hitPoints` _asenemies) 0)
      ;[1 1 1] do once location?
      (`Enemies.GotHit` _asenemies "Special" (`SceneComponent.K2_GetComponentLocation`))))
  (`self.Impact Feedback`)
  (set `self.OriginalDistance` (`GameplayStatics.GetGlobalTimeDilation`))
  (bind (_direction _timediletation) (`Timeline|revertSlowmo`)
    (:`Update`
      (`GameplayStatics.SetGlobalTimeDilation` (`KismetMathLibrary.Lerp` (`self.OriginalDistance`) 1.0 _timediletation))
      (if (>= _timediletation 0.4)
        (`/Engine/EditorBlueprintResources/StandardMacros.DoOnce` false
          (:`Completed`
            (`GameplayStatics.PlaySoundAtLocation` "/Game/Audio/SFX/firstIteration/slowdownReverse.slowdownReverse" (`self.K2_GetActorLocation`))))))
    (:`Finished`
      (`self.K2_DestroyActor`))))

(event `self.ReceiveBeginPlay`
  (`self.scaleToast`)
  (`PrimitiveComponent.SetCollisionEnabled` (`self.AoESphere`) "NoCollision")
  (`GameplayStatics.PlaySoundAtLocation` "/Game/Audio/SFX/firstIteration/slowdownShot.slowdownShot" (`self.K2_GetActorLocation`))
  (`KismetSystemLibrary.Delay` 15.0)
  (`KismetSystemLibrary.PrintString` "time destroy -inform oelke")
  (`self.K2_DestroyActor`))

(event `self.ReceiveTick`
  (params (DeltaSeconds :type "Float (single-precision)"))
  (bind _location (.location (`self.GetTransform`)))
  (if (not (`self.triggeredDetonate`))
    (`self.K2_SetActorTransform` (`KismetMathLibrary.MakeTransform` (+ _location (* (`KismetMathLibrary.GetDirectionVector` _location (`self.TargetPosition`)) (* DeltaSeconds (`self.KnifeTapSpeed`)))) (.rotation (`self.GetTransform`)) (.scale (`self.GetTransform`))))
    (if (<= (`KismetMathLibrary.VSize` (- (`SceneComponent.K2_GetComponentLocation`) (`self.TargetPosition`))) 50.0)
      (`/Engine/EditorBlueprintResources/StandardMacros.DoOnce` false
        (:`Completed`
          (`self.TriggerDetonate`)
          (set `self.triggeredDetonate` true)))
      (else
        (`GameplayStatics.SetGlobalTimeDilation` (`KismetMathLibrary.Lerp` 0.1 1.0 (`KismetMathLibrary.Square` (`KismetMathLibrary.Square` (/ (`KismetMathLibrary.VSize` (- (`self.K2_GetActorLocation`) (`self.TargetPosition`))) (`self.OriginalDistance`))))))))))

(fn `MoveTowards`
  (params (targetPosition :type "Object.Vector Structure" :default (0.0 0.0 0.0)))
  (bind _output_get (set `self.TargetPosition` targetPosition))
  (bind _output_get_2 (set `self.StartPosition` (`self.K2_GetActorLocation`)))
  (set `self.OriginalDistance` (`KismetMathLibrary.VSize` (- _output_get_2 _output_get)))
  (set `self.movDirection` (`KismetMathLibrary.Normal` (`KismetMathLibrary.GetDirectionVector` _output_get_2 (`self.TargetPosition`))))
  ;[1 1 1] rotate to direction
  (`self.K2_SetActorTransform` (`KismetMathLibrary.MakeTransform` (.location (`self.GetTransform`)) (`KismetMathLibrary.FindLookAtRotation` (`self.StartPosition`) (`self.TargetPosition`)) (.scale (`self.GetTransform`)))))

(fn `UserConstructionScript`)