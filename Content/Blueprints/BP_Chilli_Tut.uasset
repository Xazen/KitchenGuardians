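; Chilli enemy, apparently a tutorial variant, whose red/green colour marks it invulnerable or vulnerable, driven by an Amount parameter on dynamic materials.
; ColorTransition blends the colour over idle time, SwitchColor commits colour and vulnerability, and SpawnScale handles spawn scaling.
; Blocked hits flash black with sound, gated by OnlySwipe.
; Death events swap the mesh for physics giblets, with colour-matched particles and a radial impulse, then destroy the actor.
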(event `self.ReceiveBeginPlay`
  (bind _returnvalue (`PrimitiveComponent.CreateDynamicMaterialInstance` (`self.SkeletalMesh`) 0 "/Game/Materials/Textures/Characters/Chilli/Chilli_Inst.Chilli_Inst"))
  (bind _output_get (set `self.MaterialReference` _returnvalue))
  (`MaterialInstanceDynamic.SetScalarParameterValue` _output_get "Amount" (`self.currentColorCode`))
  (bind _returnvalue_2 (`PrimitiveComponent.CreateDynamicMaterialInstance` (`self.SkeletalMesh`) 1 "/Game/Materials/Textures/Characters/Chilli/Chilli_Inst.Chilli_Inst"))
  (bind _output_get_2 (set `self.MaterialReference2` _returnvalue_2))
  (`MaterialInstanceDynamic.SetScalarParameterValue` _output_get_2 "Amount" (`self.currentColorCode`)))

(event `self.gotHitInvulnerableFeedback`
  (bind _returnvalue (`self.K2_GetActorLocation`))
  (if (`self.onlySwipe`)
    ;[1 1 1] implement enemy block here
    (`self.playRandomSwipeHitSound` _returnvalue)
    (`GameplayStatics.PlaySoundAtLocation` "/Game/Audio/SFX/firstIteration/chilliBlock.chilliBlock" _returnvalue 1.0 (`KismetMathLibrary.RandomFloatInRange` 0.7 1.3))
    (`PrimitiveComponent.SetMaterial` 0 "/Game/Materials/Characters/flashBlack.flashBlack")
    (`KismetSystemLibrary.Delay` 0.05)
    (`PrimitiveComponent.SetMaterial` 0 "/Game/Materials/Textures/Characters/Chilli/Chilli_Inst.Chilli_Inst")
    (bind _returnvalue_2 (`PrimitiveComponent.CreateDynamicMaterialInstance` (`self.SkeletalMesh`) 0 "/Game/Materials/Textures/Characters/Chilli/Chilli_Inst.Chilli_Inst"))
    (bind _output_get (set `self.MaterialReference` _returnvalue_2))
    (`MaterialInstanceDynamic.SetScalarParameterValue` _output_get "Amount" (`self.currentColorCode`))
    (bind _returnvalue_3 (`PrimitiveComponent.CreateDynamicMaterialInstance` (`self.SkeletalMesh`) 1 "/Game/Materials/Textures/Characters/Chilli/Chilli_Inst.Chilli_Inst"))
    (bind _output_get_2 (set `self.MaterialReference2` _returnvalue_3))
    (`MaterialInstanceDynamic.SetScalarParameterValue` _output_get_2 "Amount" (`self.currentColorCode`))))

(event `self.diedRiceFeedback`
  (if (`self.onlySwipe`)
    (`self.playRandomSwipeHitSound` (`self.K2_GetActorLocation`))
    (set `self.willDie` true :!label _label)
    (set `self.canMove` false)
    (`ActorComponent.K2_DestroyComponent` (`self.SkeletalMesh`) :!label _label_2)
    (`ActorComponent.K2_DestroyComponent` (`self.dropShadow`))
    (`ActorComponent.K2_DestroyComponent` (`self.shadowTester`))
    (`ActorComponent.K2_DestroyComponent` (`self.ChilliTmp`))
    ;[1 1 1] Giblet Activation and Add Impulse
    (`|ExecutionSequence`
      (:`then_0`
        (if (not (`self.isEnemyVulnerable`))
          (`self.dieRedGibblet`)))
      (:`then_1`
        (`GameplayStatics.PlaySoundAtLocation` "/Game/Audio/SFX/firstIteration/chilliDied.chilliDied" (`self.K2_GetActorLocation`)))
      (:`then_2`
        (if (`self.isEnemyVulnerable`)
          (`GameplayStatics.SpawnEmitterAtLocation` "/Game/Effects/P_ChilliGreenDied.P_ChilliGreenDied" (`SceneComponent.K2_GetComponentLocation` (`self.TapReference`)))
          (else
            (`GameplayStatics.SpawnEmitterAtLocation` "/Game/Effects/P_ChilliRedDied.P_ChilliRedDied" (`SceneComponent.K2_GetComponentLocation` (`self.TapReference`))))))
      (:`then_3`
        (for _array_element (`self.gibletList`)
          (`SceneComponent.SetVisibility` _array_element true false)
          (`PrimitiveComponent.SetSimulatePhysics` _array_element true))
        (`self.GibbletImpulse`)
        (`KismetSystemLibrary.Delay` 2.5)
        (`self.K2_DestroyActor`)))))

(event `self.hitToastFeedback`
  (set `self.willDie` true)
  (set `self.canMove` false)
  (goto _label_2))

(event `self.diedToastFeedback`
  (goto _label))

(fn `ColorTransition`
  (bind _materialreference (`self.MaterialReference`))
  (bind _materialreference2 (`self.MaterialReference2`))
  (bind _returnvalue (/ (`self.idleCurrentTime`) (`self.idleTime`)))
  (if (== (`self.currentColorCode`) 1.0)
    (`MaterialInstanceDynamic.SetScalarParameterValue` _materialreference "Amount" (- 1.0 _returnvalue))
    (`MaterialInstanceDynamic.SetScalarParameterValue` _materialreference2 "Amount" 0.0)
    (else
      (`MaterialInstanceDynamic.SetScalarParameterValue` _materialreference "Amount" _returnvalue)
      (`MaterialInstanceDynamic.SetScalarParameterValue` _materialreference2 "Amount" 0.0))))

(fn `dieRedGibblet`
  (`|ExecutionSequence`
    (:`then_0`
      (bind _returnvalue (`PrimitiveComponent.CreateDynamicMaterialInstance` (`self.Giblet01`) 0 "/Game/Materials/Textures/Characters/Chilli/Chilli_Inst.Chilli_Inst"))
      (`MaterialInstanceDynamic.SetScalarParameterValue` _returnvalue "Amount" 0.0))
    (:`then_1`
      (bind _returnvalue_2 (`PrimitiveComponent.CreateDynamicMaterialInstance` (`self.Giblet02`) 0 "/Game/Materials/Textures/Characters/Chilli/Chilli_Inst.Chilli_Inst"))
      (`MaterialInstanceDynamic.SetScalarParameterValue` _returnvalue_2 "Amount" 0.0))
    (:`then_2`
      (bind _returnvalue_3 (`PrimitiveComponent.CreateDynamicMaterialInstance` (`self.Giblet03`) 0 "/Game/Materials/Textures/Characters/Chilli/Chilli_Inst.Chilli_Inst"))
      (`MaterialInstanceDynamic.SetScalarParameterValue` _returnvalue_3 "Amount" 0.0))
    (:`then_3`
      (bind _returnvalue_4 (`PrimitiveComponent.CreateDynamicMaterialInstance` (`self.Giblet04`) 0 "/Game/Materials/Textures/Characters/Chilli/Chilli_Inst.Chilli_Inst"))
      (`MaterialInstanceDynamic.SetScalarParameterValue` _returnvalue_4 "Amount" 0.0))
    (:`then_4`
      (bind _returnvalue_5 (`PrimitiveComponent.CreateDynamicMaterialInstance` (`self.Giblet05`) 0 "/Game/Materials/Textures/Characters/Chilli/Chilli_Inst.Chilli_Inst"))
      (`MaterialInstanceDynamic.SetScalarParameterValue` _returnvalue_5 "Amount" 0.0))
    (:`then_5`
      (bind _returnvalue_6 (`PrimitiveComponent.CreateDynamicMaterialInstance` (`self.Giblet06`) 0 "/Game/Materials/Textures/Characters/Chilli/Chilli_Inst.Chilli_Inst"))
      (`MaterialInstanceDynamic.SetScalarParameterValue` _returnvalue_6 "Amount" 0.0))))

(fn `GibbletImpulse`
  (bind _returnvalue (`KismetMathLibrary.RandomFloatInRange` -20.0 20.0))
  (bind _radialforce (`self.RadialForce`))
  (if (== (`self.RadialForcePosition`) (0.0 0.0 0.0))
    (`SceneComponent.K2_AddLocalOffset` _radialforce (`KismetMathLibrary.MakeVector` _returnvalue _returnvalue _returnvalue) true)
    (set `RadialForceComponent.ImpulseStrength` (`self.GibbletImpulseSwipe`) _radialforce)
    (else
      (`SceneComponent.K2_SetWorldLocation` _radialforce (`self.RadialForcePosition`) true)
      (set `RadialForceComponent.ImpulseStrength` (`self.GibbletImpulseTap`) _radialforce)))
  (`RadialForceComponent.FireImpulse` _radialforce))

(fn `playRandomSwipeHitSound`
  (params (Location :type "Object.Vector Structure" :default (0.0 0.0 0.0)))
  (switch `int` (`KismetMathLibrary.RandomIntegerInRange` 0 2)
    (:`0`
      (`GameplayStatics.PlaySoundAtLocation` "/Game/Audio/SFX/firstIteration/swipeHit1.swipeHit1" Location 1.0 (`KismetMathLibrary.RandomFloatInRange` 0.8 1.2)))
    (:`1`
      (`GameplayStatics.PlaySoundAtLocation` "/Game/Audio/SFX/firstIteration/swipeHit2.swipeHit2" Location 1.0 (`KismetMathLibrary.RandomFloatInRange` 0.8 1.2)))
    (:`2`
      (`GameplayStatics.PlaySoundAtLocation` "/Game/Audio/SFX/firstIteration/swipeHit3.swipeHit3" Location 1.0 (`KismetMathLibrary.RandomFloatInRange` 0.8 1.2)))))

(fn `SpawnScale`
  (params (DeltaTime :type "Float (double-precision)" :default 0.0))
  (bind _returnvalue (`KismetMathLibrary.Lerp` 1.0 (`self.SpawnMinScale`) (/ (`self.CurrentSpawnScaleTime`) (`self.SpawnScaleTime`))))
  (bind _output_get (set `self.CurrentSpawnScaleTime` (- (`self.CurrentSpawnScaleTime`) DeltaTime)))
  (if (<= _output_get 0.0)
    (set `self.isScaling` false)
    (set `self.CurrentSpawnScaleTime` 0.0))
  (`SceneComponent.SetWorldScale3D` (`self.Scene`) (`KismetMathLibrary.MakeVector` _returnvalue _returnvalue _returnvalue)))

(fn `switchColor`
  (bind _materialreference (`self.MaterialReference`))
  (bind _returnvalue (`MaterialInstanceDynamic.K2_GetScalarParameterValue` (`self.MaterialReference`) "Amount"))
  (if (> _returnvalue 0.5)
    (bind _output_get (set `self.currentColorCode` 1.0))
    (`MaterialInstanceDynamic.SetScalarParameterValue` _materialreference "Amount" _output_get)
    (set `self.isEnemyVulnerable` true)
    (else
      (bind _output_get_2 (set `self.currentColorCode` 0.0))
      (`MaterialInstanceDynamic.SetScalarParameterValue` _materialreference "Amount" _output_get_2)
      (`MaterialInstanceDynamic.SetScalarParameterValue` (`self.MaterialReference2`) "Amount" 0.0)
      (set `self.isEnemyVulnerable` false))))

(fn `UserConstructionScript`
  (bind _gibletlist (`self.gibletList`))
  (`/Engine/EditorBlueprintResources/StandardMacros.DoOnce` false
    (:`Completed`
      (`KismetArrayLibrary.Array_Add` _gibletlist (`self.Giblet01`))
      (`KismetArrayLibrary.Array_Add` _gibletlist (`self.Giblet02`))
      (`KismetArrayLibrary.Array_Add` _gibletlist (`self.Giblet03`))
      (`KismetArrayLibrary.Array_Add` _gibletlist (`self.Giblet04`))
      (`KismetArrayLibrary.Array_Add` _gibletlist null)
      (`KismetArrayLibrary.Array_Add` _gibletlist null))))