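; BP_Toast is the toaster character actor, with hitpoints, ammo reloading and game over on defeat.
; Tick advances the reload and flags death at zero hitpoints, while Tap starts a reload, though its touch trigger is disabled.
; Feedback events drive montages, chaining an active shot into its reload section, and start or stop charge audio.
; Hits swap in damaged materials, and both hits and death briefly flash a screen widget created at BeginPlay.
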(event `self.ReceiveActorOnInputTouchBegin`
  (params (FingerIndex :type "InputCoreTypes.ETouchIndex Enum" :default "Touch1"))
  (if false
    (`self.Tap`)))

(event `self.ReceiveTick`
  (params (DeltaSeconds :type "Float (single-precision)"))
  (`self.reloadAmmo` DeltaSeconds)
  (if (<= (`self.hitpoints`) 0)
    (set `self.isDead` true)))

(event `Tap`
  (`self.initReload`))

(event `self.ReceiveBeginPlay`
  (bind _asbp_toast_animation (cast `/Game/Animations/Toaster/BP_ToastAnimation` (`SkeletalMeshComponent.GetAnimInstance` (`self.SkeletalMesh`)))
    (:`then`
      (set `self.BpAnimToast` _asbp_toast_animation))
    (:`CastFailed`
      _))
  (bind _returnvalue (`|CreateWidget` "/Game/Blueprints/HUD/gotHit.gotHit_C" (`GameplayStatics.GetPlayerController` 0)))
  (set `self.gotHitFlash` _returnvalue)
  (`Widget.SetVisibility` _returnvalue "Hidden")
  (`UserWidget.AddToViewport` _returnvalue 0))

(event `self.GotHitFeedback`
  (bind _gothitflash (`self.gotHitFlash`))
  (bind _skeletalmesh (`self.SkeletalMesh`))
  (`PrimitiveComponent.SetMaterial` _skeletalmesh 0 "/Game/Materials/Characters/Toaster_Chan/Toaster_Chan_Damaged_MAT.Toaster_Chan_Damaged_MAT")
  (`PrimitiveComponent.SetMaterial` _skeletalmesh 1 "/Game/Materials/Characters/Toaster_Chan/Toaster_Chan_Damaged_MAT.Toaster_Chan_Damaged_MAT")
  (`AnimInstance.Montage_Play` (`self.BpAnimToast`) "/Game/Animations/Toaster/ToastMontage_GotHit.ToastMontage_GotHit" 1.0)
  (`Widget.SetVisibility` _gothitflash "Visible" :!label _label)
  (`KismetSystemLibrary.Delay` 0.15)
  (`Widget.SetVisibility` _gothitflash "Hidden"))

(event `self.DiedFeedback`
  (`GameLogic.gameOver` (`self.BP_Cube`))
  (`AnimInstance.Montage_Play` (`self.BpAnimToast`) "/Game/Animations/Toaster/ToastMontage_Defeated.ToastMontage_Defeated" 1.0)
  (goto _label))

(event `self.ShotFeedback`
  (`AnimInstance.Montage_Play` (`self.BpAnimToast`) "/Game/Animations/Toaster/ToastMontage_Shoot.ToastMontage_Shoot" 1.0))

(event `InitCharge`
  (`AnimInstance.Montage_Play` (`self.BpAnimToast`) "/Game/Animations/Toaster/ToastMontage_Reload.ToastMontage_Reload" 1.0)
  (`AudioComponent.Play` (`self.Audio`) 0.0))

(event `self.ReloadFeedback`
  (bind _returnvalue (`AnimInstance.Montage_IsActive` (`self.BpAnimToast`) "/Game/Animations/Toaster/ToastMontage_Shoot.ToastMontage_Shoot"))
  (if _returnvalue
    (`AnimInstance.Montage_SetNextSection` (`self.BpAnimToast`) "Shoot" "Reload" "/Game/Animations/Toaster/ToastMontage_Shoot.ToastMontage_Shoot")
    (else
      (`AnimInstance.Montage_Play` (`self.BpAnimToast`) "/Game/Animations/Toaster/ToastMontage_Reload.ToastMontage_Reload" 1.0))))

(event `StopCharge`
  (bind _audio (`self.Audio`))
  (bind _returnvalue (`AnimInstance.Montage_IsPlaying` (`self.BpAnimToast`) "/Game/Animations/Toaster/ToastMontage_Reload.ToastMontage_Reload"))
  (if _returnvalue
    (`AnimInstance.Montage_Stop` (`self.BpAnimToast`) 0.1 "/Game/Animations/Toaster/ToastMontage_Reload.ToastMontage_Reload"))
  (bind _returnvalue_2 (`AudioComponent.IsPlaying` _audio))
  (if _returnvalue_2
    (`AudioComponent.Stop` _audio)))

(fn `UserConstructionScript`)