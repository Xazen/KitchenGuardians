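; Third selectable guardian character with its own life points and ammo, activated by touch, which deactivates the other two unless it is always active.
; Shot and swipe functions drain the magazine and block shooting when empty, while Tick refills it on a delay and updates its text.
; GotHit reduces HUD guardian life and local life, flashing a hit widget; death lowers the maximum life that Rebirth restores.
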(event `self.ReceiveActorOnInputTouchBegin`
  (params (FingerIndex :type "InputCoreTypes.ETouchIndex Enum" :default "Touch1"))
  (if (not (`self.Always Activated`))
    (set `self.Activated` true)
    (`SceneComponent.SetVisibility` (`self.Cube2`) true false)
    (set `/Game/Blueprints/BP_otherChar1.Activated` false (`self.other1`))
    (set `/Game/Blueprints/BP_otherChar2.Activated` false (`self.other2`))))

(event `self.ReceiveBeginPlay`
  (set `self.MaxHitPoints` (`self.LifePoints`))
  (if (`self.Always Activated`)
    (`SceneComponent.SetVisibility` (`self.Cube2`) true false))
  (bind _returnvalue (`|CreateWidget` "/Game/Blueprints/HUD/gotHit.gotHit_C" (`GameplayStatics.GetPlayerController` 0)))
  (set `self.gotHitFlash` _returnvalue)
  (`Widget.SetVisibility` _returnvalue "Hidden")
  (`UserWidget.AddToViewport` _returnvalue 0))

(event `self.ReceiveTick`
  (params (DeltaSeconds :type "Float (single-precision)"))
  (bind _gothitflash (`self.gotHitFlash`))
  (if (`self.doFlash`)
    (set `self.doFlash` false)
    (`Widget.SetVisibility` _gothitflash "Visible")
    (`KismetSystemLibrary.Delay` 0.1)
    (`Widget.SetVisibility` _gothitflash "Hidden"))
  (if (and (> (`self.Projectiles`) 0.0) (not (`self.canShoot`)) (> (`self.LifePoints`) 0))
    (set `self.canShoot` true))
  (`TextRenderComponent.SetText` (`self.Magazine`) (`KismetStringLibrary.Conv_DoubleToString` (`self.Projectiles`)))
  (if (not (or (`self.Always Activated`) (`self.Activated`)))
    (`SceneComponent.SetVisibility` (`self.Cube2`) false false))
  (if (< (`self.Projectiles`) 20.0)
    (if (`self.Reload`)
      (set `self.Projectiles` (+ (`self.Projectiles`) 1.0))
      (set `self.Reload` false)
      (else
        (`KismetSystemLibrary.Delay` (`self.ReloadTime`))
        (set `self.Reload` true)))))

(event `self.ReceiveActorBeginOverlap`
  (params (OtherActor :type "Actor Object Reference")))

(fn `GotHit`
  (params (Dmg :type Integer :default 0))
  (bind _asbp_main_hud (cast `/Game/Blueprints/Misc/BP_MainHUD` (`PlayerController.GetHUD` (`GameplayStatics.GetPlayerController` 0)))
    (:`then`
      (`/Game/Blueprints/Misc/BP_MainHUD.ReduceGuardianLife` _asbp_main_hud 3))
    (:`CastFailed`
      _))
  (if (> (`self.LifePoints`) 0)
    (bind _output_get (set `self.LifePoints` (- (`self.LifePoints`) Dmg)))
    (if (<= _output_get 0)
      (set `self.LifePoints` 0)
      (set `self.canShoot` false)
      (set `self.MaxHitPoints` (+ (`self.MaxHitPoints`) -1))
      (`KismetSystemLibrary.PrintString` "Bot3 Dead")
      (else
        (set `self.doFlash` true)))
    (else
      (set `self.RebirthRefill` 0.0)
      (set `self.doFlash` true))))

(fn `Rebirth`
  (set `self.LifePoints` (`self.MaxHitPoints`))
  (set `self.RebirthRefill` 0.0))

(fn `Shot`
  (bind _output_get (set `self.Projectiles` (+ (`self.Projectiles`) -1.0)))
  (if (<= _output_get 0.0)
    (set `self.canShoot` false)
    (set `self.Projectiles` 0.0)))

(fn `SwipeHit`
  (set `self.Projectiles` 0.0)
  (if (<= 0 0)
    (set `self.canShoot` false)
    (set `self.Projectiles` 0.0)))

(fn `SwipeLength`
  (params (SwipeLength :type "Float (double-precision)" :default 0.0) (SwipeMaxLength :type "Float (double-precision)" :default 0.0))
  (bind _output_get (set `self.Projectiles` (+ (* (/ SwipeLength SwipeMaxLength) -0.25) (`self.Projectiles`))))
  (if (<= _output_get 0.0)
    (set `self.canShoot` false)
    (set `self.Projectiles` 0.0)))

(fn `UserConstructionScript`)