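; BP_NoToast is a short-lived feedback actor that signals an empty toaster.
; On BeginPlay it plays the EmptyToaster sound at its location, then blinks visibility off, on and off through short chained delays.
; It destroys itself after the final hide, leaving a trailing delay and show step wired after DestroyActor.
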(event `self.ReceiveBeginPlay`
  (`GameplayStatics.PlaySoundAtLocation` "/Game/Audio/SFX/emptyToaster.emptyToaster" (`self.K2_GetActorLocation`))
  (`KismetSystemLibrary.Delay` 0.2)
  (`SceneComponent.SetVisibility` false)
  (`KismetSystemLibrary.Delay` 0.2)
  (`SceneComponent.SetVisibility` true)
  (`KismetSystemLibrary.Delay` 0.2)
  (`SceneComponent.SetVisibility` false)
  (`self.K2_DestroyActor`)
  (`KismetSystemLibrary.Delay` 0.2)
  (`SceneComponent.SetVisibility` true))

(event `self.ReceiveActorBeginOverlap`
  (params (OtherActor :type "Actor Object Reference")))

(event `self.ReceiveTick`
  (params (DeltaSeconds :type "Float (single-precision)")))

(fn `UserConstructionScript`)