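; Touch input controller that turns taps and swipes into the toaster guardian's attacks and updates its HUD ammo and life every tick.
; A timer and drag-distance check separate taps from swipes, with different thresholds when the touch starts on an enemy.
; Taps trigger a touched toast or fire a knife, showing empty feedback when unable to shoot.
; Swipes drag a ribbon emitter between camera and raycast hit, damaging enemies crossed.
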(event EventBeginPlay
  (bind _asbp_main_hud (Utilities|Casting|CastToBP_MainHUD (HUD|GetHUD (Game|GetPlayerController 0))))
  (Variables|Default|SetmainHudRef _asbp_main_hud)
  (bind _returnvalue (UserInterface|CreateWidget "/Game/Blueprints/HUD/MagazineBars.MagazineBars_C" (Game|GetPlayerController 0)))
  (Variables|Default|SetMagazineWidget _returnvalue)
  (Widget|SetVisibility _returnvalue "Visible")
  (UserInterface|Viewport|AddtoViewport _returnvalue 0))

(event EventActorBeginOverlap
  (params (OtherActor :type Actor%20Object%20Reference)))

(event EventTick
  (params (DeltaSeconds :type Float%20%28single-precision%29))
  (CallFunction|ShowMagazine))

(event Input|KeyboardEvents|T
  (:Pressed
    (Class|Guardian|GotHit (Variables|Default|GetGuardian%20Toast))))

(event Input|TouchEvents|InputTouch
  (params (Location :type Vector :default "0, 0, 0") (FingerIndex :type ETouchIndex%20Enum :default "Touch1"))
  (:Pressed
    (bind _output_get (Variables|Default|SetStartTouchLocation Location))
    (bind _hitactor (CallFunction|MakeTouchRaycast _output_get))
    (CallFunction|AdjustSwipetollerance _hitactor)
    (Variables|Default|SetisTap true)
    (Utilities|Time|SetTimerbyFunctionName 0 "testTouchTap" (Variables|Default|GetTapCheckTime))
    (Utilities|FlowControl|Sequence
      (:then_0
        (goto _label_2 Reset))))
  (:Released
    (Utilities|FlowControl|Sequence
      (:then_0
        (if (Variables|Default|GetisTap)
          (CallFunction|TestHandleTapInput Location)
          (elif (not (Variables|Default|GetisSwipeDestroyed))
            (CallFunction|DestroySwordSwipe))))
      (:then_1
        (goto _label Reset))))
  (:Moved
    (if (Variables|Default|GetisTap)
      (Development|PrintString (Utilities|String|Append "swipe distance:" (Utilities|String|ToString(Float) (Math|Vector|VectorLength (- (Variables|Default|GetStartTouchLocation) Location)))))
      (if (> (Math|Vector|VectorLength (- (Variables|Default|GetStartTouchLocation) Location)) (Variables|Default|GetTapCheckLength))
        (Utilities|FlowControl|DoOnce false :!label _label
          (:Completed
            (Development|PrintString "made Swipe becaus Length")
            (CallFunction|TestTouchTap))))
      (elif (not (Variables|/Script/KitchenGuardians.Guardian|GetisDead (Variables|Default|GetGuardian%20Toast)))
        (Utilities|FlowControl|Sequence
          (:then_0
            (Utilities|FlowControl|DoOnce false :!label _label_2
              (:Completed
                (bind (_hitsomething _hitactor_2 _hitlocation) (CallFunction|MakeTouchRaycast Location))
                (CallFunction|SwordSwipeInit Location 0 1 _hitactor_2 _hitlocation 0.0)
                (Variables|Default|SetisSwipeDestroyed false))))
          (:then_1
            (if (not (Variables|Default|GetisSwipeDestroyed))
              (bind (_hitsomething_2 _hitactor_3 _hitlocation_2) (CallFunction|MakeTouchRaycast Location))
              (CallFunction|SwordSwipeMove _hitactor_3 _hitlocation_2 Location))))
        (else
          (CallFunction|DestroySwordSwipe))))))

(fn ConstructionScript)

(fn GetOwnVector
  (params (Position0 :type Vector :default "0, 0, 0") (Position1 :type Vector :default "0, 0, 0"))
  (bind (_x _y) (Math|Vector|BreakVector Position0))
  (bind (_x_2 _y_2) (Math|Vector|BreakVector Position1))
  (return (Class|KismetMathLibrary|GetDirectionVector (Math|Vector|MakeVector _x _y 0.0) (Math|Vector|MakeVector _x_2 _y_2 0.0))))

(fn MakeTouchRaycast
  (params (Position :type Vector :default "0, 0, 0"))
  (bind (_x _y) (Math|Vector|BreakVector Position))
  (bind _returnvalue (Game|GetPlayerController 0))
  (bind (_worldlocation _worlddirection) (Class|PlayerController|DeprojectScreenPositiontoWorld _returnvalue _x _y))
  (bind (_outhit _returnvalue_2) (Collision|LineTraceByChannel _worldlocation (+ _worldlocation (* _worlddirection 2e+03)) "TraceTypeQuery1" true 0 "None"))
  (return _returnvalue_2 (.HitActor (Collision|BreakHitResult _outhit)) (.ImpactPoint (Collision|BreakHitResult _outhit))))

(fn ComparePosition
  (params (Old :type Actor%20Object%20Reference) (New :type Actor%20Object%20Reference))
  (return (> (.Y (Math|Vector|BreakVector (Class|KismetMathLibrary|GetDirectionVector (Transformation|GetActorLocation Old) (Transformation|GetActorLocation New)))) 0.0)))

(fn GetWorldLocation
  (params (ScreenLocation :type Vector :default "0, 0, 0"))
  (bind (_x _y) (Math|Vector|BreakVector ScreenLocation))
  (return (.WorldLocation (Class|PlayerController|DeprojectScreenPositiontoWorld (Game|GetPlayerController 0) _x _y))))

(fn ShowMagazine
  (bind _guardian_toast (Variables|Default|GetGuardian%20Toast))
  (Default|RefreshGuardianAmmo (Variables|Default|GetmainHudRef) (Variables|/Script/KitchenGuardians.Guardian|GetprojectilesCurrent _guardian_toast) (Variables|/Script/KitchenGuardians.Guardian|GetprojectilesMaximum _guardian_toast) "Toaster")
  (Default|RefreshGuardianLife (Variables|Default|GetmainHudRef) (Variables|/Script/KitchenGuardians.Guardian|Gethitpoints (Variables|Default|GetGuardian%20Toast)) "Toaster"))

(fn SwordSwipeInit
  (params (TouchStartPosition :type Vector :default "0, 0, 0") (TouchIndex :type Integer :default 0) (TouchStatus :type Integer :default 0) (LastSwipedActor :type Actor%20Object%20Reference) (RibbonOrigin :type Vector :default "0, 0, 0") (TimeStamp :type Float%20%28single-precision%29 :default 0.0))
  (Utilities|Array|SetArrayElem (Variables|Default|GetTouchStates) TouchIndex TouchStatus)
  (bind _output_get (Variables|Default|SetlastSwipedActor LastSwipedActor))
  (bind _asenemies (Utilities|Casting|CastToEnemies _output_get)
    (:then
      (Default|GotHit _asenemies "Swipe"))
    (:CastFailed
      _))
  (bind _returnvalue (Effects|SpawnEmitteratLocation "/Game/VFX/Particles/MA_SwipeRibbon.MA_SwipeRibbon" RibbonOrigin "0, 0, 0" false))
  (bind _output_get_2 (Variables|Default|SetSwipeRibbon _returnvalue))
  (bind _returnvalue_2 (Rendering|Material|CreateDynamicMaterialInstance _output_get_2 0 0 :!class /Script/Engine.PrimitiveComponent))
  (Variables|Default|SetSwipeMat _returnvalue_2))

(fn SwordSwipeMove
  (params (HitActor :type Actor%20Object%20Reference) (HitLocation :type Vector :default "0, 0, 0") (TouchPosition :type Vector :default "0, 0, 0"))
  (bind (_x _y) (Math|Vector|BreakVector TouchPosition))
  (Transformation|SetWorldLocation (Variables|Default|GetSwipeRibbon) (Math|Vector|Lerp(Vector) (.WorldLocation (Class|PlayerController|DeprojectScreenPositiontoWorld (Game|GetPlayerController 0) _x _y)) HitLocation 0.2) false)
  (if (not (== HitActor (Variables|Default|GetlastSwipedActor)))
    (bind _output_get (Variables|Default|SetlastSwipedActor HitActor))
    (bind _asenemies (Utilities|Casting|CastToEnemies _output_get))
    (Default|GotHit _asenemies "Swipe")))

(fn TestTouchTap
  (Variables|Default|SetisTap false))

(fn TestHandleTapInput
  (params (TouchLocation :type Vector :default "0, 0, 0"))
  (bind (_x _y) (Math|Vector|BreakVector TouchLocation))
  (bind _returnvalue (Class|Guardian|CanShoot (Variables|Default|GetGuardian%20Toast)))
  (if _returnvalue
    (bind (_hitsomething _hitactor _hitlocation) (CallFunction|MakeTouchRaycast TouchLocation))
    (bind _output_get (LocalVariables|SetLoc_Actor _hitactor))
    (LocalVariables|SetLoc_Class (Utilities|GetClass _output_get))
    ;[1 1 1] whether toaster is On
    (if true
      (if (== (LocalVariables|GetLoc_Class) "/Game/Blueprints/BP_Toast.BP_Toast_C")
        (bind _asbp_toast (Utilities|Casting|CastToBP_Toast (LocalVariables|GetLoc_Actor)))
        (Default|Tap _asbp_toast)
        (else
          (CallFunction|SpawnToastProjectile _hitlocation))))
    (else
      (Audio|PlaySoundatLocation "/Game/Audio/SFX/Placeholder/emptyToaster.emptyToaster" TouchLocation)
      (bind _foundwidgets (Widget|GetAllWidgetsOfClass "/Game/Blueprints/HUD/emptyToast.emptyToast_C" true))
      (for _array_element _foundwidgets
        ;[1 1 1] when not casted all widgets got removed
        (bind _asempty_toast (Utilities|Casting|CastToemptyToast _array_element))
        (Widget|RemovefromParent _asempty_toast))
      (bind _returnvalue_2 (UserInterface|CreateWidget "/Game/Blueprints/HUD/emptyToast.emptyToast_C" (Game|GetPlayerController 0)))
      (UserInterface|Viewport|AddtoViewport _returnvalue_2 0)
      (Class|UserWidget|SetPositioninViewport _returnvalue_2 (Math|Vector2D|MakeVector2D (+ _x -3e+01) (+ _y -3e+01))))))

(fn DestroySwordSwipe
  (Components|DestroyComponent (Variables|Default|GetSwipeRibbon))
  (Variables|Default|SetisSwipeDestroyed true))

(fn SpawnToastProjectile
  (params (TargetPosition :type Vector :default "0, 0, 0"))
  (bind _returnvalue (Class|Guardian|CanShoot (Variables|Default|GetGuardian%20Toast)))
  (if _returnvalue
    (Class|Guardian|Shot (Variables|Default|GetGuardian%20Toast) 1)
    (bind _returnvalue_2 (Game|SpawnActorfromClass "/Game/Blueprints/BP_Knife.BP_Knife_C" (Math|Transform|MakeTransform (Transformation|GetSocketLocation (Variables|Default|GetGuardian%20Toast) "None")) true 0))
    (Utilities|Casting|CastToBP_Cube (Variables|Default|GetCube))
    (Default|MoveTowards _returnvalue_2 TargetPosition)))

(fn AdjustSwipetollerance
  (params (startActor :type Actor%20Object%20Reference))
  (Utilities|Casting|CastToEnemies startActor
    (:then
      (Variables|Default|SetTapCheckTime (Variables|Default|GetTapCheckTimeMax))
      (Variables|Default|SetTapCheckLength (Variables|Default|GetTapCheckLengthMax)))
    (:CastFailed
      (Variables|Default|SetTapCheckTime (Variables|Default|GetTapCheckTimeMin))
      (Variables|Default|SetTapCheckLength (Variables|Default|GetTapCheckLengthMin)))))