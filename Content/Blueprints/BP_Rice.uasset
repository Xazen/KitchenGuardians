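; BP_Rice is guardian 1, a tappable character with hitpoints and projectile ammo; tapping it activates it and deactivates Toast and Ice.
; At zero hitpoints it enters rebirth: taps fill a HUD bar that hits and Tick adjust, reaching either revival or death.
; Swipe functions drain ammo, and Tick restores it fully after a delay when empty; the incremental Refill timer's setup is unreachable.
; Hits flash a GotHit widget.
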(event `Tap`
  (if (not (`self.Always Activated`))
    (set `self.activated` true)
    (`SceneComponent.SetVisibility` (`self.cube2`) true false)
    (set `/Game/Blueprints/BP_Toast.Activated` false (`self.Guardian Toast`))
    (set `/Game/Blueprints/BP_Ice.Activated` false (`self.Guardian Ice`)))
  (if (`self.RebirthActive`)
    (bind _output_get (set `self.reviveTapsCurrent` (+ (`self.reviveTapsCurrent`) 1.0)))
    (`/Game/Blueprints/Misc/BP_MainHUD.RefreshGuardianTap` (`self.mainHudRef`) 1 _output_get (`KismetMathLibrary.Conv_IntToDouble` (`self.reviveTapsMaximum`)))
    (if (>= _output_get (`KismetMathLibrary.Conv_IntToDouble` (`self.reviveTapsMaximum`)))
      (`/Game/Blueprints/Misc/BP_MainHUD.SetTapBarVisibilityForGuardian` (`self.mainHudRef`) 1 "Hidden")
      (`self.Rebirth`))))

(event `self.ReceiveActorOnInputTouchBegin`
  (params (FingerIndex :type "InputCoreTypes.ETouchIndex Enum" :default "Touch1"))
  (if false
    (`self.Tap`)))

(event `self.ReceiveBeginPlay`
  (if (`self.Always Activated`)
    (`SceneComponent.SetVisibility` (`self.cube2`) true false))
  (bind _returnvalue (`|CreateWidget` "/Game/Blueprints/HUD/gotHit.gotHit_C" (`GameplayStatics.GetPlayerController` 0)))
  (set `self.gotHitFlash` _returnvalue)
  (`Widget.SetVisibility` _returnvalue "Hidden")
  (`UserWidget.AddToViewport` _returnvalue 0)
  (bind _asbp_main_hud (cast `/Game/Blueprints/Misc/BP_MainHUD` (`PlayerController.GetHUD` (`GameplayStatics.GetPlayerController` 0))))
  (bind _output_get (set `self.mainHudRef` _asbp_main_hud))
  (`/Game/Blueprints/Misc/BP_MainHUD.SetTapBarVisibilityForGuardian` _output_get 1 "Hidden"))

(event `self.ReceiveTick`
  (params (DeltaSeconds :type "Float (single-precision)"))
  (bind _projectilescurrent (`self.projectilesCurrent`))
  (bind _gothitflash (`self.gotHitFlash`))
  (if (`self.RebirthActive`)
    (bind _output_get (set `self.reviveTapsCurrent` (+ (* (* DeltaSeconds (`KismetMathLibrary.Conv_IntToDouble` (`self.reviveTapsRemovedSecond`))) (`KismetMathLibrary.Conv_IntToDouble` (`self.reviveTapsRemovedSecondMultiplier`))) (`self.reviveTapsCurrent`))))
    (if (<= _output_get 0.0)
      (set `self.reviveTapsCurrent` 0.0)
      (set `self.IsDead` true)
      (elif (>= _output_get (`KismetMathLibrary.Conv_IntToDouble` (`self.reviveTapsMaximum`)))
        (`/Game/Blueprints/Misc/BP_MainHUD.SetTapBarVisibilityForGuardian` (`self.mainHudRef`) 1 "Hidden")
        (`self.Rebirth`)))
    (`/Game/Blueprints/Misc/BP_MainHUD.RefreshGuardianTap` (`self.mainHudRef`) 1 (`self.reviveTapsCurrent`) (`KismetMathLibrary.Conv_IntToDouble` (`self.reviveTapsMaximum`))))
  (if (`self.doFlash`)
    (set `self.doFlash` false)
    (`Widget.SetVisibility` _gothitflash "Visible")
    (`KismetSystemLibrary.Delay` 0.1)
    (`Widget.SetVisibility` _gothitflash "Hidden"))
  (if (and (> (`self.projectilesCurrent`) 0.0) (> (`self.hitpoints`) 0))
    _
    (else
      _))
  (if (not (or (`self.Always Activated`) (`self.activated`)))
    (`SceneComponent.SetVisibility` (`self.cube2`) false false))
  (if (and (< _projectilescurrent (`self.projectilesMaximum`)) (not (`self.RebirthActive`)))
    (if (== _projectilescurrent 0.0)
      (`/Engine/EditorBlueprintResources/StandardMacros.DoOnce` false :!label _label
        (:`Completed`
          (`KismetSystemLibrary.K2_PauseTimer` null "Refill")
          (`KismetSystemLibrary.Delay` (`self.FullRefillTime`))
          (set `self.projectilesCurrent` (`self.projectilesMaximum`))
          (goto _label_2 :!via `Reset`)))
      (else
        (`/Engine/EditorBlueprintResources/StandardMacros.DoOnce` false :!label _label_2
          (:`Completed`
            (`KismetSystemLibrary.K2_UnPauseTimer` null "Refill")
            (`|ExecutionSequence`
              (:`then_0`
                (goto _label_3 :!via `Reset`))
              (:`then_1`
                (goto _label :!via `Reset`)))))))
    (else
      (`/Engine/EditorBlueprintResources/StandardMacros.DoOnce` false :!label _label_3
        (:`Completed`
          (`KismetSystemLibrary.K2_PauseTimer` null "Refill")
          (goto _label_2 :!via `Reset`))))))

(event `self.ReceiveActorBeginOverlap`
  (params (OtherActor :type "Actor Object Reference")))

(fn `GotHit`
  (params (Dmg :type Integer :default 0))
  (bind _mainhudref (`self.mainHudRef`))
  (if (`self.RebirthActive`)
    (bind _output_get (set `self.reviveTapsCurrent` (- (`self.reviveTapsCurrent`) (`KismetMathLibrary.Conv_IntToDouble` (`self.reviveTapsRemovedEnemy`)))))
    (if (<= _output_get 0.0)
      (set `self.reviveTapsCurrent` 0.0)
      (set `self.IsDead` true))
    (set `self.doFlash` true :!label _label)
    (elif (> (`self.hitpoints`) 0)
      (bind _output_get_2 (set `self.hitpoints` (- (`self.hitpoints`) Dmg)))
      (if (<= _output_get_2 0)
        (set `self.hitpoints` 0)
        (set `self.RebirthActive` true)
        (`/Game/Blueprints/Misc/BP_MainHUD.SetTapBarVisibilityForGuardian` _mainhudref 1 "Visible")
        (bind _output_get_3 (set `self.reviveTapsCurrent` (`KismetMathLibrary.Conv_IntToDouble` (`self.reviveTapsStart`))))
        (`/Game/Blueprints/Misc/BP_MainHUD.RefreshGuardianTap` _mainhudref 1 _output_get_3 (`KismetMathLibrary.Conv_IntToDouble` (`self.reviveTapsMaximum`)))
        (else
          (set `self.doFlash` true)))
      (else
        (goto _label)))))

(fn `Rebirth`
  (if (`self.reviveIsFirst`)
    (set `self.reviveIsFirst` false)
    (set `self.hitpoints` (`self.reviveHitpointsFirst`))
    (else
      (set `self.hitpoints` (`self.reviveHitpointsNext`))))
  (set `self.reviveTapsCurrent` (`KismetMathLibrary.Conv_IntToDouble` (`self.reviveTapsStart`)))
  (set `self.reviveTapsMaximum` (+ (`self.reviveTapsMaximum`) (`self.reviveTapsAdditional`)))
  (set `self.RebirthActive` false))

(fn `Refill`
  (set `self.projectilesCurrent` (+ (`self.projectilesCurrent`) 1.0)))

(fn `Shot`
  (bind _output_get (set `self.projectilesCurrent` (+ (`self.projectilesCurrent`) 0.0)))
  (if (<= _output_get 0.0)
    (set `self.projectilesCurrent` 0.0)))

(fn `SwipeHit`
  (bind _output_get (set `self.projectilesCurrent` (+ (`self.projectilesCurrent`) -1.0)))
  (if (<= _output_get 0.0)
    (set `self.projectilesCurrent` 0.0)))

(fn `SwipeLength`
  (params (SwipeLength :type "Float (double-precision)" :default 0.0) (SwipeMaxLength :type "Float (double-precision)" :default 0.0))
  (bind _output_get (set `self.projectilesCurrent` (+ (* (/ SwipeLength SwipeMaxLength) -0.125) (`self.projectilesCurrent`))))
  (if (<= _output_get 0.0)
    (set `self.projectilesCurrent` 0.0)))

(fn `SwipeTime`
  (params (SwipeCurrentTime :type "Float (double-precision)" :default 0.0) (SwipeMaxTime :type "Float (double-precision)" :default 0.0))
  (bind _output_get (set `self.projectilesCurrent` (+ (* (/ SwipeCurrentTime SwipeMaxTime) -7.0) (`self.projectilesCurrent`))))
  (if (<= _output_get 0.0)
    (set `self.projectilesCurrent` 0.0)))

(fn `UserConstructionScript`)