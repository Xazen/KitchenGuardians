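; BP_Pumpkin_Tut is a pumpkin target, apparently for the tutorial, that dies when a touch on its TapBox is released while shooting is allowed.
; Death removes mesh and shadow, plays particles and pitch-randomized sound, then simulates physics on pre-placed giblets before delayed destruction.
; GibbletImpulse fires a radial force from the stored position at tap strength, or a random offset at swipe strength.
; Helper functions provide random swipe-hit sounds and spawn scale-up.
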(event `self.tapBox.OnInputTouchEnd`
  (params (FingerIndex :type "InputCoreTypes.ETouchIndex Enum" :default "Touch1") (TouchedComponent :type "PrimitiveComponent Object Reference"))
  (if (`/Game/Blueprints/BP_Cam.canShootonRelease` (`self.camRefForTap`))
    (set `self.willDie` true)
    (set `self.canMove` false)
    (`ActorComponent.K2_DestroyComponent` (`self.SkeletalMesh`))
    ;[1 1 1] because no skeletal mesh by now
    (`ActorComponent.K2_DestroyComponent` (`self.SkeletalMesh`))
    (`ActorComponent.K2_DestroyComponent` (`self.dropShadow`))
    (`ActorComponent.K2_DestroyComponent` (`self.shadowTester`))
    (`|ExecutionSequence`
      (:`then_0`
        (`GameplayStatics.SpawnEmitterAtLocation` "/Game/Effects/P_pumpkinDie.P_pumpkinDie" (`SceneComponent.K2_GetComponentLocation` (`self.TapReference`)))
        (`GameplayStatics.PlaySoundAtLocation` "/Game/Audio/SFX/firstIteration/pumpkinDied.pumpkinDied" (`self.K2_GetActorLocation`) 1.0 (`KismetMathLibrary.RandomFloatInRange` 0.7 1.4)))
      (:`then_1`
        ;[1 1 1] Giblet Activation and Add Impulse
        (for _array_element (`self.gibletList`)
          (`SceneComponent.SetVisibility` _array_element true false)
          (`PrimitiveComponent.SetSimulatePhysics` _array_element true))
        (`self.GibbletImpulse`)
        (`KismetSystemLibrary.Delay` (`self.GibbletStayTime`))
        (`self.K2_DestroyActor`)))))

(fn `GibbletImpulse`
  (bind _returnvalue (`KismetMathLibrary.RandomFloatInRange` -25.0 25.0))
  (bind _radialforce (`self.RadialForce`))
  (if (== (`self.RadialForcePosition`) (0.0 0.0 0.0))
    (`SceneComponent.K2_AddLocalOffset` _radialforce (`KismetMathLibrary.MakeVector` _returnvalue _returnvalue _returnvalue) true)
    (set `RadialForceComponent.ImpulseStrength` (`self.GibbletImpulseSwipe`) _radialforce)
    (else
      (`SceneComponent.K2_SetWorldLocation` _radialforce (`self.RadialForcePosition`) true)
      (set `RadialForceComponent.ImpulseStrength` (`self.GibbletImpulseTap`) _radialforce)))
  (`RadialForceComponent.FireImpulse` _radialforce))

(fn `playRandomSwipeHitSound`
  (params (Location :type "Object.Vector Structure" :default (0.0 0.0 0.0)))
  (switch `int` (`KismetMathLibrary.RandomIntegerInRange` 0 2)
    (:`0`
      (`GameplayStatics.PlaySoundAtLocation` "/Game/Audio/SFX/firstIteration/swipeHit1.swipeHit1" Location 1.0 (`KismetMathLibrary.RandomFloatInRange` 0.8 1.2)))
    (:`1`
      (`GameplayStatics.PlaySoundAtLocation` "/Game/Audio/SFX/firstIteration/swipeHit2.swipeHit2" Location 1.0 (`KismetMathLibrary.RandomFloatInRange` 0.8 1.2)))
    (:`2`
      (`GameplayStatics.PlaySoundAtLocation` "/Game/Audio/SFX/firstIteration/swipeHit3.swipeHit3" Location 1.0 (`KismetMathLibrary.RandomFloatInRange` 0.8 1.2)))))

(fn `SpawnScale`
  (params (DeltaTime :type "Float (double-precision)" :default 0.0))
  (bind _returnvalue (`KismetMathLibrary.Lerp` 1.0 (`self.SpawnMinScale`) (/ (`self.CurrentSpawnScaleTime`) (`self.SpawnScaleTime`))))
  (bind _output_get (set `self.CurrentSpawnScaleTime` (- (`self.CurrentSpawnScaleTime`) DeltaTime)))
  (if (<= _output_get 0.0)
    (set `self.isScaling` false)
    (set `self.CurrentSpawnScaleTime` 0.0))
  (`SceneComponent.SetWorldScale3D` (`self.Scene`) (`KismetMathLibrary.MakeVector` _returnvalue _returnvalue _returnvalue)))

(fn `UserConstructionScript`
  (bind _gibletlist (`self.gibletList`))
  (`/Engine/EditorBlueprintResources/StandardMacros.DoOnce` false
    (:`Completed`
      (`KismetArrayLibrary.Array_Add` _gibletlist (`self.Pumpkin_Gibblets_1__Gibblet_Part_01`))
      (`KismetArrayLibrary.Array_Add` _gibletlist (`self.Pumpkin_Gibblets_1__Gibblet_Part_02`))
      (`KismetArrayLibrary.Array_Add` _gibletlist (`self.Pumpkin_Gibblets_1__Gibblet_Part_03`))
      (`KismetArrayLibrary.Array_Add` _gibletlist (`self.Pumpkin_Gibblets_1__LP_Auge`))
      (`KismetArrayLibrary.Array_Add` _gibletlist (`self.Pumpkin_Gibblets_1__Gibblet_Part_04`)))))