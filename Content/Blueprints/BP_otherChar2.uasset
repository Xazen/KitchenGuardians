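; Guardian 2 character, one of three touch-selectable guardians, with hit points, a two-shot magazine and tap-to-revive.
; Touching it deactivates the other two or starts a reload when empty, and Tick runs the reload timer.
; Losing all life opens a rebirth tap bar on BP_MainHUD that decays and shrinks when hit, marking death at zero.
; Filling it restores health and raises the next tap requirement; damage briefly flashes a screen widget.
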(event `self.ReceiveActorOnInputTouchBegin`
  (params (FingerIndex :type "InputCoreTypes.ETouchIndex Enum" :default "Touch1"))
  (if (not (`self.AlwaysActive`))
    (set `self.Activated` true)
    (`SceneComponent.SetVisibility` (`self.Cube2`) true false)
    (set `/Game/Blueprints/BP_otherChar1.Activated` false (`self.other1`))
    (set `/Game/Blueprints/BP_otherChar3.Activated` false (`self.other2`)))
  (if (`self.RebirthActive`)
    (bind _output_get (set `self.TapCurrentValue` (+ (`self.TapCurrentValue`) 1.0)))
    (`/Game/Blueprints/Misc/BP_MainHUD.RefreshGuardianTap` (`self.mainHudRef`) 2 _output_get (`self.TapMaxValue`))
    (if (>= _output_get (`self.TapMaxValue`))
      (`/Game/Blueprints/Misc/BP_MainHUD.SetTapBarVisibilityForGuardian` (`self.mainHudRef`) 2 "Hidden")
      (`self.Rebirth`))
    (else
      (`|ExecutionSequence`
        (:`then_0`
          (if (== (`self.Projectiles`) 0.0)
            (`/Engine/EditorBlueprintResources/StandardMacros.DoOnce` false :!label _label
              (:`Completed`
                (set `self.reloading` true)))))))))

(event `self.ReceiveBeginPlay`
  (set `self.MaxHitPoints` (`self.LifePoints`))
  (if (`self.AlwaysActive`)
    (`SceneComponent.SetVisibility` (`self.Cube2`) true false))
  (bind _returnvalue (`|CreateWidget` "/Game/Blueprints/HUD/gotHit.gotHit_C" (`GameplayStatics.GetPlayerController` 0)))
  (set `self.gotHitFlash` _returnvalue)
  (`Widget.SetVisibility` _returnvalue "Hidden")
  (`UserWidget.AddToViewport` _returnvalue 0)
  (bind _asbp_main_hud (cast `/Game/Blueprints/Misc/BP_MainHUD` (`PlayerController.GetHUD` (`GameplayStatics.GetPlayerController` 0))))
  (bind _output_get (set `self.mainHudRef` _asbp_main_hud))
  (`/Game/Blueprints/Misc/BP_MainHUD.SetTapBarVisibilityForGuardian` _output_get 2 "Hidden"))

(event `self.ReceiveTick`
  (params (DeltaSeconds :type "Float (single-precision)"))
  (bind _gothitflash (`self.gotHitFlash`))
  (bind _reloadtime (`self.ReloadTime`))
  (if (`self.reloading`)
    (bind _output_get (set `self.currentReloadTime` (+ (`self.currentReloadTime`) DeltaSeconds)))
    (set `self.Projectiles` _output_get)
    (set `self.maxProjectiles` _reloadtime)
    (if (>= _output_get _reloadtime)
      (set `self.currentReloadTime` 0.0)
      (set `self.Projectiles` 2.0)
      (set `self.maxProjectiles` 2.0)
      (set `self.reloading` false)
      (`|ExecutionSequence`
        (:`then_0`
          (goto _label :!via `Reset`))
        (:`then_1`
          _))))
  (if (`self.RebirthActive`)
    (bind _output_get_2 (set `self.TapCurrentValue` (- (`self.TapCurrentValue`) (* DeltaSeconds (`self.TapReductionPerSecond`)))))
    (if (<= _output_get_2 0.0)
      (set `self.TapCurrentValue` 0.0)
      (set `self.IsDead` true))
    (`/Game/Blueprints/Misc/BP_MainHUD.RefreshGuardianTap` (`self.mainHudRef`) 2 (`self.TapCurrentValue`) (`self.TapMaxValue`)))
  (if (`self.doFlash`)
    (set `self.doFlash` false)
    (`Widget.SetVisibility` _gothitflash "Visible")
    (`KismetSystemLibrary.Delay` 0.1)
    (`Widget.SetVisibility` _gothitflash "Hidden"))
  (if (and (> (`self.Projectiles`) 0.0) (not (`self.canShoot`)) (> (`self.LifePoints`) 0) (not (`self.reloading`)))
    (set `self.canShoot` true))
  (`TextRenderComponent.SetText` (`self.Magazine`) "")
  (if (not (or (`self.AlwaysActive`) (`self.Activated`)))
    (`SceneComponent.SetVisibility` (`self.Cube2`) false false))
  (if (< (`self.Projectiles`) 2.0)
    (if (`self.Reload`)
      (if (`self.RebirthActive`)
        (set `self.Reload` false :!label _label_2)
        (else
          (bind _output_get_3 (set `self.Projectiles` (+ (`self.Projectiles`) 0.0)))
          (if (>= _output_get_3 2.0)
            (set `self.Projectiles` 0.0)
            (goto _label_2))))
      (else
        (`KismetSystemLibrary.Delay` (`self.ReloadTime`))
        (set `self.Reload` true)))))

(event `self.ReceiveActorBeginOverlap`
  (params (OtherActor :type "Actor Object Reference")))

(fn `GotHit`
  (params (Dmg :type Integer :default 0))
  (bind _mainhudref (`self.mainHudRef`))
  (if (`self.RebirthActive`)
    (bind _output_get (set `self.TapCurrentValue` (- (`self.TapCurrentValue`) (`self.TapsRemovedViaHit`))))
    (if (<= _output_get 0.0)
      (set `self.TapCurrentValue` 0.0)
      (set `self.IsDead` true))
    (set `self.doFlash` true :!label _label)
    (elif (> (`self.LifePoints`) 0)
      (bind _output_get_2 (set `self.LifePoints` (- (`self.LifePoints`) Dmg)))
      (if (<= _output_get_2 0)
        (set `self.LifePoints` 0)
        (set `self.canShoot` false)
        (set `self.RebirthActive` true)
        (`/Game/Blueprints/Misc/BP_MainHUD.SetTapBarVisibilityForGuardian` _mainhudref 2 "Visible")
        (bind _output_get_3 (set `self.TapCurrentValue` (`self.TapStartValue`)))
        (`/Game/Blueprints/Misc/BP_MainHUD.RefreshGuardianTap` _mainhudref 2 _output_get_3 (`self.TapMaxValue`))
        (else
          (set `self.doFlash` true)))
      (else
        (set `self.RebirthRefill` 0.0)
        (goto _label)))))

(fn `Rebirth`
  (if (`self.firstRevive`)
    (set `self.firstRevive` false)
    (set `self.MaxHitPoints` (`self.FirstReviveHitpoints`))
    (else
      (set `self.MaxHitPoints` (`self.AfterFirstReviveHitpoints`))))
  (set `self.LifePoints` (`self.MaxHitPoints`))
  (set `self.RebirthRefill` 0.0)
  (set `self.TapCurrentValue` (`self.TapStartValue`))
  (set `self.TapMaxValue` (+ (`self.TapMaxValue`) (`self.TapAdditionalTapsperreviva`)))
  (set `self.RebirthActive` false))

(fn `Shot`
  (bind _output_get (set `self.Projectiles` (+ (`self.Projectiles`) -1.0)))
  (if (<= _output_get 0.0)
    (set `self.canShoot` false)
    (set `self.Projectiles` 0.0)))

(fn `SwipeHit`
  (bind _output_get (set `self.Projectiles` (+ (`self.Projectiles`) -1.0)))
  (if (<= _output_get 0.0)
    (set `self.canShoot` false)
    (set `self.Projectiles` 0.0)))

(fn `UserConstructionScript`)