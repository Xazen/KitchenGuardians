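; Fridge spawner that launches BP_FruitSpline2 actors at its own transform when K is pressed, apparently as a jump test.
; Each spawn receives splines gathered from CurveArray, plus references to Ricebot and three other objects.
; Each press also shortens ReloadTime and raises Factor, but the timed Tick spawning is switched off and the live spawn ignores Factor.
; Score-weighted red/green fruit spawning on waypoint routes remains as unconnected legacy logic.
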(event EventBeginPlay)

(event EventActorBeginOverlap
  (params (OtherActor :type Actor%20Object%20Reference)))

(event EventTick
  (params (DeltaSeconds :type Float%20%28single-precision%29))
  (if false
    (if (Variables|Default|GetReloaded)
      (Variables|Default|SetReloaded false)
      (CallFunction|SpawnObject (Variables|Default|GetFactor) 0.0)
      (Variables|Default|SetReloadTime (* (Variables|Default|GetReloadTime) 0.97))
      (Variables|Default|SetFactor (* (Variables|Default|GetFactor) 1.02))
      (else
        (Utilities|FlowControl|Delay (Variables|Default|GetReloadTime))
        (Variables|Default|SetReloaded true)))))

(event Input|KeyboardEvents|K
  (:Pressed
    (CallFunction|SpawnObject (Variables|Default|GetFactor) 0.0)
    (Variables|Default|SetReloadTime (* (Variables|Default|GetReloadTime) 0.97))
    (Variables|Default|SetFactor (* (Variables|Default|GetFactor) 1.02))))

(fn ConstructionScript)

(fn SpawnObject
  (params (Factor :type Float%20%28single-precision%29 :default 0.0) (SpawnCase :type Float%20%28single-precision%29 :default 0.0))
  (bind _returnvalue (Transformation|GetActorTransform))
  (bind (_location _rotation) (Math|Transform|BreakTransform _returnvalue))
  (bind _returnvalue_2 (Game|SpawnActorfromClass "/Game/jumpTest/BP_FruitSpline2.BP_FruitSpline2_C" (Math|Transform|MakeTransform _location _rotation) true 0))
  (CallFunction|GetArrays)
  (Variables|/Game/jumpTest/BP_FruitSpline2.BP_FruitSpline2_C|SetSpline _returnvalue_2 (Variables|Default|GetSplinesArray))
  (Variables|/Game/jumpTest/BP_FruitSpline2.BP_FruitSpline2_C|Setother1 _returnvalue_2 (Variables|Default|Getother1))
  (Variables|/Game/jumpTest/BP_FruitSpline2.BP_FruitSpline2_C|Setother2 _returnvalue_2 (Variables|Default|Getother2))
  (Variables|/Game/jumpTest/BP_FruitSpline2.BP_FruitSpline2_C|Setother3 _returnvalue_2 (Variables|Default|Getother3))
  (Variables|/Game/jumpTest/BP_FruitSpline2.BP_FruitSpline2_C|SetRicebot _returnvalue_2 (Variables|Default|GetRicebot)))

(fn GetArrays
  (for (_array_element _array_index) (Variables|Default|GetcurveArray)
    (Utilities|Array|SetArrayElem (Variables|Default|GetSplinesArray) _array_index (Variables|/Game/Blueprints/BP_curve.BP_curve_C|GetSpline _array_element) true)))