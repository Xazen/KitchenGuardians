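; BP_FruitSpline is a tappable fruit that travels along a spline and costs Ricebot a life if it reaches the end.
; Tick advances its distance fraction at a speed that grows with progress, plus a term derived from the spline's vertical direction.
; A touch, while hits remain, fires the first activated of two spawners, else a third.
; If that spawner can shoot, a BP_Knife homes on the fruit and Ricebot plays.
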(event EventBeginPlay)

(event EventActorBeginOverlap
  (params (OtherActor :type Actor%20Object%20Reference)))

(event EventTick
  (params (DeltaSeconds :type Float%20%28single-precision%29))
  (bind _returnvalue (Transformation|GetActorTransform))
  (bind _spline (Variables|Default|GetSpline))
  (bind (_location _rotation _scale) (Math|Transform|BreakTransform _returnvalue))
  (if true
    (if (not false)
      (Transformation|SetActorTransform (Math|Transform|MakeTransform (Class|SplineComponent|GetWorldLocationatDistanceAlongSpline _spline (* (Spline|GetSplineLength _spline) (Variables|Default|GetDistPerc))) _rotation _scale))
      (bind _output_get (Variables|Default|SetDistPerc (+ (Variables|Default|GetDistPerc) (* DeltaSeconds (+ (* (Math|Float|Absolute(Float) (Math|Trig|Cos(Degrees) (.Z (Math|Vector|BreakVector (Class|SplineComponent|GetWorldDirectionatDistanceAlongSpline _spline (* (Spline|GetSplineLength _spline) (Variables|Default|GetDistPerc))))))) 0.4) (+ (* (Variables|Default|GetDistPerc) 0.3) 0.01))))))
      (if (>= _output_get 1.0)
        (Default|LostLife (Variables|Default|GetRicebot))
        (Actor|DestroyActor)))))

(event EventActorOnInputTouchBegin
  (params (FingerIndex :type ETouchIndex%20Enum :default "Touch1"))
  (CallFunction|SpawnKnife))

(fn ConstructionScript)

(fn GetVector
  (return (Transformation|GetWorldLocation)))

(fn SpawnKnife
  (bind _ricebot (Variables|Default|GetRiceBot))
  (if (> (Variables|Default|GetFruitHits) 0)
    (Variables|Default|SetFruitHits (+ (Variables|Default|GetFruitHits) -1))
    (if (== (Variables|Default|GetHitpoints) 0)
      (Variables|Default|Setloaded false))
    (bind (_knifespawn _canshoot) (CallFunction|GetKnifeSpawn))
    (if _canshoot
      (bind _returnvalue (Game|SpawnActorfromClass "/Game/Blueprints/BP_Knife.BP_Knife_C" _knifespawn true 0))
      (Default|MoveTowards _returnvalue self _ricebot false)
      (Audio|Components|Audio|Play _ricebot 0.0))))

(fn GetKnifeSpawn
  (bind _other1 (Variables|Default|Getother1))
  (bind _other2 (Variables|Default|Getother2))
  (bind _other3 (Variables|Default|Getother3))
  (if (Variables|/Game/Blueprints/BP_otherChar1.BP_otherChar1_C|GetActivated _other1)
    (LocalVariables|Setloca (Transformation|GetActorTransform _other1))
    (LocalVariables|Setload (Variables|/Game/Blueprints/BP_otherChar1.BP_otherChar1_C|GetcanShoot _other1))
    (Default|Shot _other1)
    (elif (Variables|/Game/Blueprints/BP_otherChar2.BP_otherChar2_C|GetActivated _other2)
      (LocalVariables|Setloca (Transformation|GetActorTransform _other2))
      (LocalVariables|Setload (Variables|/Game/Blueprints/BP_otherChar2.BP_otherChar2_C|GetcanShoot _other2))
      (Default|Shot _other2)
      (else
        (LocalVariables|Setloca (Transformation|GetActorTransform _other3))
        (LocalVariables|Setload (Variables|/Game/Blueprints/BP_otherChar3.BP_otherChar3_C|GetcanShoot _other3))
        (Default|Shot _other3))))
  (return (LocalVariables|Getloca) (LocalVariables|Getload)))